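; Base actor for a box-shaped signal quality zone in the voice chat system, telling player characters which signal-loss area they occupy.
; On server-side overlap, a character without an active zone registers this one through an interface-fetched reference and broadcasts its AreaZones value through a dispatcher.
; On exit, the server clears that character's zone reference and broadcasts the default enum value; the re-register branch there never runs.
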(event `self.Box.OnComponentBeginOverlap`
  (params (OverlappedComponent :type "PrimitiveComponent Object Reference") (OtherActor :type "Actor Object Reference") (OtherComp :type "PrimitiveComponent Object Reference") (OtherBodyIndex :type Integer) (bFromSweep :type Boolean) (SweepResult :type "HitResult Structure (by ref)"))
  (`/Engine/EditorBlueprintResources/ActorMacros.Switch Has Authority`
    (:`Authority`
      (set `self.hasLeftArea?` false)
      (bind _characterref (message `/Game/AdvancedVoIPVoiceChatSystem/Blueprints/Interfaces/Player/BPI_VoiceChat_Character.BPI_VoiceChatCharacterPlayerMP_Ref` OtherActor))
      (`/Game/AdvancedVoIPVoiceChatSystem/Blueprints/CharacterBP/Multiplayer/BP_VoiceChat_Character_White.SignalZoneTriggered` _characterref
        (:`then`)
        (:`else`
          (`/Game/AdvancedVoIPVoiceChatSystem/Blueprints/CharacterBP/Multiplayer/BP_VoiceChat_Character_White.SRV_ZoneTriggered` _characterref self)
          (`/Game/AdvancedVoIPVoiceChatSystem/Blueprints/CharacterBP/Multiplayer/BP_VoiceChat_Character_White.isZoneTriggered?_Dispatcher` _characterref (`self.areaZones`)))))))

(event `self.Box.OnComponentEndOverlap`
  (params (OverlappedComponent :type "PrimitiveComponent Object Reference") (OtherActor :type "Actor Object Reference") (OtherComp :type "PrimitiveComponent Object Reference") (OtherBodyIndex :type Integer))
  (`/Engine/EditorBlueprintResources/ActorMacros.Switch Has Authority`
    (:`Authority`
      (set `self.hasLeftArea?` true)
      (if (`self.hasLeftArea?`)
        (bind _characterref (message `/Game/AdvancedVoIPVoiceChatSystem/Blueprints/Interfaces/Player/BPI_VoiceChat_Character.BPI_VoiceChatCharacterPlayerMP_Ref` OtherActor))
        (set `/Game/AdvancedVoIPVoiceChatSystem/Blueprints/CharacterBP/Multiplayer/BP_VoiceChat_Character_White.SignalZoneTriggered` null _characterref)
        (`/Game/AdvancedVoIPVoiceChatSystem/Blueprints/CharacterBP/Multiplayer/BP_VoiceChat_Character_White.isZoneTriggered?_Dispatcher` _characterref "NewEnumerator0")
        (else
          (bind _characterref_2 (message `/Game/AdvancedVoIPVoiceChatSystem/Blueprints/Interfaces/Player/BPI_VoiceChat_Character.BPI_VoiceChatCharacterPlayerMP_Ref` OtherActor))
          (`/Game/AdvancedVoIPVoiceChatSystem/Blueprints/CharacterBP/Multiplayer/BP_VoiceChat_Character_White.SignalZoneTriggered` _characterref_2
            (:`then`
              _)
            (:`else`
              _))
          (`/Game/AdvancedVoIPVoiceChatSystem/Blueprints/CharacterBP/Multiplayer/BP_VoiceChat_Character_White.SRV_ZoneTriggered` _characterref_2 self)
          (`/Game/AdvancedVoIPVoiceChatSystem/Blueprints/CharacterBP/Multiplayer/BP_VoiceChat_Character_White.isZoneTriggered?_Dispatcher` _characterref_2 (`self.areaZones`)))))))

(fn `OnRep_NewVar_0`)

(fn `UserConstructionScript`)