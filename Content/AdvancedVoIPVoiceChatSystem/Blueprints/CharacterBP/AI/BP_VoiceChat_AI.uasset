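; AI character for the voice chat system that displays whether it has heard a sound on its TextRender.
; AIPerception updates loop through each updated actor's last sensed stimuli, setting the text to heard or not heard based on stimulus age.
; A multicast event re-enters that same loop, but the call to its server-side trigger and the text color changes are left unconnected.
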(event `self.AIPerception.OnPerceptionUpdated`
  (params (UpdatedActors :type "Array of Actor Object Reference (by ref)"))
  (for _array_element UpdatedActors :!label _label
    (bind _info (`AIPerceptionComponent.GetActorsPerception` (`self.AIPerception`) _array_element))
    (for _array_element_2 (`.LastSensedStimuli` (break `ActorPerceptionBlueprintInfo` _info))
      (if (>= (`.Age` (break `AIStimulus` _array_element_2)) 5.0)
        (set `self.AI_ResponseText` "I can not hear nothing at all !")
        (`TextRenderComponent.K2_SetText` (`self.TextRender`) (`self.AI_ResponseText`))
        (else
          (set `self.AI_ResponseText` "I've Heard YA!")
          (`TextRenderComponent.K2_SetText` (`self.TextRender`) (`self.AI_ResponseText`)))))))

(event `SRV_DetectedBySoundNotification`
  (`self.Mcast_DetectedBySoundNotification`))

(event `Mcast_DetectedBySoundNotification`
  (goto _label))

(fn `UserConstructionScript`
  (`parent.UserConstructionScript`))