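; VoIP talker component that routes a player's voice to global chat, team chat, walkie-talkies or cellphones.
; Talk begin activates the voice audio and sends it to source buses, using data tables keyed by signal zone and frequency or phone circuit.
; Talk end deactivates the audio and clears most sends.
; Server events swap attenuation, and an interruption dispatcher triggers a multicast that toggles mic-threshold console commands to restart talking.
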(event `self.BPOnTalkingBegin`
  (params (AudioComponent :type "AudioComponent Object Reference"))
  (bind _voip_audiocomponent (`self.VOIP_AudioComponent`))
  (bind _voip_audiocomponent_2 (`self.VOIP_AudioComponent`))
  (bind _playerref (`self.PlayerRef`))
  (bind _voip_audiocomponent_3 (`self.VOIP_AudioComponent`))
  (bind _playerref_2 (`self.PlayerRef`))
  (bind _voip_audiocomponent_4 (`self.VOIP_AudioComponent`))
  (bind _circuitnumberoffset (`/Game/AdvancedVoIPVoiceChatSystem/Blueprints/CharacterBP/Multiplayer/BP_VoiceChat_Character_White.CircuitNumberOffset` _playerref))
  (bind _voiceactorref (`/Game/AdvancedVoIPVoiceChatSystem/Blueprints/CharacterBP/Multiplayer/BP_VoiceChat_Character_White.VoiceActorRef` _playerref_2))
  (bind _output_get (set `self.VOIP_AudioComponent` AudioComponent))
  (set `self.rebootVOIP_FromReceiverPoint` true)
  (`/Engine/EditorBlueprintResources/StandardMacros.IsValid` _output_get
    (:`Is Valid`
      (`/Engine/EditorBlueprintResources/StandardMacros.IsValid` _playerref_2
        (:`Is Valid`
          (if (`/Game/AdvancedVoIPVoiceChatSystem/Blueprints/CharacterBP/Multiplayer/BP_VoiceChat_Character_White.isGlobalSpeak?` _playerref_2)
            (if (`self.muteResetVOIP_FromSenderPoint_WT-Speak`)
              ;[1 1 1] Team Speak and Global Speak with mute possibilities
              (`self.Activate` _voip_audiocomponent_4 false)
              (`AudioComponent.SetSourceBusSendPostEffect` _voip_audiocomponent_4 "/Game/AdvancedVoIPVoiceChatSystem/Audio/GlobalChatBuses/SB_GlobalVoiceChat.SB_GlobalVoiceChat" 1.0))
            (elif (`/Game/AdvancedVoIPVoiceChatSystem/Blueprints/CharacterBP/Multiplayer/BP_VoiceChat_Character_White.isTeamSpeak?` _playerref_2)
              (if (`self.muteResetVOIP_FromSenderPoint_WT-Speak`)
                (switch `/Game/AdvancedVoIPVoiceChatSystem/Blueprints/E_Team_Speak` (`/Game/AdvancedVoIPVoiceChatSystem/Blueprints/CharacterBP/Multiplayer/BP_VoiceChat_Character_White.TeamSpeakInfo` (`self.PlayerRef`))
                  (:`NewEnumerator0`
                    (`self.Activate` _voip_audiocomponent_4 false)
                    (`AudioComponent.SetSourceBusSendPostEffect` _voip_audiocomponent_4 "/Game/AdvancedVoIPVoiceChatSystem/Audio/TeamChat_Buses/SB_TeamVoiceChat_TeamA.SB_TeamVoiceChat_TeamA" 1.0))
                  (:`NewEnumerator1`
                    (`self.Activate` _voip_audiocomponent_4 false)
                    (`AudioComponent.SetSourceBusSendPostEffect` _voip_audiocomponent_4 "/Game/AdvancedVoIPVoiceChatSystem/Audio/TeamChat_Buses/SB_TeamVoiceChat_TeamB.SB_TeamVoiceChat_TeamB" 1.0))))
              (else
                (`/Engine/EditorBlueprintResources/StandardMacros.IsValid` _voiceactorref
                  (:`Is Valid`
                    (switch `/Game/AdvancedVoIPVoiceChatSystem/Blueprints/E_VoiceActorTypes` (`/Game/AdvancedVoIPVoiceChatSystem/Blueprints/VoiceActors/BP_VoiceActor_Master.VoiceActorType` _voiceactorref)
                      (:`NewEnumerator1`
                        (bind _walkietalkiesinglebandref (message `/Game/AdvancedVoIPVoiceChatSystem/Blueprints/Interfaces/VoiceActors/BPI_WalkieTalkie.BPI_WalkieTalkieSingleBandRef` (`/Game/AdvancedVoIPVoiceChatSystem/Blueprints/CharacterBP/Multiplayer/BP_VoiceChat_Character_White.VoiceActorRef` (`self.PlayerRef`))))
                        (if (`/Game/AdvancedVoIPVoiceChatSystem/Blueprints/VoiceActors/BP_VoiceActor_WalkieTalkie_SingleBand.isWalkieTalkieOn?` _walkietalkiesinglebandref)
                          (if (`/Game/AdvancedVoIPVoiceChatSystem/Blueprints/VoiceActors/BP_VoiceActor_WalkieTalkie_SingleBand.isWalkieTalkieTransmiting?` _walkietalkiesinglebandref)
                            (if (`self.muteResetVOIP_FromSenderPoint_WT-Speak`)
                              (bind _beepbusonly (`/Game/AdvancedVoIPVoiceChatSystem/Blueprints/VoiceActors/BP_VoiceActor_WalkieTalkie_SingleBand.BeepBusOnly` _walkietalkiesinglebandref))
                              (`self.Activate` _beepbusonly false)
                              (`AudioComponent.SetSourceBusSendPostEffect` _beepbusonly "/Game/AdvancedVoIPVoiceChatSystem/Audio/Radio_Buses/SB_radioSourceBus_99_1.SB_radioSourceBus_99_1" 1.0)
                              (bind _staticsoundbusonly (`/Game/AdvancedVoIPVoiceChatSystem/Blueprints/VoiceActors/BP_VoiceActor_WalkieTalkie_SingleBand.StaticSoundBusOnly` _walkietalkiesinglebandref))
                              (`self.Activate` _staticsoundbusonly false)
                              (`AudioComponent.SetSourceBusSendPostEffect` _staticsoundbusonly "/Game/AdvancedVoIPVoiceChatSystem/Audio/Radio_Buses/SB_radioSourceBus_99_1.SB_radioSourceBus_99_1" 1.0)
                              (bind _returnvalue (`|GetDataTableRow` "/Game/AdvancedVoIPVoiceChatSystem/Audio/Radio_Buses/PlayersBoxes/DataTables/DT_RadioFrequencies.DT_RadioFrequencies" (`KismetStringLibrary.Conv_StringToName` (`KismetStringLibrary.Conv_ByteToString` (select `/Game/AdvancedVoIPVoiceChatSystem/Blueprints/E_AreaZones` (`/Game/AdvancedVoIPVoiceChatSystem/Blueprints/CharacterBP/Multiplayer/BP_VoiceChat_Character_White.AreaZones_P` (`self.PlayerRef`)) :`NewEnumerator1` 1 :`NewEnumerator2` 2 :`NewEnumerator5` 3 :`NewEnumerator3` 4 :`NewEnumerator4` 5 :`NewEnumerator6` 99 :!type "Byte"))))
                                (:`then`
                                  (`self.Activate` _voip_audiocomponent false)
                                  (`AudioComponent.SetSourceBusSendPostEffect` _voip_audiocomponent (`.SB_RadioSourceBus_5_870D9D794DCC2C31F091ACA6D331AA8B` (break `/Game/AdvancedVoIPVoiceChatSystem/Audio/Radio_Buses/PlayersBoxes/DataTables/F_RadioFrequencies` _returnvalue)) 1.0)
                                  (`AudioComponent.SetSubmixSend` _voip_audiocomponent "/Game/AdvancedVoIPVoiceChatSystem/Audio/SubMix/SBM_walkieTalkieInput.SBM_walkieTalkieInput" 1.0)
                                  (`AudioComponent.SetSubmixSend` _voip_audiocomponent "/Game/AdvancedVoIPVoiceChatSystem/Audio/SubMix/SBM_AudioInputAnalysis.SBM_AudioInputAnalysis" 1.0)))))))
                      (:`NewEnumerator5`
                        (bind _walkietalkiemultibandref (message `/Game/AdvancedVoIPVoiceChatSystem/Blueprints/Interfaces/VoiceActors/BPI_WalkieTalkie.BPI_WalkieTalkieMultiBandRef` (`/Game/AdvancedVoIPVoiceChatSystem/Blueprints/CharacterBP/Multiplayer/BP_VoiceChat_Character_White.VoiceActorRef` (`self.PlayerRef`))))
                        (if (`/Game/AdvancedVoIPVoiceChatSystem/Blueprints/VoiceActors/BP_VoiceActor_WalkieTalkie_SingleBand.isWalkieTalkieOn?` _walkietalkiemultibandref)
                          (if (`/Game/AdvancedVoIPVoiceChatSystem/Blueprints/VoiceActors/BP_VoiceActor_WalkieTalkie_SingleBand.isWalkieTalkieTransmiting?` _walkietalkiemultibandref)
                            (if (`self.muteResetVOIP_FromSenderPoint_WT-Speak`)
                              (bind _returnvalue_2 (`|GetDataTableRow` "/Game/AdvancedVoIPVoiceChatSystem/Audio/Radio_Buses/PlayersBoxes/DataTables/DT_RadioFrequencies.DT_RadioFrequencies" (`KismetStringLibrary.Conv_StringToName` (`KismetStringLibrary.Conv_ByteToString` (+ (select `/Game/AdvancedVoIPVoiceChatSystem/Blueprints/E_AreaZones` (`/Game/AdvancedVoIPVoiceChatSystem/Blueprints/CharacterBP/Multiplayer/BP_VoiceChat_Character_White.AreaZones_P` (`self.PlayerRef`)) :`NewEnumerator1` 1 :`NewEnumerator2` 2 :`NewEnumerator5` 3 :`NewEnumerator3` 4 :`NewEnumerator4` 5 :`NewEnumerator6` 99 :!type "Byte") (select `/Game/AdvancedVoIPVoiceChatSystem/Blueprints/E_RadioFrequencies` (`/Game/AdvancedVoIPVoiceChatSystem/Blueprints/VoiceActors/BP_VoiceActor_WalkieTalkie_MultiBand.Frequencies` _walkietalkiemultibandref) :`NewEnumerator1` 6 :`NewEnumerator2` 12 :!type "Byte")))))
                                (:`then`
                                  (bind _beepbusonly_2 (`/Game/AdvancedVoIPVoiceChatSystem/Blueprints/VoiceActors/BP_VoiceActor_WalkieTalkie_SingleBand.BeepBusOnly` _walkietalkiemultibandref))
                                  (`self.Activate` _beepbusonly_2 false)
                                  (bind (_soundbusid _e_radiofrequencies _sb_radiosourcebus) (break `/Game/AdvancedVoIPVoiceChatSystem/Audio/Radio_Buses/PlayersBoxes/DataTables/F_RadioFrequencies` _returnvalue_2))
                                  (`AudioComponent.SetSourceBusSendPostEffect` _beepbusonly_2 _sb_radiosourcebus 1.0)
                                  (bind _staticsoundbusonly_2 (`/Game/AdvancedVoIPVoiceChatSystem/Blueprints/VoiceActors/BP_VoiceActor_WalkieTalkie_SingleBand.StaticSoundBusOnly` _walkietalkiemultibandref))
                                  (`self.Activate` _staticsoundbusonly_2 false)
                                  (`AudioComponent.SetSourceBusSendPostEffect` _staticsoundbusonly_2 _sb_radiosourcebus 1.0)
                                  (`self.Activate` _voip_audiocomponent_2 false)
                                  (`AudioComponent.SetSourceBusSendPostEffect` _voip_audiocomponent_2 _sb_radiosourcebus 1.0)
                                  (`AudioComponent.SetSubmixSend` _voip_audiocomponent_2 "/Game/AdvancedVoIPVoiceChatSystem/Audio/SubMix/SBM_walkieTalkieInput.SBM_walkieTalkieInput" 1.0)
                                  (`KismetSystemLibrary.PrintString` "Speaking" true true (struct :`R` 1.0 :`A` 1.0))))))))
                      (:`NewEnumerator6`
                        (bind _telephoneref (message `/Game/AdvancedVoIPVoiceChatSystem/Blueprints/Interfaces/VoiceActors/BPI_Telephone.BPI_TelephoneRef` (`/Game/AdvancedVoIPVoiceChatSystem/Blueprints/CharacterBP/Multiplayer/BP_VoiceChat_Character_White.VoiceActorRef` _playerref)))
                        (bind _ps (message `/Game/AdvancedVoIPVoiceChatSystem/Blueprints/Interfaces/Modes/BPI_PS_VoiceChat.BPI_PS_VoiceChatRef` (`Pawn.PlayerState` _playerref)))
                        (if (`/Game/AdvancedVoIPVoiceChatSystem/Blueprints/VoiceActors/BP_VoiceActor_Telephone.isCellphoneOn?_Phone` _telephoneref)
                          (if (`/Game/AdvancedVoIPVoiceChatSystem/Blueprints/Modes/BP_PS_VoiceChat_MP.isCellphoneTransmitting_PS?` _ps)
                            (bind _returnvalue_3 (`|GetDataTableRow` "/Game/AdvancedVoIPVoiceChatSystem/Audio/PhoneCircuit_Buses/DataTables/DT_PlayerCircuit_Cellphone.DT_PlayerCircuit_Cellphone" (`KismetStringLibrary.Conv_StringToName` (`KismetStringLibrary.Conv_IntToString` (+ (- (* (+ (`/Game/AdvancedVoIPVoiceChatSystem/Blueprints/CharacterBP/Multiplayer/BP_VoiceChat_Character_White.RemoteCircuit` _playerref) 1) _circuitnumberoffset) _circuitnumberoffset) (`/Game/AdvancedVoIPVoiceChatSystem/Blueprints/CharacterBP/Multiplayer/BP_VoiceChat_Character_White.CircuitNumber` _playerref)))))
                              (:`then`
                                (`self.Deactivate` _voip_audiocomponent_3)
                                (`self.Activate` _voip_audiocomponent_3 false)
                                (bind _soundsourcebusmappings (break `/Game/AdvancedVoIPVoiceChatSystem/Audio/PhoneCircuit_Buses/DataTables/F_PlayerCircuit` _returnvalue_3))
                                (`AudioComponent.SetSourceBusSendPostEffect` _voip_audiocomponent_3 _soundsourcebusmappings 1.0)
                                (`AudioComponent.SetSubmixSend` _voip_audiocomponent_3 "/Game/AdvancedVoIPVoiceChatSystem/Audio/SubMix/SBM_walkieTalkieInput.SBM_walkieTalkieInput" 1.0)
                                (`KismetSystemLibrary.PrintString` (`KismetSystemLibrary.GetDisplayName` _soundsourcebusmappings) true true (struct :`R` 1.0 :`G` 0.945419 :`A` 1.0) 15.0)))))))))))))))))

(event `self.BPOnTalkingEnd`
  (bind _voip_audiocomponent (`self.VOIP_AudioComponent`))
  (bind _voip_audiocomponent_2 (`self.VOIP_AudioComponent`))
  (bind _voip_audiocomponent_3 (`self.VOIP_AudioComponent`))
  (bind _playerref (`self.PlayerRef`))
  (bind _voiceactorref (`/Game/AdvancedVoIPVoiceChatSystem/Blueprints/CharacterBP/Multiplayer/BP_VoiceChat_Character_White.VoiceActorRef` _playerref))
  ;[1 1 1] End-Talk
  (`/Engine/EditorBlueprintResources/StandardMacros.IsValid` (`self.VOIP_AudioComponent`)
    (:`Is Valid`
      (`|ExecutionSequence`
        (:`then_0`
          (`/Engine/EditorBlueprintResources/StandardMacros.IsValid` _voiceactorref
            (:`Is Valid`
              (switch `/Game/AdvancedVoIPVoiceChatSystem/Blueprints/E_VoiceActorTypes` (`/Game/AdvancedVoIPVoiceChatSystem/Blueprints/VoiceActors/BP_VoiceActor_Master.VoiceActorType` _voiceactorref)
                (:`NewEnumerator1`
                  (bind _walkietalkiesinglebandref (message `/Game/AdvancedVoIPVoiceChatSystem/Blueprints/Interfaces/VoiceActors/BPI_WalkieTalkie.BPI_WalkieTalkieSingleBandRef` _voiceactorref))
                  (`self.Deactivate` (`self.VOIP_AudioComponent`))
                  (bind _staticsoundbusonly (`/Game/AdvancedVoIPVoiceChatSystem/Blueprints/VoiceActors/BP_VoiceActor_WalkieTalkie_SingleBand.StaticSoundBusOnly` _walkietalkiesinglebandref))
                  (`self.Deactivate` _staticsoundbusonly)
                  (`AudioComponent.SetSourceBusSendPostEffect` _staticsoundbusonly "/Game/AdvancedVoIPVoiceChatSystem/Audio/Radio_Buses/SB_radioSourceBus_99_1.SB_radioSourceBus_99_1" 0.0)
                  (`AudioComponent.SetSourceBusSendPostEffect` _voip_audiocomponent "/Game/AdvancedVoIPVoiceChatSystem/Audio/Radio_Buses/PlayersBoxes/SB_99_1L.SB_99_1L" 0.0)
                  (`AudioComponent.SetSourceBusSendPostEffect` _voip_audiocomponent "/Game/AdvancedVoIPVoiceChatSystem/Audio/Radio_Buses/PlayersBoxes/SB_99_1M.SB_99_1M" 0.0)
                  (`AudioComponent.SetSourceBusSendPostEffect` _voip_audiocomponent "/Game/AdvancedVoIPVoiceChatSystem/Audio/Radio_Buses/PlayersBoxes/SB_99_1M1.SB_99_1M1" 0.0)
                  (`AudioComponent.SetSourceBusSendPostEffect` _voip_audiocomponent "/Game/AdvancedVoIPVoiceChatSystem/Audio/Radio_Buses/PlayersBoxes/SB_99_1H.SB_99_1H" 0.0)
                  (`AudioComponent.SetSourceBusSendPostEffect` _voip_audiocomponent "/Game/AdvancedVoIPVoiceChatSystem/Audio/Radio_Buses/PlayersBoxes/SB_99_1C.SB_99_1C" 0.0))
                (:`NewEnumerator5`
                  (bind _walkietalkiemultibandref (message `/Game/AdvancedVoIPVoiceChatSystem/Blueprints/Interfaces/VoiceActors/BPI_WalkieTalkie.BPI_WalkieTalkieMultiBandRef` _voiceactorref))
                  (`self.Deactivate` (`self.VOIP_AudioComponent`))
                  (switch `/Game/AdvancedVoIPVoiceChatSystem/Blueprints/E_RadioFrequencies` (`/Game/AdvancedVoIPVoiceChatSystem/Blueprints/VoiceActors/BP_VoiceActor_WalkieTalkie_MultiBand.Frequencies` _walkietalkiemultibandref)
                    (:`NewEnumerator0`
                      (bind _beepbusonly (`/Game/AdvancedVoIPVoiceChatSystem/Blueprints/VoiceActors/BP_VoiceActor_WalkieTalkie_SingleBand.BeepBusOnly` _walkietalkiemultibandref))
                      (`self.Deactivate` _beepbusonly)
                      (`AudioComponent.SetSourceBusSendPostEffect` _beepbusonly "/Game/AdvancedVoIPVoiceChatSystem/Audio/Radio_Buses/SB_radioSourceBus_99_1.SB_radioSourceBus_99_1" 0.0)
                      (bind _staticsoundbusonly_2 (`/Game/AdvancedVoIPVoiceChatSystem/Blueprints/VoiceActors/BP_VoiceActor_WalkieTalkie_SingleBand.StaticSoundBusOnly` _walkietalkiemultibandref))
                      (`self.Deactivate` _staticsoundbusonly_2)
                      (`AudioComponent.SetSourceBusSendPostEffect` _staticsoundbusonly_2 "/Game/AdvancedVoIPVoiceChatSystem/Audio/Radio_Buses/SB_radioSourceBus_99_1.SB_radioSourceBus_99_1" 0.0)
                      (`AudioComponent.SetSourceBusSendPostEffect` _voip_audiocomponent_2 "/Game/AdvancedVoIPVoiceChatSystem/Audio/Radio_Buses/PlayersBoxes/SB_99_1L.SB_99_1L" 0.0)
                      (`AudioComponent.SetSourceBusSendPostEffect` _voip_audiocomponent_2 "/Game/AdvancedVoIPVoiceChatSystem/Audio/Radio_Buses/PlayersBoxes/SB_99_1M.SB_99_1M" 0.0)
                      (`AudioComponent.SetSourceBusSendPostEffect` _voip_audiocomponent_2 "/Game/AdvancedVoIPVoiceChatSystem/Audio/Radio_Buses/PlayersBoxes/SB_99_1M1.SB_99_1M1" 0.0)
                      (`AudioComponent.SetSourceBusSendPostEffect` _voip_audiocomponent_2 "/Game/AdvancedVoIPVoiceChatSystem/Audio/Radio_Buses/PlayersBoxes/SB_99_1H.SB_99_1H" 0.0)
                      (`AudioComponent.SetSourceBusSendPostEffect` _voip_audiocomponent_2 "/Game/AdvancedVoIPVoiceChatSystem/Audio/Radio_Buses/PlayersBoxes/SB_99_1C.SB_99_1C" 0.0))
                    (:`NewEnumerator1`
                      (`self.Deactivate` _beepbusonly)
                      (`AudioComponent.SetSourceBusSendPostEffect` _beepbusonly "/Game/AdvancedVoIPVoiceChatSystem/Audio/Radio_Buses/SB_radioSourceBus_102_6.SB_radioSourceBus_102_6" 0.0)
                      (`self.Deactivate` _staticsoundbusonly_2)
                      (`AudioComponent.SetSourceBusSendPostEffect` _staticsoundbusonly_2 "/Game/AdvancedVoIPVoiceChatSystem/Audio/Radio_Buses/SB_radioSourceBus_102_6.SB_radioSourceBus_102_6" 0.0)
                      (`AudioComponent.SetSourceBusSendPostEffect` _voip_audiocomponent_2 "/Game/AdvancedVoIPVoiceChatSystem/Audio/Radio_Buses/PlayersBoxes/SB_102_6L.SB_102_6L" 0.0)
                      (`AudioComponent.SetSourceBusSendPostEffect` _voip_audiocomponent_2 "/Game/AdvancedVoIPVoiceChatSystem/Audio/Radio_Buses/PlayersBoxes/SB_102_6M.SB_102_6M" 0.0)
                      (`AudioComponent.SetSourceBusSendPostEffect` _voip_audiocomponent_2 "/Game/AdvancedVoIPVoiceChatSystem/Audio/Radio_Buses/PlayersBoxes/SB_102_6M1.SB_102_6M1" 0.0)
                      (`AudioComponent.SetSourceBusSendPostEffect` _voip_audiocomponent_2 "/Game/AdvancedVoIPVoiceChatSystem/Audio/Radio_Buses/PlayersBoxes/SB_102_6H.SB_102_6H" 0.0)
                      (`AudioComponent.SetSourceBusSendPostEffect` _voip_audiocomponent_2 "/Game/AdvancedVoIPVoiceChatSystem/Audio/Radio_Buses/PlayersBoxes/SB_102_6C.SB_102_6C" 0.0))
                    (:`NewEnumerator2`
                      (`self.Deactivate` _beepbusonly)
                      (`AudioComponent.SetSourceBusSendPostEffect` _beepbusonly "/Game/AdvancedVoIPVoiceChatSystem/Audio/Radio_Buses/SB_radioSourceBus_102_6.SB_radioSourceBus_102_6" 0.0)
                      (`self.Deactivate` _staticsoundbusonly_2)
                      (`AudioComponent.SetSourceBusSendPostEffect` _staticsoundbusonly_2 "/Game/AdvancedVoIPVoiceChatSystem/Audio/Radio_Buses/SB_radioSourceBus_102_6.SB_radioSourceBus_102_6" 0.0)
                      (`AudioComponent.SetSourceBusSendPostEffect` _voip_audiocomponent_2 "/Game/AdvancedVoIPVoiceChatSystem/Audio/Radio_Buses/PlayersBoxes/SB_104_0L.SB_104_0L" 0.0)
                      (`AudioComponent.SetSourceBusSendPostEffect` _voip_audiocomponent_2 "/Game/AdvancedVoIPVoiceChatSystem/Audio/Radio_Buses/PlayersBoxes/SB_104_0M.SB_104_0M" 0.0)
                      (`AudioComponent.SetSourceBusSendPostEffect` _voip_audiocomponent_2 "/Game/AdvancedVoIPVoiceChatSystem/Audio/Radio_Buses/PlayersBoxes/SB_104_0M1.SB_104_0M1" 0.0)
                      (`AudioComponent.SetSourceBusSendPostEffect` _voip_audiocomponent_2 "/Game/AdvancedVoIPVoiceChatSystem/Audio/Radio_Buses/PlayersBoxes/SB_104_0H.SB_104_0H" 0.0)
                      (`AudioComponent.SetSourceBusSendPostEffect` _voip_audiocomponent_2 "/Game/AdvancedVoIPVoiceChatSystem/Audio/Radio_Buses/PlayersBoxes/SB_104_0C.SB_104_0C" 0.0))))
                (:`NewEnumerator6`
                  (bind _telephoneref (message `/Game/AdvancedVoIPVoiceChatSystem/Blueprints/Interfaces/VoiceActors/BPI_Telephone.BPI_TelephoneRef` _voiceactorref))
                  (`self.Deactivate` (`self.VOIP_AudioComponent`))
                  (`self.Deactivate` (`/Game/AdvancedVoIPVoiceChatSystem/Blueprints/VoiceActors/BP_VoiceActor_Master.Audio` _telephoneref))
                  (`KismetSystemLibrary.PrintString` "END TALK"))))))
        (:`then_1`
          (if (not (`/Game/AdvancedVoIPVoiceChatSystem/Blueprints/CharacterBP/Multiplayer/BP_VoiceChat_Character_White.isTeamSpeak?` _playerref))
            (switch `/Game/AdvancedVoIPVoiceChatSystem/Blueprints/E_Team_Speak` (`/Game/AdvancedVoIPVoiceChatSystem/Blueprints/CharacterBP/Multiplayer/BP_VoiceChat_Character_White.TeamSpeakInfo` _playerref)
              (:`NewEnumerator0`
                (`self.Deactivate` _voip_audiocomponent_3)
                (`AudioComponent.SetSourceBusSendPostEffect` _voip_audiocomponent_3 "/Game/AdvancedVoIPVoiceChatSystem/Audio/TeamChat_Buses/SB_TeamVoiceChat_TeamA.SB_TeamVoiceChat_TeamA" 0.0))
              (:`NewEnumerator1`
                (`self.Deactivate` _voip_audiocomponent_3)
                (`AudioComponent.SetSourceBusSendPostEffect` _voip_audiocomponent_3 "/Game/AdvancedVoIPVoiceChatSystem/Audio/TeamChat_Buses/SB_TeamVoiceChat_TeamB.SB_TeamVoiceChat_TeamB" 0.0)))))
        (:`then_2`
          (if (not (`/Game/AdvancedVoIPVoiceChatSystem/Blueprints/CharacterBP/Multiplayer/BP_VoiceChat_Character_White.isGlobalSpeak?` _playerref))
            (`self.Deactivate` _voip_audiocomponent_3)
            (`AudioComponent.SetSourceBusSendPostEffect` _voip_audiocomponent_3 "/Game/AdvancedVoIPVoiceChatSystem/Audio/GlobalChatBuses/SB_GlobalVoiceChat.SB_GlobalVoiceChat" 0.0)))))))

(event `ChangeAttProx`
  (params (SoundAttenuation :type "SoundAttenuation Object Reference") (CapsuleCollision :type "CapsuleComponent Object Reference"))
  (set `self.Settings` (make `VoiceSettings` CapsuleCollision SoundAttenuation)))

(event `ChangeAttAll`
  (params (SoundAttenuation :type "SoundAttenuation Object Reference"))
  (set `self.Settings` (make `VoiceSettings` null SoundAttenuation)))

(event `SRV_ChangeAttenuationProx`
  (params (SoundAttenuation :type "SoundAttenuation Object Reference") (CapsuleCollision :type "CapsuleComponent Object Reference"))
  (`self.ChangeAttProx` SoundAttenuation CapsuleCollision))

(event `SRV_ChangeAttenuationAll`
  (params (SoundAttenuation :type "SoundAttenuation Object Reference"))
  (`self.ChangeAttAll` SoundAttenuation))

(event `self.ReceiveTick`
  (params (DeltaSeconds :type "Float (single-precision)"))
  ;[1 0 0] #TEST for AI connect pins first - Proof it works use with OSS.VoiceLoopback 1 if its Local Machine and don't have second Real PC (seperate sound card) connect with node AI_Report in BP_VoiceChat_Character_TP_MP ( ###EnableThis### section )
)

(event `AI_Report`
  (params (PlayerRef :type "/Game/AdvancedVoIPVoiceChatSystem/Blueprints/CharacterBP/BaseCharacter/BP_VoiceChat_CharacterBase_MultiPlayer Object Reference"))
  ;[1 0 0] #TEST for AI connect pins first - Proof it works use with OSS.VoiceLoopback 1 if its Local Machine and don't have second Real PC (seperate sound card) connect with node AI_Report in BP_VoiceChat_Character_TP_MP ( ###EnableThis### section )
  (`self.Mcast_AI_Report` PlayerRef))

(event `Mcast_AI_Report`
  (params (PlayerRef :type "/Game/AdvancedVoIPVoiceChatSystem/Blueprints/CharacterBP/BaseCharacter/BP_VoiceChat_CharacterBase_MultiPlayer Object Reference"))
  ;[1 0 0] #TEST for AI connect pins first - Proof it works use with OSS.VoiceLoopback 1 if its Local Machine and don't have second Real PC (seperate sound card) connect with node AI_Report in BP_VoiceChat_Character_TP_MP ( ###EnableThis### section )
  (bind _characterref (message `/Game/AdvancedVoIPVoiceChatSystem/Blueprints/Interfaces/Player/BPI_VoiceChat_Character.BPI_VoiceChatCharacterPlayerMP_Ref` PlayerRef))
  (set `self.PlayerRefviaTrigger` _characterref))

(event `self.ReceiveBeginPlay`
  ;[1 1 1] Live-Reset Of Overlap AreaBoxes. Stops Begin-Talk and Restarts it
  (add `self.isInterupted_VOIP?_Dispatcher` (delegate `isInterupted_VOIP?_Dispatcher_Event`)))

(event `isInterupted_VOIP?_Dispatcher_Event`
  ;[1 1 1] Live-Reset Of Overlap AreaBoxes. Stops Begin-Talk and Restarts it
  (`self.SRV_isInterupted_VOIP?_INIT`))

(event `SRV_isInterupted_VOIP?_INIT`
  ;[1 1 1] Live-Reset Of Overlap AreaBoxes. Stops Begin-Talk and Restarts it
  (`self.MCast_isInterupted_VOIP?_INIT`))

(event `MCast_isInterupted_VOIP?_INIT`
  ;[1 1 1] Live-Reset Of Overlap AreaBoxes. Stops Begin-Talk and Restarts it
  (set `self.rebootVOIP_FromReceiverPoint` false)
  (`KismetSystemLibrary.ExecuteConsoleCommand` "voice.MicNoiseGateThreshold 0.02" null)
  (`KismetSystemLibrary.ExecuteConsoleCommand` "voice.SilenceDetectionThreshold 0.02" null)
  (if (not (`self.rebootVOIP_FromReceiverPoint`)) :!label _label
    (bind _counter (`/Engine/EditorBlueprintResources/StandardMacros.Do N` 5 :!label _label_2)
      (:`Exit`
        (if (== _counter 5)
          _
          (else
            (`KismetSystemLibrary.RetriggerableDelay` 1.0)
            (goto _label))))))
  (`KismetSystemLibrary.ExecuteConsoleCommand` "voice.MicNoiseGateThreshold 0.3" null)
  (`KismetSystemLibrary.ExecuteConsoleCommand` "voice.SilenceDetectionThreshold -1" null)
  (goto _label_2 :!via `Reset`))

(fn `BPI_VoiceCharacterRef`
  (returns (CharacterReference :type "Character Object Reference"))
  (return null))

(fn `BPI_VoiceChatCharacterPlayerMP_Ref`
  (returns (CharacterRef :type "/Game/AdvancedVoIPVoiceChatSystem/Blueprints/CharacterBP/Multiplayer/BP_VoiceChat_Character_White Object Reference"))
  (return null))

(fn `BPI_VoiceEngine`
  (returns (EngineReference :type "/Game/AdvancedVoIPVoiceChatSystem/Blueprints/BP_VoiceEngine_notUsedYet Object Reference"))
  (return null))