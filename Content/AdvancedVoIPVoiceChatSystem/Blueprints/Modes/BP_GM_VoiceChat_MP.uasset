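; Multiplayer voice-chat game mode that caches team spawn points, spawns black or white team characters, and applies low-quality test graphics settings on BeginPlay.
; On login, logout and team change, the server maintains a map of stable player circuit numbers, reusing freed slots.
; Timer-gated registration serializes simultaneous joins, waits for PlayerState and pawn, writes the number to both, and calls AutoOffComms on players' characters to fix late-join hearing.
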(event `self.ReceiveBeginPlay`
  ;[0 0 0 1 24] #ShowCaseCode #deleteItIfYouWant no depencies here
  ;;[1 1 1] Low Quality Settings Connect/Disconnect this to Begin Play if you want to test with lowest settings enabled on the hosts
  (`|ExecutionSequence`
    (:`then_0`
      (`KismetSystemLibrary.ExecuteConsoleCommand` "OSS.VoiceLoopback 0" null)
      (bind _returnvalue (`GameUserSettings.GetGameUserSettings`))
      (`GameUserSettings.SetScreenResolution` _returnvalue (`self.ScreenRes`))
      (`GameUserSettings.SetViewDistanceQuality` _returnvalue 0)
      (`GameUserSettings.SetPostProcessingQuality` _returnvalue 0)
      (`GameUserSettings.SetShadowQuality` _returnvalue 0)
      (`GameUserSettings.SetTextureQuality` _returnvalue 0)
      (`GameUserSettings.SetResolutionScaleValueEx` _returnvalue 0.0)
      (`GameUserSettings.SetFrameRateLimit` _returnvalue 30.0)
      (`GameUserSettings.SetFullscreenMode` _returnvalue "Windowed")
      (`GameUserSettings.ApplySettings` _returnvalue false))
    (:`then_1`
      (bind _outactors (`GameplayStatics.GetAllActorsOfClass` "/Game/AdvancedVoIPVoiceChatSystem/Blueprints/Modes/BP_S_BlackTeam_Spawn.BP_S_BlackTeam_Spawn_C"))
      (set `self.BlackSpawnPoints` _outactors))
    (:`then_2`
      (bind _outactors_2 (`GameplayStatics.GetAllActorsOfClass` "/Game/AdvancedVoIPVoiceChatSystem/Blueprints/Modes/BP_S_WhiteTeam_Spawn.BP_S_WhiteTeam_Spawn_C"))
      (set `self.WhiteSpawnPoints` _outactors_2))))

(event `SpawnBlackTeam`
  (params (PlayerController :type "PlayerController Object Reference"))
  (bind _blackspawnpoints (`self.BlackSpawnPoints`))
  ;[0 0 0 1 24] #ShowCaseCode #deleteItIfYouWant You can use this OR use your own logic but beware to update all the depedencies of this code
  ;;[1 1 1] Spawn Control
  (message `/Game/AdvancedVoIPVoiceChatSystem/Blueprints/Interfaces/Modes/BPI_PC_VoiceChat.BPI_SpawnPlayer` PlayerController "/Game/AdvancedVoIPVoiceChatSystem/Blueprints/CharacterBP/Multiplayer/BP_VoiceChat_Character_Black.BP_VoiceChat_Character_Black_C" (`self.GetTransform` (`|GetArrayItem` _blackspawnpoints (`KismetMathLibrary.RandomIntegerInRange` 0 (- (`KismetArrayLibrary.Array_Length` _blackspawnpoints) 1))))))

(event `RemovePlayerChangedTeam`
  (params (`changing PC` :type "PlayerController Object Reference"))
  ;[1 0 0 1 24] #DoNotDeleteIt You can adjust it (e.g., add max limit avoiding join new player after a specific limit reached) but the whole VoIP depends on it. What happends here is We created a "database" like system that each player gets a number starting from 0 when joining when the same player leaves the spot on dataabase becomes blank/null and you cannot interact with that number e.g.,4 so you can't call player 4 but if someone else joins then gets the number 4. That way we keep consistent entries for all previous players without any distruptions on current active voice channels
  ;;[1 1 1] Player Entry Stable numbering scheme Database
  ;;;[0 0 0] Used when a player changes Team
  (`/Engine/EditorBlueprintResources/ActorMacros.Switch Has Authority`
    (:`Authority`
      (`/Engine/EditorBlueprintResources/StandardMacros.IsValid` `changing PC`
        (:`Is Valid`
          (`KismetArrayLibrary.Array_RemoveItem` (`self.PlayerControllerRef`) `changing PC`)
          (bind _values (`BlueprintMapLibrary.Map_Values` (`self.PlayerAndCircuitNumberBurnedIn`)))
          (for (_array_element _array_index) _values
            (if (== _array_element `changing PC`)
              (`BlueprintMapLibrary.Map_Remove` (`self.PlayerAndCircuitNumberBurnedIn`) _array_index)
              (break))))))))

(event `addChangedTeam`
  (params (NewPlayer :type "PlayerController Object Reference"))
  ;[1 0 0 1 24] #DoNotDeleteIt You can adjust it (e.g., add max limit avoiding join new player after a specific limit reached) but the whole VoIP depends on it. What happends here is We created a "database" like system that each player gets a number starting from 0 when joining when the same player leaves the spot on dataabase becomes blank/null and you cannot interact with that number e.g.,4 so you can't call player 4 but if someone else joins then gets the number 4. That way we keep consistent entries for all previous players without any distruptions on current active voice channels
  ;;[1 1 1] Player Entry Stable numbering scheme Database
  ;;;[0 0 0] Used when a player changes Team
  (`/Engine/EditorBlueprintResources/ActorMacros.Switch Has Authority`
    (:`Authority`
      (`/Engine/EditorBlueprintResources/StandardMacros.IsValid` NewPlayer
        (:`Is Valid`
          (if (`KismetSystemLibrary.K2_IsTimerActiveHandle` (`self.ConcurrentJoinQueueWait_ChangeTeam_Timer`)) :!label _label
            (`KismetSystemLibrary.Delay` 0.2)
            (goto _label)
            (else
              (bind _returnvalue (`KismetSystemLibrary.K2_SetTimerDelegate` (delegate `ConcurrentJoinQueueWait_AddChangedTeam`) 0.2))
              (set `self.ConcurrentJoinQueueWait_ChangeTeam_Timer` _returnvalue))))))))

(event `ConcurrentJoinQueueWait_AddChangedTeam`
  ;[1 0 0 1 24] #DoNotDeleteIt You can adjust it (e.g., add max limit avoiding join new player after a specific limit reached) but the whole VoIP depends on it. What happends here is We created a "database" like system that each player gets a number starting from 0 when joining when the same player leaves the spot on dataabase becomes blank/null and you cannot interact with that number e.g.,4 so you can't call player 4 but if someone else joins then gets the number 4. That way we keep consistent entries for all previous players without any distruptions on current active voice channels
  ;;[1 1 1] Player Entry Stable numbering scheme Database
  ;;;[0 0 0] Used when a player changes Team
  (bind _returnvalue (`KismetArrayLibrary.Array_Add` (`self.PlayerControllerRef`) (stale `addChangedTeam` NewPlayer)))
  (`|ExecutionSequence`
    (:`then_0`
      (for _array_element (`self.PlayerControllerRef`)
        (`/Engine/EditorBlueprintResources/StandardMacros.IsValid` (`Controller.PlayerState` _array_element) :!label _label_2
          (:`Is Valid`
            (bind _asbp_voice_chat_character_white (cast `/Game/AdvancedVoIPVoiceChatSystem/Blueprints/CharacterBP/Multiplayer/BP_VoiceChat_Character_White` (`Controller.K2_GetPawn` _array_element)))
            (`/Game/AdvancedVoIPVoiceChatSystem/Blueprints/CharacterBP/Multiplayer/BP_VoiceChat_Character_White.AutoOffComms` _asbp_voice_chat_character_white))
          (:`Is Not Valid`
            (`KismetSystemLibrary.Delay` 0.2)
            (goto _label_2)))))
    (:`then_1`
      (`/Engine/EditorBlueprintResources/StandardMacros.IsValid` (`Controller.PlayerState` (stale `addChangedTeam` NewPlayer)) :!label _label_3
        (:`Is Valid`
          (bind _returnvalue_2 (`Controller.K2_GetPawn` (stale `addChangedTeam` NewPlayer)))
          (if (`KismetSystemLibrary.IsValid` _returnvalue_2) :!label _label_4
            (bind _asbp_voice_chat_character_white_2 (cast `/Game/AdvancedVoIPVoiceChatSystem/Blueprints/CharacterBP/Multiplayer/BP_VoiceChat_Character_White` _returnvalue_2))
            (if (<= _returnvalue (`self.maxPlayers`))
              (for _index (range (+ (`self.maxPlayers`) 1))
                (if (== (`BlueprintMapLibrary.Map_Find` (`self.PlayerAndCircuitNumberBurnedIn`) _index) null)
                  (`BlueprintMapLibrary.Map_Add` (`self.PlayerAndCircuitNumberBurnedIn`) _index (stale `addChangedTeam` NewPlayer))
                  (`/Game/AdvancedVoIPVoiceChatSystem/Blueprints/CharacterBP/Multiplayer/BP_VoiceChat_Character_White.Add_Circuit` _asbp_voice_chat_character_white_2 _index)
                  (bind _asbp_ps_voice_chat_mp (cast `/Game/AdvancedVoIPVoiceChatSystem/Blueprints/Modes/BP_PS_VoiceChat_MP` (`Pawn.PlayerState` _asbp_voice_chat_character_white_2)))
                  (set `/Game/AdvancedVoIPVoiceChatSystem/Blueprints/Modes/BP_PS_VoiceChat_MP.CircuitNumberLocal_PS` _index _asbp_ps_voice_chat_mp)
                  (`KismetSystemLibrary.K2_ClearAndInvalidateTimerHandle` (`self.ConcurrentJoinQueueWait_ChangeTeam_Timer`))
                  (break))))
            (else
              (`KismetSystemLibrary.Delay` 1.0)
              (goto _label_4))))
        (:`Is Not Valid`
          (`KismetSystemLibrary.Delay` 1.0)
          (goto _label_3))))))

(event `SpawnWhiteTeam`
  (params (PlayerController :type "PlayerController Object Reference"))
  (bind _whitespawnpoints (`self.WhiteSpawnPoints`))
  ;[0 0 0 1 24] #ShowCaseCode #deleteItIfYouWant You can use this OR use your own logic but beware to update all the depedencies of this code
  ;;[1 1 1] Spawn Control
  (message `/Game/AdvancedVoIPVoiceChatSystem/Blueprints/Interfaces/Modes/BPI_PC_VoiceChat.BPI_SpawnPlayer` PlayerController "/Game/AdvancedVoIPVoiceChatSystem/Blueprints/CharacterBP/Multiplayer/BP_VoiceChat_Character_White.BP_VoiceChat_Character_White_C" (`self.GetTransform` (`|GetArrayItem` _whitespawnpoints (`KismetMathLibrary.RandomIntegerInRange` 0 (- (`KismetArrayLibrary.Array_Length` _whitespawnpoints) 1))))))

(event `ConcurrentJoinQueueWait_Join`
  ;[1 0 0 1 24] #DoNotDeleteIt You can adjust it (e.g., add max limit avoiding join new player after a specific limit reached) but the whole VoIP depends on it. What happends here is We created a "database" like system that each player gets a number starting from 0 when joining when the same player leaves the spot on dataabase becomes blank/null and you cannot interact with that number e.g.,4 so you can't call player 4 but if someone else joins then gets the number 4. That way we keep consistent entries for all previous players without any distruptions on current active voice channels
  ;;[1 1 1] Player Entry Stable numbering scheme Database
  ;;;[0 0 0] #1
  (bind _returnvalue (`KismetArrayLibrary.Array_Add` (`self.PlayerControllerRef`) (stale `self.K2_PostLogin` NewPlayer)))
  (`|ExecutionSequence`
    (:`then_0`
      (for _array_element (`self.PlayerControllerRef`)
        (`/Engine/EditorBlueprintResources/StandardMacros.IsValid` (`Controller.PlayerState` _array_element) :!label _label_5
          (:`Is Valid`
            (bind _asbp_voice_chat_character_white (cast `/Game/AdvancedVoIPVoiceChatSystem/Blueprints/CharacterBP/Multiplayer/BP_VoiceChat_Character_White` (`Controller.K2_GetPawn` _array_element)))
            (`/Game/AdvancedVoIPVoiceChatSystem/Blueprints/CharacterBP/Multiplayer/BP_VoiceChat_Character_White.AutoOffComms` _asbp_voice_chat_character_white))
          (:`Is Not Valid`
            (`KismetSystemLibrary.Delay` 0.2)
            (goto _label_5)))))
    (:`then_1`
      (`/Engine/EditorBlueprintResources/StandardMacros.IsValid` (`Controller.PlayerState` (stale `self.K2_PostLogin` NewPlayer)) :!label _label_6
        (:`Is Valid`
          (bind _returnvalue_2 (`Controller.K2_GetPawn` (stale `self.K2_PostLogin` NewPlayer)))
          (if (`KismetSystemLibrary.IsValid` _returnvalue_2) :!label _label_7
            (bind _asbp_voice_chat_character_white_2 (cast `/Game/AdvancedVoIPVoiceChatSystem/Blueprints/CharacterBP/Multiplayer/BP_VoiceChat_Character_White` _returnvalue_2))
            (if (<= _returnvalue (`self.maxPlayers`))
              (for _index (range (+ (`self.maxPlayers`) 1))
                (if (== (`BlueprintMapLibrary.Map_Find` (`self.PlayerAndCircuitNumberBurnedIn`) _index) null)
                  (`BlueprintMapLibrary.Map_Add` (`self.PlayerAndCircuitNumberBurnedIn`) _index (stale `self.K2_PostLogin` NewPlayer))
                  (`/Game/AdvancedVoIPVoiceChatSystem/Blueprints/CharacterBP/Multiplayer/BP_VoiceChat_Character_White.Add_Circuit` _asbp_voice_chat_character_white_2 _index)
                  (bind _asbp_ps_voice_chat_mp (cast `/Game/AdvancedVoIPVoiceChatSystem/Blueprints/Modes/BP_PS_VoiceChat_MP` (`Pawn.PlayerState` _asbp_voice_chat_character_white_2)))
                  (set `/Game/AdvancedVoIPVoiceChatSystem/Blueprints/Modes/BP_PS_VoiceChat_MP.CircuitNumberLocal_PS` _index _asbp_ps_voice_chat_mp)
                  (`KismetSystemLibrary.K2_ClearAndInvalidateTimerHandle` (`self.ConcurrentJoinQueueWait_Timer_ADD`))
                  (break))))
            (else
              (`KismetSystemLibrary.Delay` 1.0)
              (goto _label_7))))
        (:`Is Not Valid`
          (`KismetSystemLibrary.Delay` 1.0)
          (goto _label_6))))))

(event `self.K2_PostLogin`
  (params (NewPlayer :type "PlayerController Object Reference"))
  ;[1 0 0 1 24] #DoNotDeleteIt You can adjust it (e.g., add max limit avoiding join new player after a specific limit reached) but the whole VoIP depends on it. What happends here is We created a "database" like system that each player gets a number starting from 0 when joining when the same player leaves the spot on dataabase becomes blank/null and you cannot interact with that number e.g.,4 so you can't call player 4 but if someone else joins then gets the number 4. That way we keep consistent entries for all previous players without any distruptions on current active voice channels
  ;;[1 1 1] Player Entry Stable numbering scheme Database
  ;;;[0 0 0] #1
  (`/Engine/EditorBlueprintResources/ActorMacros.Switch Has Authority`
    (:`Authority`
      (`/Engine/EditorBlueprintResources/StandardMacros.IsValid` NewPlayer
        (:`Is Valid`
          (if (`KismetSystemLibrary.K2_IsTimerActiveHandle` (`self.ConcurrentJoinQueueWait_Timer_ADD`)) :!label _label_8
            (`KismetSystemLibrary.Delay` 0.2)
            (goto _label_8)
            (else
              (bind _returnvalue (`KismetSystemLibrary.K2_SetTimerDelegate` (delegate `ConcurrentJoinQueueWait_Join`) 0.2))
              (set `self.ConcurrentJoinQueueWait_Timer_ADD` _returnvalue))))))))

(event `self.K2_OnLogout`
  (params (ExitingController :type "Controller Object Reference"))
  (bind _asplayer_controller (cast `PlayerController` ExitingController :!pure true))
  ;[1 0 0 1 24] #DoNotDeleteIt You can adjust it (e.g., add max limit avoiding join new player after a specific limit reached) but the whole VoIP depends on it. What happends here is We created a "database" like system that each player gets a number starting from 0 when joining when the same player leaves the spot on dataabase becomes blank/null and you cannot interact with that number e.g.,4 so you can't call player 4 but if someone else joins then gets the number 4. That way we keep consistent entries for all previous players without any distruptions on current active voice channels
  ;;[1 1 1] Player Entry Stable numbering scheme Database
  ;;;[0 0 0] #2
  (`/Engine/EditorBlueprintResources/ActorMacros.Switch Has Authority`
    (:`Authority`
      (`/Engine/EditorBlueprintResources/StandardMacros.IsValid` ExitingController
        (:`Is Valid`
          (`KismetArrayLibrary.Array_RemoveItem` (`self.PlayerControllerRef`) _asplayer_controller)
          (bind _values (`BlueprintMapLibrary.Map_Values` (`self.PlayerAndCircuitNumberBurnedIn`)))
          (for (_array_element _array_index) _values
            (if (== _array_element _asplayer_controller)
              (`BlueprintMapLibrary.Map_Remove` (`self.PlayerAndCircuitNumberBurnedIn`) _array_index)
              (break))))))))

(fn `BP_GM_VoiceChat_MP_AutoGenFunc`)

(fn `BPI_GM_VoiceChat_Ref`
  (returns (GameModeMultiplayer :type "/Game/AdvancedVoIPVoiceChatSystem/Blueprints/Modes/BP_GM_VoiceChat_MP Object Reference"))
  (return self))

(fn `UserConstructionScript`)