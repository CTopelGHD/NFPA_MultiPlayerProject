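; Showcase player controller for the multiplayer voice chat system that handles team joining and respawning.
; Black and White team requests arrive through interface events and go to the game mode's team spawn functions with this controller.
; The spawn callback clears the pawn's HUD, destroys the old pawn via a server-to-multicast chain, then spawns and possesses the new character.
; Server events keep the game mode's changed-team records in sync.
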(event `self.ReceiveBeginPlay`
  ;[0 0 0 1 24] #ShowCaseCode #deleteItIfYouWant BUT make sure to update its depencies and use your own logic for Team Join or JUST inherit it and use this
  ;;[1 1 1] Spawn Player here Widget -> PlayerController -> GameMode -> PlayerController
  (bind _asbp_gm_voice_chat_mp (cast `/Game/AdvancedVoIPVoiceChatSystem/Blueprints/Modes/BP_GM_VoiceChat_MP` (`GameplayStatics.GetGameMode`)))
  (set `self.GameMode` _asbp_gm_voice_chat_mp))

(event `/Game/AdvancedVoIPVoiceChatSystem/Blueprints/Interfaces/Modes/BPI_PC_VoiceChat.BPI_BlackTeam`
  ;[0 0 0 1 24] #ShowCaseCode #deleteItIfYouWant BUT make sure to update its depencies and use your own logic for Team Join or JUST inherit it and use this
  ;;[1 1 1] Spawn Player here Widget -> PlayerController -> GameMode -> PlayerController
  (`self.RequestBlackSpawn`))

(event `RequestBlackSpawn`
  ;[0 0 0 1 24] #ShowCaseCode #deleteItIfYouWant BUT make sure to update its depencies and use your own logic for Team Join or JUST inherit it and use this
  ;;[1 1 1] Spawn Player here Widget -> PlayerController -> GameMode -> PlayerController
  (`/Game/AdvancedVoIPVoiceChatSystem/Blueprints/Modes/BP_GM_VoiceChat_MP.SpawnBlackTeam` (`self.GameMode`) self))

(event `/Game/AdvancedVoIPVoiceChatSystem/Blueprints/Interfaces/Modes/BPI_PC_VoiceChat.BPI_WhiteTeam`
  ;[0 0 0 1 24] #ShowCaseCode #deleteItIfYouWant BUT make sure to update its depencies and use your own logic for Team Join or JUST inherit it and use this
  ;;[1 1 1] Spawn Player here Widget -> PlayerController -> GameMode -> PlayerController
  (`self.RequestWhiteSpawn`))

(event `RequestWhiteSpawn`
  ;[0 0 0 1 24] #ShowCaseCode #deleteItIfYouWant BUT make sure to update its depencies and use your own logic for Team Join or JUST inherit it and use this
  ;;[1 1 1] Spawn Player here Widget -> PlayerController -> GameMode -> PlayerController
  (`/Game/AdvancedVoIPVoiceChatSystem/Blueprints/Modes/BP_GM_VoiceChat_MP.SpawnWhiteTeam` (`self.GameMode`) self))

(event `SRV_RemovePlayerFromWorld`
  ;[0 0 0 1 24] #ShowCaseCode #deleteItIfYouWant BUT make sure to update its depencies and use your own logic for Team Join or JUST inherit it and use this
  ;;[1 1 1] Spawn Player here Widget -> PlayerController -> GameMode -> PlayerController
  (`self.MCast_RemovePlayerFromWorld`))

(event `/Game/AdvancedVoIPVoiceChatSystem/Blueprints/Interfaces/Modes/BPI_PC_VoiceChat.BPI_SpawnPlayer`
  (params (BaseCharacter :type "Character Class Reference") (Transform :type "Transform Structure"))
  ;[0 0 0 1 24] #ShowCaseCode #deleteItIfYouWant BUT make sure to update its depencies and use your own logic for Team Join or JUST inherit it and use this
  ;;[1 1 1] Spawn Player here Widget -> PlayerController -> GameMode -> PlayerController
  (`self.CL_RemoveMenu`)
  (`self.SRV_RemovePlayerFromWorld`)
  (bind _returnvalue (`|SpawnActorFromClass` BaseCharacter Transform "AdjustIfPossibleButAlwaysSpawn" "OverrideRootScale" null null))
  (`self.SRV_AddChangedTeam` self)
  (`self.Possess` _returnvalue))

(event `CL_RemoveMenu`
  ;[0 0 0 1 24] #ShowCaseCode #deleteItIfYouWant BUT make sure to update its depencies and use your own logic for Team Join or JUST inherit it and use this
  ;;[1 1 1] Spawn Player here Widget -> PlayerController -> GameMode -> PlayerController
  (bind _characterref (message `/Game/AdvancedVoIPVoiceChatSystem/Blueprints/Interfaces/Player/BPI_VoiceChat_Character.BPI_VoiceChatCharacterPlayerMP_Ref` (`self.K2_GetPawn`)))
  (`Widget.RemoveFromParent` (`/Game/AdvancedVoIPVoiceChatSystem/Blueprints/CharacterBP/Multiplayer/BP_VoiceChat_Character_White.HudRef` _characterref))
  (`WidgetBlueprintLibrary.SetInputMode_GameOnly` self)
  (set `self.bShowMouseCursor` false))

(event `MCast_RemovePlayerFromWorld`
  (bind _returnvalue (`self.K2_GetPawn`))
  ;[0 0 0 1 24] #ShowCaseCode #deleteItIfYouWant BUT make sure to update its depencies and use your own logic for Team Join or JUST inherit it and use this
  ;;[1 1 1] Spawn Player here Widget -> PlayerController -> GameMode -> PlayerController
  (`/Engine/EditorBlueprintResources/StandardMacros.IsValid` _returnvalue
    (:`Is Valid`
      (`self.SRV_Remove_ChangeTeamMap` self)
      (`self.K2_DestroyActor` _returnvalue))))

(event `SRV_Remove_ChangeTeamMap`
  (params (`Changing PC` :type "PlayerController Object Reference"))
  ;[0 0 0 1 24] #ShowCaseCode #deleteItIfYouWant BUT make sure to update its depencies and use your own logic for Team Join or JUST inherit it and use this
  ;;[1 1 1] Spawn Player here Widget -> PlayerController -> GameMode -> PlayerController
  (bind _asbp_gm_voice_chat_mp (cast `/Game/AdvancedVoIPVoiceChatSystem/Blueprints/Modes/BP_GM_VoiceChat_MP` (`GameplayStatics.GetGameMode`)))
  (`/Game/AdvancedVoIPVoiceChatSystem/Blueprints/Modes/BP_GM_VoiceChat_MP.RemovePlayerChangedTeam` _asbp_gm_voice_chat_mp `Changing PC`))

(event `SRV_AddChangedTeam`
  (params (`Changing PC` :type "PlayerController Object Reference"))
  ;[0 0 0 1 24] #ShowCaseCode #deleteItIfYouWant BUT make sure to update its depencies and use your own logic for Team Join or JUST inherit it and use this
  ;;[1 1 1] Spawn Player here Widget -> PlayerController -> GameMode -> PlayerController
  (bind _asbp_gm_voice_chat_mp (cast `/Game/AdvancedVoIPVoiceChatSystem/Blueprints/Modes/BP_GM_VoiceChat_MP` (`GameplayStatics.GetGameMode`)))
  (`/Game/AdvancedVoIPVoiceChatSystem/Blueprints/Modes/BP_GM_VoiceChat_MP.addChangedTeam` _asbp_gm_voice_chat_mp `Changing PC`))

(fn `BPI_PC_VoiceChatRef`
  (returns (PlayerControllerRef :type "/Game/AdvancedVoIPVoiceChatSystem/Blueprints/Modes/BP_PC_VoiceChat Object Reference"))
  (return self))

(fn `UserConstructionScript`)