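; Base pickup actor for the voice chat system that offers itself and its ActorToSpawn to a player character overlapping its trigger.
; On the server, begin overlap fetches the character through an interface and calls SRVSetPickup if its PickupVoiceActor is empty.
; End overlap clears that reference without checking which pickup it holds.
; SRV_RemoveActorFromWorld relays to a multicast event that destroys the pickup.
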(event `self.OverlapTrigger.OnComponentBeginOverlap`
  (params (OverlappedComponent :type "PrimitiveComponent Object Reference") (OtherActor :type "Actor Object Reference") (OtherComp :type "PrimitiveComponent Object Reference") (OtherBodyIndex :type Integer) (bFromSweep :type Boolean) (SweepResult :type "HitResult Structure (by ref)"))
  ;[1 1 1] Simple Multiplayer PickUp System Interaction
  (`/Engine/EditorBlueprintResources/ActorMacros.Switch Has Authority`
    (:`Authority`
      (bind _characterref (message `/Game/AdvancedVoIPVoiceChatSystem/Blueprints/Interfaces/Player/BPI_VoiceChat_Character.BPI_VoiceChatCharacterPlayerMP_Ref` OtherActor))
      (`/Game/AdvancedVoIPVoiceChatSystem/Blueprints/CharacterBP/Multiplayer/BP_VoiceChat_Character_White.Pickup_VoiceActor` _characterref
        (:`then`)
        (:`else`
          (`/Game/AdvancedVoIPVoiceChatSystem/Blueprints/CharacterBP/Multiplayer/BP_VoiceChat_Character_White.SRV_SetPickup` _characterref self (`self.ActorToSpawn`)))))))

(event `self.OverlapTrigger.OnComponentEndOverlap`
  (params (OverlappedComponent :type "PrimitiveComponent Object Reference") (OtherActor :type "Actor Object Reference") (OtherComp :type "PrimitiveComponent Object Reference") (OtherBodyIndex :type Integer))
  ;[1 1 1] Simple Multiplayer PickUp System Interaction
  (`/Engine/EditorBlueprintResources/ActorMacros.Switch Has Authority`
    (:`Authority`
      (bind _characterref (message `/Game/AdvancedVoIPVoiceChatSystem/Blueprints/Interfaces/Player/BPI_VoiceChat_Character.BPI_VoiceChatCharacterPlayerMP_Ref` OtherActor))
      (set `/Game/AdvancedVoIPVoiceChatSystem/Blueprints/CharacterBP/Multiplayer/BP_VoiceChat_Character_White.Pickup_VoiceActor` null _characterref))))

(event `SRV_RemoveActorFromWorld`
  ;[1 1 1] Simple Multiplayer PickUp System Interaction
  (`self.MCast_RemoveActorFromWorld`))

(event `MCast_RemoveActorFromWorld`
  ;[1 1 1] Simple Multiplayer PickUp System Interaction
  (`self.K2_DestroyActor`))

(fn `UserConstructionScript`)