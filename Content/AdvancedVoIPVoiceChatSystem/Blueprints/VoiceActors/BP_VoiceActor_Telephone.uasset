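; Telephone voice actor for multiplayer VoIP that lets players place, receive and end cellphone calls.
; It creates a phone widget listing other players; choosing one checks whether that circuit is busy, then dials and starts transmission after a timer.
; Server RPCs multicast sending, receiving, answered and transmitting flags into each PlayerState, driving ringtone, dial audio and HUD messages.
; A short timer re-enables redial after failed calls, and a reset function clears call state and audio.
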(event `SRV_isCellphoneTransmitting?_PS`
  (params (`isCellphoneTransmitting?` :type Boolean) (PS :type "/Game/AdvancedVoIPVoiceChatSystem/Blueprints/Modes/BP_PS_VoiceChat_MP Object Reference"))
  (set `/Game/AdvancedVoIPVoiceChatSystem/Blueprints/Modes/BP_PS_VoiceChat_MP.isCellphoneTransmitting_PS?` `isCellphoneTransmitting?` PS))

(event `SRV_isCellphoneTransmiting?`
  (params (`isCellphoneTransmiting?_Phone` :type Boolean))
  (bind _returnvalue (`self.GetOwner`))
  (`/Engine/EditorBlueprintResources/ActorMacros.Switch Has Authority`
    (:`Authority`
      (`/Engine/EditorBlueprintResources/StandardMacros.IsValid` _returnvalue :!label _label
        (:`Is Valid`
          (bind _characterref (message `/Game/AdvancedVoIPVoiceChatSystem/Blueprints/Interfaces/Player/BPI_VoiceChat_Character.BPI_VoiceChatCharacterPlayerMP_Ref` _returnvalue))
          (bind _playerstate (`Pawn.PlayerState` _characterref))
          (`/Engine/EditorBlueprintResources/StandardMacros.IsValid` _playerstate :!label _label_2
            (:`Is Valid`
              (bind _ps (message `/Game/AdvancedVoIPVoiceChatSystem/Blueprints/Interfaces/Modes/BPI_PS_VoiceChat.BPI_PS_VoiceChatRef` _playerstate))
              (`self.MCast_isCellphoneTransmiting?` `isCellphoneTransmiting?_Phone` _ps))
            (:`Is Not Valid`
              (`KismetSystemLibrary.Delay` 0.2)
              (goto _label_2))))
        (:`Is Not Valid`
          (`KismetSystemLibrary.Delay` 0.2)
          (goto _label))))))

(event `MCast_isCellphoneTransmiting?`
  (params (`isCellphoneTransmiting?_Phone` :type Boolean) (PS :type "/Game/AdvancedVoIPVoiceChatSystem/Blueprints/Modes/BP_PS_VoiceChat_MP Object Reference"))
  (bind _output_get (set `/Game/AdvancedVoIPVoiceChatSystem/Blueprints/Modes/BP_PS_VoiceChat_MP.isCellphoneTransmitting_PS?` `isCellphoneTransmiting?_Phone` PS))
  (set `self.isCellphoneTransmiting?_Phone` _output_get))

(event `SRV_CellphoneON`
  (set `self.isCellphoneOn?_Phone` true))

(event `SRV_CellphoneOFF`
  (set `self.isCellphoneOn?_Phone` false))

(event `CL_PhoneUI`
  (params (PlayerControllerRef :type "PlayerController Object Reference"))
  (`self.CreatePhoneUI` PlayerControllerRef))

(event `SRV_SearchPlayers`
  (params (PlayerControllerRef :type "PlayerController Object Reference"))
  (`self.CL_SearchPlayers` PlayerControllerRef))

(event `SRV_RefreshPhoneUI`
  (`/Engine/EditorBlueprintResources/ActorMacros.Switch Has Authority`
    (:`Authority`
      (`self.CL_RefreshPhoneUI`))))

(event `CL_SearchPlayers`
  (params (PlayerControllerRef :type "PlayerController Object Reference"))
  (`self.SearchPlayers` PlayerControllerRef))

(event `CL_RefreshPhoneUI`
  (bind _phonewidget (`self.PhoneWidget`))
  (bind _issendingcall__phone (`self.isSendingCall?_Phone`))
  (if _issendingcall__phone
    (`PanelWidget.ClearChildren` (`/Game/AdvancedVoIPVoiceChatSystem/Widgets/WB_UI_Cellphone.CellPhoneList` _phonewidget))
    (else
      (`/Engine/EditorBlueprintResources/StandardMacros.IsValid` _phonewidget
        (:`Is Valid`
          (if (`/Game/AdvancedVoIPVoiceChatSystem/Widgets/WB_UI_Cellphone.PhoneUIVisible?` _phonewidget)
            _
            (elif (not _issendingcall__phone)
              (`/Game/AdvancedVoIPVoiceChatSystem/Widgets/WB_UI_Cellphone.TogglePhoneUI` _phonewidget)
              (bind _asplayer_controller (cast `PlayerController` (`self.GetInstigatorController`)))
              (`self.SRV_SearchPlayers` _asplayer_controller))))))))

(event `SRV_CallReceive?`
  (params (`isReceivingCall?` :type Boolean) (PS :type "/Game/AdvancedVoIPVoiceChatSystem/Blueprints/Modes/BP_PS_VoiceChat_MP Object Reference") (`isDropped?` :type Boolean))
  (`/Engine/EditorBlueprintResources/ActorMacros.Switch Has Authority`
    (:`Authority`
      (`self.MCast_CallReceive?` `isReceivingCall?` PS `isDropped?`))))

(event `MCast_CallReceive?`
  (params (`isReceivingCall?_PS` :type Boolean) (PS :type "/Game/AdvancedVoIPVoiceChatSystem/Blueprints/Modes/BP_PS_VoiceChat_MP Object Reference") (`isDropped?` :type Boolean))
  (bind _returnvalue (`self.GetOwner`))
  (bind _calldial (`self.CallDial`))
  (bind _ringtone (`self.RingTone`))
  (bind _ringtone_2 (`self.RingTone`))
  (bind _output_get (set `/Game/AdvancedVoIPVoiceChatSystem/Blueprints/Modes/BP_PS_VoiceChat_MP.isReceivingCall?_PS` `isReceivingCall?_PS` PS))
  (bind _output_get_2 (set `self.isReceivingCall?_Phone` _output_get))
  (if _output_get_2
    (bind _characterref (message `/Game/AdvancedVoIPVoiceChatSystem/Blueprints/Interfaces/Player/BPI_VoiceChat_Character.BPI_VoiceChatCharacterPlayerMP_Ref` _returnvalue))
    (`/Game/AdvancedVoIPVoiceChatSystem/Blueprints/CharacterBP/Multiplayer/BP_VoiceChat_Character_White.CL_Local_HUD` _characterref "Incoming Call!")
    (`ActorComponent.Activate` _ringtone false)
    (`AudioComponent.Play` _ringtone 0.0)
    (elif `isDropped?`
      (bind _characterref_2 (message `/Game/AdvancedVoIPVoiceChatSystem/Blueprints/Interfaces/Player/BPI_VoiceChat_Character.BPI_VoiceChatCharacterPlayerMP_Ref` _returnvalue))
      (if (`AudioComponent.IsPlaying` _calldial)
        (`AudioComponent.Stop` _calldial)
        (`ActorComponent.Deactivate` _calldial))
      (if (`AudioComponent.IsPlaying` _ringtone_2)
        (`AudioComponent.Stop` _ringtone_2)
        (`ActorComponent.Deactivate` _ringtone_2))
      (`/Game/AdvancedVoIPVoiceChatSystem/Blueprints/CharacterBP/Multiplayer/BP_VoiceChat_Character_White.SRV_Local_HUD` _characterref_2 "Call did not answer"))))

(event `SRV_CallPickupRemote_PS`
  (params (`CallAnswer?` :type Boolean) (PS :type "/Game/AdvancedVoIPVoiceChatSystem/Blueprints/Modes/BP_PS_VoiceChat_MP Object Reference"))
  (`/Engine/EditorBlueprintResources/ActorMacros.Switch Has Authority`
    (:`Authority`
      (`self.MCast_CallPickupRemote` `CallAnswer?` PS))))

(event `MCast_CallPickupRemote`
  (params (`isCallAnswered?_PS` :type Boolean) (PS :type "/Game/AdvancedVoIPVoiceChatSystem/Blueprints/Modes/BP_PS_VoiceChat_MP Object Reference"))
  (bind _calldial (`self.CallDial`))
  (bind _ringtone (`self.RingTone`))
  (bind _audio (`self.Audio`))
  (bind _ringtone_2 (`self.RingTone`))
  ;[1 0 0 1 12] CallDial not play cellphone after hangUp from pickup Remote here Happens (bassically when remote presses terminate call here the sender gets executed from him/delegate) as source not initiator (remote) add breakpoint to stop callDIal to see
  (bind _output_get (set `/Game/AdvancedVoIPVoiceChatSystem/Blueprints/Modes/BP_PS_VoiceChat_MP.isCallAnswered?_PS` `isCallAnswered?_PS` PS))
  (bind _output_get_2 (set `self.isCallAnswered?_Phone` _output_get))
  (if _output_get_2
    (bind _characterref (message `/Game/AdvancedVoIPVoiceChatSystem/Blueprints/Interfaces/Player/BPI_VoiceChat_Character.BPI_VoiceChatCharacterPlayerMP_Ref` (`self.GetOwner`)))
    (`/Game/AdvancedVoIPVoiceChatSystem/Blueprints/CharacterBP/Multiplayer/BP_VoiceChat_Character_White.SRV_Local_HUD` _characterref "Call Answered")
    (if (`AudioComponent.IsPlaying` _calldial)
      (`AudioComponent.Stop` _calldial)
      (`ActorComponent.Deactivate` _calldial))
    (if (`AudioComponent.IsPlaying` _ringtone)
      (`AudioComponent.Stop` _ringtone)
      (`ActorComponent.Deactivate` _ringtone))
    (else
      (`ActorComponent.Deactivate` _audio)
      (`AudioComponent.SetSound` _audio null)
      (set `self.isCellphoneTransmiting?_Phone` false)
      (if (`AudioComponent.IsPlaying` _ringtone_2)
        (`AudioComponent.Stop` _ringtone_2)
        (`ActorComponent.Deactivate` _ringtone_2)))))

(event `SRV_isSendingCall?`
  (params (`isSendingCall?` :type Boolean) (PS :type "/Game/AdvancedVoIPVoiceChatSystem/Blueprints/Modes/BP_PS_VoiceChat_MP Object Reference") (`isDropped?` :type Boolean) (`isTurnedOff?` :type Boolean))
  (`/Engine/EditorBlueprintResources/ActorMacros.Switch Has Authority`
    (:`Authority`
      (`self.MCast_isSendingCall?` `isSendingCall?` PS `isDropped?` `isTurnedOff?`))))

(event `MCast_isSendingCall?`
  (params (`isSendingCall?_PS` :type Boolean) (PS :type "/Game/AdvancedVoIPVoiceChatSystem/Blueprints/Modes/BP_PS_VoiceChat_MP Object Reference") (`isDropped?` :type Boolean) (`isTurnedOff?` :type Boolean))
  (bind _calldial (`self.CallDial`))
  (bind _output_get (set `/Game/AdvancedVoIPVoiceChatSystem/Blueprints/Modes/BP_PS_VoiceChat_MP.isSendingCall?_PS` `isSendingCall?_PS` PS))
  (set `self.isSendingCall?_Phone` _output_get)
  (bind _characterref (message `/Game/AdvancedVoIPVoiceChatSystem/Blueprints/Interfaces/Player/BPI_VoiceChat_Character.BPI_VoiceChatCharacterPlayerMP_Ref` (`self.GetOwner`)))
  (if `isDropped?`
    ;[1 1 1 1 12] Make Extra Branch Here with same flow if you want after HangUp from Source before answer Call the message Terminated/dropped call then follow up with call did not answer if you do not this message do the above!
    (`/Game/AdvancedVoIPVoiceChatSystem/Blueprints/CharacterBP/Multiplayer/BP_VoiceChat_Character_White.SRV_Local_HUD` _characterref "Call did not answer")
    (if (`AudioComponent.IsPlaying` _calldial)
      (`AudioComponent.Stop` _calldial)
      (`ActorComponent.Deactivate` _calldial))
    (if (not (`KismetSystemLibrary.K2_IsTimerActiveHandle` (`self.MCast_isSendingCall_reCall_Timer`))) :!label _label_3
      ;[1 1 1] adjust to 4-5 if needed .. time that menu telephone opens up after a hold right click before answered by the destination .. Must match with Cellphone Circuit Setup #MATCHHERE <- search for it
      (bind _returnvalue (`KismetSystemLibrary.K2_SetTimerDelegate` (delegate `resetLocalRecall`) 2.0))
      (set `self.MCast_isSendingCall_reCall_Timer` _returnvalue))
    (elif `isTurnedOff?`
      (`/Game/AdvancedVoIPVoiceChatSystem/Blueprints/CharacterBP/Multiplayer/BP_VoiceChat_Character_White.CL_Local_HUD` _characterref "Player Has Telephone Turned OFF")
      (if (`AudioComponent.IsPlaying` _calldial)
        (`AudioComponent.Stop` _calldial)
        (`ActorComponent.Deactivate` _calldial)
        (goto _label_3)
        (else
          (goto _label_3))))))

(event `resetLocalRecall`
  (set `self.canRecall?` true)
  (`KismetSystemLibrary.K2_ClearAndInvalidateTimerHandle` (`self.MCast_isSendingCall_reCall_Timer`)))

(event `CL_canRecall?`
  (params (`canRecall?` :type Boolean))
  (set `self.canRecall?` `canRecall?`))

(event `SRV_canRecall?`
  (params (`canRecall?` :type Boolean))
  (`self.CL_canRecall?` `canRecall?`))

(event `SRV_setSoundLocal`
  (params (SoundBase :type "SoundBase Object Reference"))
  (`/Engine/EditorBlueprintResources/ActorMacros.Switch Has Authority`
    (:`Authority`
      (`self.CL_setSoundLocal` SoundBase))))

(event `CL_setSoundLocal`
  (params (SoundBase :type "SoundBase Object Reference"))
  (bind _audio (`self.Audio`))
  (`ActorComponent.Deactivate` _audio)
  (`AudioComponent.SetSound` _audio SoundBase)
  (`ActorComponent.Activate` _audio false))

(event `/Game/AdvancedVoIPVoiceChatSystem/Blueprints/Interfaces/VoiceActors/BPI_Telephone.BPI_NameCompareGET`
  (params (PlayerName :type Text) (RemoteCircuit :type Integer))
  (bind _returnvalue (`self.GetOwner`))
  (bind _calldial (`self.CallDial`))
  ;[1 1 1] Send Information about Player From Player that makes the Call. Here is also Information about Remote PlayerState (PS) and setting/checking variables and name
  (if (not (`KismetSystemLibrary.K2_IsTimerActiveHandle` (`self.SRV_Transmit_ON?_Timer`)))
    (for _array_element (`GameStateBase.PlayerArray` (`GameplayStatics.GetGameState`))
      (bind _ps (message `/Game/AdvancedVoIPVoiceChatSystem/Blueprints/Interfaces/Modes/BPI_PS_VoiceChat.BPI_PS_VoiceChatRef` _array_element))
      (bind _characterref (message `/Game/AdvancedVoIPVoiceChatSystem/Blueprints/Interfaces/Player/BPI_VoiceChat_Character.BPI_VoiceChatCharacterPlayerMP_Ref` (`self.GetOwner`)))
      (if (== (`/Game/AdvancedVoIPVoiceChatSystem/Blueprints/Modes/BP_PS_VoiceChat_MP.CircuitNumberLocal_PS` _ps) RemoteCircuit)
        (if (or (`/Game/AdvancedVoIPVoiceChatSystem/Blueprints/Modes/BP_PS_VoiceChat_MP.isReceivingCall?_PS` _ps) (`/Game/AdvancedVoIPVoiceChatSystem/Blueprints/Modes/BP_PS_VoiceChat_MP.isCallAnswered?_PS` _ps) (`/Game/AdvancedVoIPVoiceChatSystem/Blueprints/Modes/BP_PS_VoiceChat_MP.isSendingCall?_PS` _ps))
          (bind _hudref (`/Game/AdvancedVoIPVoiceChatSystem/Blueprints/CharacterBP/Multiplayer/BP_VoiceChat_Character_White.HudRef` _characterref))
          (`/Engine/EditorBlueprintResources/StandardMacros.IsValid` _hudref
            (:`Is Valid`
              (`/Game/AdvancedVoIPVoiceChatSystem/Widgets/WB_Player_HUD.ShowNotificationWarning` _hudref "This Circuit is Busy")))
          (else
            (set `self.TextToDisplayCmp` PlayerName)
            (`/Game/AdvancedVoIPVoiceChatSystem/Widgets/WB_UI_Cellphone.CL_SendingCallHideWidget` (`self.PhoneWidget`))
            (`/Engine/EditorBlueprintResources/StandardMacros.IsValid` _returnvalue :!label _label_4
              (:`Is Valid`
                (bind _characterref_2 (message `/Game/AdvancedVoIPVoiceChatSystem/Blueprints/Interfaces/Player/BPI_VoiceChat_Character.BPI_VoiceChatCharacterPlayerMP_Ref` _returnvalue))
                (bind _ps_2 (message `/Game/AdvancedVoIPVoiceChatSystem/Blueprints/Interfaces/Modes/BPI_PS_VoiceChat.BPI_PS_VoiceChatRef` (`Pawn.PlayerState` _characterref_2)))
                (set `self.isSendingCall?_Phone` true)
                (`self.SRV_isSendingCall?` true _ps_2)
                (`ActorComponent.Activate` _calldial false)
                (`KismetSystemLibrary.Delay` 0.2)
                (`AudioComponent.Play` _calldial 0.0)
                (`AudioParameterControllerInterface.SetTriggerParameter` _calldial "Play")
                (bind _returnvalue_2 (`KismetSystemLibrary.K2_SetTimerDelegate` (delegate `Delay_SRV_Transmit_ON?`) 2.0))
                (set `self.SRV_Transmit_ON?_Timer` _returnvalue_2))
              (:`Is Not Valid`
                (`KismetSystemLibrary.Delay` 0.2)
                (goto _label_4)))))))))

(event `Delay_SRV_Transmit_ON?`
  ;[1 1 1] Send Information about Player From Player that makes the Call. Here is also Information about Remote PlayerState (PS) and setting/checking variables and name
  (`KismetSystemLibrary.K2_ClearAndInvalidateTimerHandle` (`self.SRV_Transmit_ON?_Timer`))
  (`/Game/AdvancedVoIPVoiceChatSystem/Blueprints/CharacterBP/Multiplayer/BP_VoiceChat_Character_White.SRV_TransmitON?` (stale `/Game/AdvancedVoIPVoiceChatSystem/Blueprints/Interfaces/VoiceActors/BPI_Telephone.BPI_NameCompareGET` _characterref_2) (stale `/Game/AdvancedVoIPVoiceChatSystem/Blueprints/Interfaces/VoiceActors/BPI_Telephone.BPI_NameCompareGET` RemoteCircuit))
  (`/Game/AdvancedVoIPVoiceChatSystem/Blueprints/CharacterBP/Multiplayer/BP_VoiceChat_Character_White.CL_PreventFastHangUp` (stale `/Game/AdvancedVoIPVoiceChatSystem/Blueprints/Interfaces/VoiceActors/BPI_Telephone.BPI_NameCompareGET` _characterref_2)))

(fn `BPI_TelephoneRef`
  (returns (TelephoneRef :type "/Game/AdvancedVoIPVoiceChatSystem/Blueprints/VoiceActors/BP_VoiceActor_Telephone Object Reference"))
  (return self))

(fn `CreateButtonListAndSetText`
  (params (PlayersAvailable :type Text) (PlayerControllerRef :type "PlayerController Object Reference"))
  (returns (PlayersAvailableButtons :type "Button Object Reference"))
  (bind _returnvalue (`|CreateWidget` "/Game/AdvancedVoIPVoiceChatSystem/Widgets/WB_UI_Cellphone_ComponentButton.WB_UI_Cellphone_ComponentButton_C" PlayerControllerRef))
  (bind _output_get (set `self.TextToDisplay` PlayersAvailable))
  (`TextBlock.SetText` (`/Game/AdvancedVoIPVoiceChatSystem/Widgets/WB_UI_Cellphone_ComponentButton.CellphonePlayerNamesText` _returnvalue) _output_get)
  (return (`/Game/AdvancedVoIPVoiceChatSystem/Widgets/WB_UI_Cellphone_ComponentButton.CellPhoneButton` _returnvalue)))

(fn `CreatePhoneUI`
  (params (PlayerRef :type "PlayerController Object Reference"))
  (bind _output_get (set `self.PlayerControllerRef` PlayerRef))
  (`/Engine/EditorBlueprintResources/StandardMacros.IsValid` (`self.PhoneWidget`)
    (:`Is Not Valid`
      (bind _returnvalue (`|CreateWidget` "/Game/AdvancedVoIPVoiceChatSystem/Widgets/WB_UI_Cellphone.WB_UI_Cellphone_C" _output_get))
      (`/Engine/EditorBlueprintResources/StandardMacros.IsValid` _returnvalue
        (:`Is Valid`
          (bind _output_get_2 (set `self.PhoneWidget` _returnvalue))
          (`UserWidget.AddToViewport` _output_get_2 0))))))

(fn `OnRep_isCellphoneOn?`)

(fn `Reset Phone when OFF`
  (params (PS :type "/Game/AdvancedVoIPVoiceChatSystem/Blueprints/Modes/BP_PS_VoiceChat_MP Object Reference"))
  (bind _audio (`self.Audio`))
  (bind _calldial (`self.CallDial`))
  (bind _ringtone (`self.RingTone`))
  (set `self.canRecall?` true)
  (`ActorComponent.Deactivate` _audio)
  (set `AudioComponent.SourceEffectChain` "/Game/AdvancedVoIPVoiceChatSystem/Audio/RingTones/FX/SEPC_WT_onWT.SEPC_WT_onWT" _audio)
  (bind _characterref (message `/Game/AdvancedVoIPVoiceChatSystem/Blueprints/Interfaces/Player/BPI_VoiceChat_Character.BPI_VoiceChatCharacterPlayerMP_Ref` (`self.GetOwner`)))
  (`/Game/AdvancedVoIPVoiceChatSystem/Blueprints/CharacterBP/Multiplayer/BP_VoiceChat_Character_White.SRV_ReceivingCallSenderCircuitRemote` _characterref -999 PS)
  (`self.SRV_CallReceive?` false PS)
  (`self.SRV_CallPickupRemote_PS` false PS)
  (`self.SRV_isSendingCall?` false PS)
  (`|ExecutionSequence`
    (:`then_0`
      (if (`AudioComponent.IsPlaying` _calldial)
        (`AudioComponent.Stop` _calldial)))
    (:`then_1`
      (if (`ActorComponent.IsActive` _calldial)
        (`ActorComponent.Deactivate` _calldial)))
    (:`then_2`
      (if (`AudioComponent.IsPlaying` _ringtone)
        (`AudioComponent.Stop` _ringtone)))
    (:`then_3`
      (if (`ActorComponent.IsActive` _ringtone)
        (`ActorComponent.Deactivate` _ringtone)))))

(fn `SearchPlayers`
  (params (PlayerRef :type "PlayerController Object Reference"))
  (bind _phonewidget (`self.PhoneWidget`))
  (for _array_element (`GameStateBase.PlayerArray` (`GameplayStatics.GetGameState`))
    (bind _returnvalue (`PlayerState.GetPlayerName` _array_element))
    (if (`KismetStringLibrary.NotEqual_StrStr` (`PlayerState.GetPlayerName` (`Controller.PlayerState` PlayerRef)) _returnvalue)
      (bind _playersavailablebuttons (`self.CreateButtonListAndSetText` (`KismetTextLibrary.Conv_StringToText` _returnvalue) PlayerRef))
      (`/Engine/EditorBlueprintResources/StandardMacros.IsValid` _phonewidget
        (:`Is Valid`
          (`PanelWidget.AddChild` (`/Game/AdvancedVoIPVoiceChatSystem/Widgets/WB_UI_Cellphone.CellPhoneList` _phonewidget) _playersavailablebuttons))))))

(fn `UserConstructionScript`
  (`parent.UserConstructionScript`)
  (`self.CL_PhoneUI` (`self.PlayerControllerRef`))
  (set `self.canRecall?` true))