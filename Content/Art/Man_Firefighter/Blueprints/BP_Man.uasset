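; BP_Man is a male firefighter character assembled from a body mesh and modular outfit meshes.
; The construction script makes the pants, boots, gloves and helmet follow the body through leader pose, leaving jacket and equipment unlinked.
; SetupOutfitsVisability then switches on four Slot scalar parameters on the body materials.
; BeginPlay applies the helmet morph target to the body mesh.
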(event `self.ReceiveBeginPlay`
  (`SkeletalMeshComponent.SetMorphTarget` (`self.Mesh`) "mt_firefighter_helmet" 1.0 true))

(fn `SetupOutfitsVisability`
  (`|ExecutionSequence`
    (:`then_0`
      (`MeshComponent.SetScalarParameterValueOnMaterials` (`self.Mesh`) "Slot_1" 1.0))
    (:`then_1`
      (`MeshComponent.SetScalarParameterValueOnMaterials` (`self.Mesh`) "Slot_2" 1.0))
    (:`then_2`
      (`MeshComponent.SetScalarParameterValueOnMaterials` (`self.Mesh`) "Slot_3" 1.0))
    (:`then_3`
      (`MeshComponent.SetScalarParameterValueOnMaterials` (`self.Mesh`) "Slot_4" 1.0))))

(fn `UserConstructionScript`
  (`SkinnedMeshComponent.SetLeaderPoseComponent` (`self.SKM_m_med_nrw_Firefighter_Pants`) (`self.Mesh`) false false)
  (`SkinnedMeshComponent.SetLeaderPoseComponent` (`self.SKM_m_med_nrw_Firefighter_Boots`) (`self.Mesh`) false false)
  (`SkinnedMeshComponent.SetLeaderPoseComponent` (`self.SKM_m_med_nrw_Firefighter_Gloves`) (`self.Mesh`) false false)
  (`SkinnedMeshComponent.SetLeaderPoseComponent` (`self.SKM_m_med_nrw_Firefighter_Helmet`) (`self.Mesh`) false false)
  (`self.SetupOutfitsVisability`))