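; Electric-vehicle (EV) fire actor that stages smoke, jet flame, secondary fire and reignition effects, and lets the player put the fire out.
; StartSmoke sequences tagged Niagara actors on delays and ramps the jet stream's FlameVelocity by timeline before enabling its flame and spark spawn rates.
; Separate events fade or stop effects, partly by zeroing fluid density and temperature.
; FireKiller overlaps count hits; past the threshold it kills all effects and disables spraying.
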(event `self.ReceiveBeginPlay`
  ;[1 1 1] Begin Play
  (bind _outactors (`GameplayStatics.GetAllActorsOfClassWithTag` "/Script/Niagara.NiagaraActor" "SmokeAndFire"))
  (set `self.Out ActorsNiagaraSmokeAndFireParticlesArray` _outactors)
  (bind _returnvalue (`GameplayStatics.GetActorOfClass` "/Game/Core/TrainingManager/BP_InteractiveWench.BP_InteractiveWench_C"))
  (set `self.Wench Ref` _returnvalue)
  (bind _outactors_2 (`GameplayStatics.GetAllActorsOfClassWithTag` "/Script/Niagara.NiagaraActor" "HasDensityUserParameter"))
  (set `self.Out HasDensityUserParameterActors` _outactors_2))

(event `ToggleJetStreamOn`
  (bind (_direction _lerp) (`Timeline|Timeline_1` :!via `PlayFromStart`)
    (:`Update`
      (`NiagaraComponent.SetVariableVec3` (`self.NS_JetStream`) "FlameVelocity" (`KismetMathLibrary.VLerp` (0.0 0.0 0.0) (`self.FullStream Velocity`) _lerp)))
    (:`Finished`
      (`self.FinishedJetStream`))))

(event `StartSmoke`
  ;[0.05127 0.05127 0.05127] Starts Smoke and Residuals on a Set Timer
  (`self.ToggleNiagaraSystem` "SmokeStart" true)
  (`self.ToggleNiagaraSystem` "FrontWindow")
  (`self.ToggleNiagaraSystem` "ExtendedEV_Smoke" true)
  (`KismetSystemLibrary.Delay` 90.0)
  (`self.ToggleJetStreamOn`)
  (`KismetSystemLibrary.Delay` 5.0)
  (`self.ToggleNiagaraSystem` "SecondaryFire" true)
  (`KismetSystemLibrary.Delay` 5.0)
  (`self.ToggleNiagaraSystem` "FrontWindow" true))

(event `ToggleALL_OFF`
  (for _array_element (`self.Out ActorsNiagaraSmokeAndFireParticlesArray`)
    (`ActorComponent.Deactivate` (`NiagaraActor.NiagaraComponent` _array_element)))
  (`ActorComponent.Deactivate` (`self.NS_JetStream`)))

(event `FadeOutSmoke`
  ;[0.05127 0.05127 0.05127] Fade Out Smoke
  (bind _outactors (`GameplayStatics.GetAllActorsOfClassWithTag` "/Script/Niagara.NiagaraActor" "SecondaryFire"))
  (for _array_element _outactors
    (`ActorComponent.Deactivate` (`NiagaraActor.NiagaraComponent` _array_element))
    (`KismetSystemLibrary.Delay` 10.0)
    (`KismetSystemLibrary.Delay` 2.0)
    (`ActorComponent.Deactivate` (`self.NS_JetStream`))
    (for _array_element_2 (`self.Out HasDensityUserParameterActors`)
      (`NiagaraComponent.SetVariableFloat` (`NiagaraActor.NiagaraComponent` _array_element_2) "DensityMultiplier" 0.0))))

(event `StartReignitionFire`
  ;[0.05127 0.05127 0.05127] Reignitioin Start And Stop Events
  (bind _outactors (`GameplayStatics.GetAllActorsOfClassWithTag` "/Script/Niagara.NiagaraActor" "ReignitionStart"))
  (for _array_element _outactors
    (`ActorComponent.Activate` (`NiagaraActor.NiagaraComponent` _array_element) false)))

(event `Start After Fire`
  (`self.StartReignitionFire`)
  (`KismetSystemLibrary.Delay` 10.0)
  (`self.StopReignitionFire`))

(event `StopReignitionFire`
  ;[0.05127 0.05127 0.05127] Reignitioin Start And Stop Events
  (bind _outactors (`GameplayStatics.GetAllActorsOfClassWithTag` "/Script/Niagara.NiagaraActor" "ReignitionFire"))
  (for _array_element _outactors
    (`ActorComponent.Deactivate` (`NiagaraActor.NiagaraComponent` _array_element))
    (bind _outactors_2 (`GameplayStatics.GetAllActorsOfClassWithTag` "/Script/Niagara.NiagaraActor" "ReignitionFireFluid"))
    (for _array_element_2 _outactors_2
      (bind _niagaracomponent (`NiagaraActor.NiagaraComponent` _array_element_2))
      (`NiagaraComponent.SetVariableFloat` _niagaracomponent "DensityMultiplier" 0.0)
      (`NiagaraComponent.SetVariableFloat` _niagaracomponent "TemperatureMultiplier" 0.0))))

(event `self.TriggerBox.OnComponentBeginOverlap`
  (params (OverlappedComponent :type "PrimitiveComponent Object Reference") (OtherActor :type "Actor Object Reference") (OtherComp :type "PrimitiveComponent Object Reference") (OtherBodyIndex :type Integer) (bFromSweep :type Boolean) (SweepResult :type "HitResult Structure (by ref)"))
  (bind _returnvalue (`GameplayStatics.GetPlayerController` 0))
  (bind _returnvalue_2 (`KismetStringLibrary.Conv_IntToString` (`self.TimesHit`)))
  (if (`ActorComponent.ComponentHasTag` OtherComp "FireKiller")
    (if (>= (`self.TimesHit`) 10)
      (`self.ToggleALL_OFF`)
      (`GameplayStatics.PlaySound2D` "/Game/Art/Audio/SFX/Extinguish/PutOut_Cue.PutOut_Cue" 1.0 1.0 0.0 null null)
      (`KismetSystemLibrary.PrintString` _returnvalue_2)
      (`KismetSystemLibrary.Delay` 3.0)
      (set `self.TimesHit` 0)
      (`self.ToggleALL_OFF`)
      (message `/Game/Core/Interfaces/BPI_GameController.Freeze| UnFreeze FPS Pawn` _returnvalue false)
      (message `/Game/Core/Interfaces/BPI_GameController.ToggleSprayGun` _returnvalue)
      (message `/Game/Core/Interfaces/BPI_GameController.Set CanUseSpray` _returnvalue false)
      (`PrimitiveComponent.SetCollisionEnabled` (`/Game/Core/TrainingManager/BP_InteractiveWench.Collision` (`self.Wench Ref`)) "QueryOnly")
      (else
        (`/Engine/EditorBlueprintResources/StandardMacros.DoOnce` false :!label _label
          (:`Completed`
            (`self.Add HitCount`)
            (`GameplayStatics.PlaySound2D` "/Game/Art/Audio/SFX/Extinguish/PutOut_Cue.PutOut_Cue" 1.0 1.0 0.0 null null)
            (`KismetSystemLibrary.PrintString` _returnvalue_2)))))))

(event `self.TriggerBox.OnComponentEndOverlap`
  (params (OverlappedComponent :type "PrimitiveComponent Object Reference") (OtherActor :type "Actor Object Reference") (OtherComp :type "PrimitiveComponent Object Reference") (OtherBodyIndex :type Integer))
  (if (`ActorComponent.ComponentHasTag` OtherComp "FireKiller")
    (goto _label :!via `Reset`)))

(event `Add HitCount`
  (`/Engine/EditorBlueprintResources/StandardMacros.IncrementInt` (`self.TimesHit`)))

(fn `FinishedJetStream`
  (`NiagaraComponent.SetVariableFloat` (`self.NS_JetStream`) "Jet Flame Smoke SpawnRate" (`self.Jet Flame Smoke SpawnRate`))
  (`NiagaraComponent.SetVariableFloat` (`self.NS_JetStream`) "Skinny Jet Fire SpawnRate" (`self.Skinny Jet Fire SpawnRate`))
  (`NiagaraComponent.SetVariableFloat` (`self.NS_JetStream`) "Sparks SpawnRate" (`self.Sparks SpawnRate`)))

(fn `Set Niagra User Parameters`
  (`NiagaraComponent.SetVariableVec3` (`self.NS_JetStream`) "FlameVelocity" (0.0 0.0 0.0))
  (`NiagaraComponent.SetVariableFloat` (`self.NS_JetStream`) "SmokeASpawnRate" 10.0)
  (`NiagaraComponent.SetVariableFloat` (`self.NS_JetStream`) "SmokeBSpawnRate" 0.0)
  (`NiagaraComponent.SetVariableVec3` (`self.NS_JetStream`) "Smoke A Location" (`self.Phase 1 Smoke A Location`))
  (`NiagaraComponent.SetVariableVec3` (`self.NS_JetStream`) "Phase 1 Smoke B Location Inverse" (`self.Phase 1 Smoke B Location Inverse`))
  (`NiagaraComponent.SetVariableVec3` (`self.NS_JetStream`) "Phase 1 Smoke B Location" (`self.Phase 1 Smoke B Location`))
  (`NiagaraComponent.SetVariableFloat` (`self.NS_JetStream`) "Jet Flame Smoke SpawnRate" 0.0)
  (`NiagaraComponent.SetVariableFloat` (`self.NS_JetStream`) "Skinny Jet Fire SpawnRate" 0.0)
  (`NiagaraComponent.SetVariableFloat` (`self.NS_JetStream`) "Sparks SpawnRate" 0.0)
  (`NiagaraComponent.SetVariableVec2` (`self.NS_JetStream`) "Smoke A Scale" (0.0 0.0))
  (`NiagaraComponent.SetVariableVec3` (`self.NS_JetStream`) "ResidualFire Location" (`self.Residual Fire Location`))
  (`NiagaraComponent.SetVariableVec3` (`self.NS_JetStream`) "Residual BFire Location" (`self.Residual BFire Location`)))

(fn `ToggleNiagaraSystem`
  (params (NS_Tag :type Name) (`TurnOn?` :type Boolean))
  (for _array_element (`self.Out ActorsNiagaraSmokeAndFireParticlesArray`)
    (if (`self.ActorHasTag` _array_element NS_Tag)
      (if `TurnOn?`
        (bind _niagaracomponent (`NiagaraActor.NiagaraComponent` _array_element))
        (`ActorComponent.Activate` _niagaracomponent false)
        (else
          (`ActorComponent.Deactivate` _niagaracomponent))))))

(fn `Turn Off Niagara System`
  (`NiagaraComponent.SetVariableFloat` (`self.NS_JetStream`) "Jet Flame Smoke SpawnRate" 0.0)
  (`NiagaraComponent.SetVariableFloat` (`self.NS_JetStream`) "Skinny Jet Fire SpawnRate" 0.0)
  (`NiagaraComponent.SetVariableFloat` (`self.NS_JetStream`) "Sparks SpawnRate" 0.0)
  (`NiagaraComponent.SetVariableFloat` (`self.NS_JetStream`) "SmokeASpawnRate" 8.0)
  (`NiagaraComponent.SetVariableFloat` (`self.NS_JetStream`) "SmokeBSpawnRate" 0.0)
  (`NiagaraComponent.SetVariableVec3` (`self.NS_JetStream`) "FlameVelocity" (0.0 0.0 0.0)))

(fn `Turn On Niagara System`
  (`NiagaraComponent.SetVariableFloat` (`self.NS_JetStream`) "SmokeASpawnRate" (`self.Smoke A SpawnRate`))
  (`NiagaraComponent.SetVariableFloat` (`self.NS_JetStream`) "SmokeBSpawnRate" (`self.Smoke B SpawnRate`)))

(fn `UserConstructionScript`
  (`self.Set Niagra User Parameters`))