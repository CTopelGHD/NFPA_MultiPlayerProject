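; Blueprint that controls the thermal gun HUD, exposing events to show and hide it, update its temp text and toggle its back button.
; ShowUI swaps tagged fake-sky actors in and tagged decals out, collapses unit AI status UI, then phases in the game HUD's ThermalGunUI with UI-only input.
; HideUI phases the widget out and removes it after a short delay, without reverting those changes.
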(event `ToggleFakeSkyActors`
  (params (ToggleFakeSkyActors :type Boolean))
  (set `self.bToggleFakeSkyActors` ToggleFakeSkyActors)
  (bind _outactors (`GameplayStatics.GetAllActorsWithTag` "ThermalGunFakeSky"))
  (for _array_element _outactors
    (`self.SetActorHiddenInGame` _array_element (not (`self.bToggleFakeSkyActors`))))
  (bind _outactors_2 (`GameplayStatics.GetAllActorsOfClass` "/Script/Engine.DecalActor"))
  (for _array_element_2 _outactors_2
    (if (`ActorComponent.ComponentHasTag` (`DecalActor.Decal` _array_element_2) "ThermalGunFakeSky")
      (`self.SetActorHiddenInGame` _array_element_2 (`self.bToggleFakeSkyActors`)))))

(event `self.ReceiveBeginPlay`
  (bind _returnvalue (`GameplayStatics.GetActorOfClass` "/Game/Core/Systems/Pawns/FirstPerson/FPSPawn.FPSPawn_C"))
  (set `self.FPSPawn` _returnvalue))

(event `ShowUI`
  (`|ExecutionSequence`
    (:`then_0`
      (`self.ToggleFakeSkyActors` true)
      (bind _asgame_controller (cast `/Game/Core/Systems/Pawns/GameController` (`GameplayStatics.GetPlayerController` 0)))
      (`/Game/Core/Systems/Pawns/GameController.ToggleUnitAI_StatusUI_Visibility` _asgame_controller "Collapsed"))
    (:`then_1`
      (bind _wbp_gamehud (message `/Game/Core/Interfaces/BPI_GameController.GetWBP_GameHUD` (`GameplayStatics.GetPlayerController` 0)))
      (bind _thermalgunui (`/Game/UI/GameHUD/WBP_GameHUD.ThermalGunUI` _wbp_gamehud))
      (set `self.WBP_ThermalGunUI` _thermalgunui)
      (`Widget.SetVisibility` _thermalgunui "SelfHitTestInvisible")
      (`WidgetBlueprintLibrary.SetInputMode_UIOnlyEx` (`GameplayStatics.GetPlayerController` 0) _thermalgunui)
      (`/Game/UI/ThermalGun/ThermalGunUI.Phase IN` _thermalgunui))))

(event `HideUI`
  (bind _wbp_gamehud (message `/Game/Core/Interfaces/BPI_GameController.GetWBP_GameHUD` (`GameplayStatics.GetPlayerController` 0)))
  (bind _thermalgunui (`/Game/UI/GameHUD/WBP_GameHUD.ThermalGunUI` _wbp_gamehud))
  (`/Game/UI/ThermalGun/ThermalGunUI.Phase OUT` _thermalgunui)
  (`KismetSystemLibrary.Delay` 0.5)
  (`Widget.RemoveFromParent` _thermalgunui))

(event `SetTempTextValue`
  (params (InText :type Text))
  (`self.WBP_ThermalGunUI`
    (:`then`
      _)
    (:`else`
      (bind _wbp_gamehud (message `/Game/Core/Interfaces/BPI_GameController.GetWBP_GameHUD` (`GameplayStatics.GetPlayerController` 0)))
      (set `self.WBP_ThermalGunUI` (`/Game/UI/GameHUD/WBP_GameHUD.ThermalGunUI` _wbp_gamehud))))
  (`/Game/UI/ThermalGun/ThermalGunUI.UpdateTempText` (`self.WBP_ThermalGunUI`) InText))

(event `Enable Back Button`
  (`self.WBP_ThermalGunUI`
    (:`then`
      _)
    (:`else`
      (bind _wbp_gamehud (message `/Game/Core/Interfaces/BPI_GameController.GetWBP_GameHUD` (`GameplayStatics.GetPlayerController` 0)))
      (set `self.WBP_ThermalGunUI` (`/Game/UI/GameHUD/WBP_GameHUD.ThermalGunUI` _wbp_gamehud))))
  (`/Game/UI/ThermalGun/ThermalGunUI.Enable Back Button` (`self.WBP_ThermalGunUI`) true)
  (set `PlayerController.bShowMouseCursor` true (`GameplayStatics.GetPlayerController` 0)))

(event `Disable Back Button`
  (`self.WBP_ThermalGunUI`
    (:`then`
      _)
    (:`else`
      (bind _wbp_gamehud (message `/Game/Core/Interfaces/BPI_GameController.GetWBP_GameHUD` (`GameplayStatics.GetPlayerController` 0)))
      (set `self.WBP_ThermalGunUI` (`/Game/UI/GameHUD/WBP_GameHUD.ThermalGunUI` _wbp_gamehud))))
  (`/Game/UI/ThermalGun/ThermalGunUI.Enable Back Button` (`self.WBP_ThermalGunUI`) false))

(fn `UserConstructionScript`)