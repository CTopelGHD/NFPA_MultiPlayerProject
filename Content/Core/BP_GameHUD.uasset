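; BP_GameHUD manages which root UI is on screen, the main menu or the in-game HUD, based on the loaded level.
; On BeginPlay it creates both widgets, then runs InitOnLevelLoad after a short delay.
; InitOnLevelLoad clears both from the viewport, then shows and expands the menu on the main menu level, or shows the game HUD and collapses the menu elsewhere.
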(event `self.ReceiveBeginPlay`
  (`|ExecutionSequence`
    (:`then_0`
      (bind _returnvalue (`|CreateWidget` "/Game/UI/GameHUD/WBP_GameHUD.WBP_GameHUD_C"))
      (set `self.WBP_GameHUD` _returnvalue))
    (:`then_1`
      (bind _returnvalue_2 (`|CreateWidget` "/Game/UI/MainMenu/WBP_MainMenu.WBP_MainMenu_C"))
      (set `self.WBP_MainMenu` _returnvalue_2))
    (:`then_2`
      (`KismetSystemLibrary.Delay` 0.2)
      (`self.InitOnLevelLoad`))))

(event `InitOnLevelLoad`
  (bind _wbp_mainmenu (`self.WBP_MainMenu`))
  (bind _returnvalue (`GameplayStatics.GetCurrentLevelName` true))
  (`KismetSystemLibrary.PrintString` _returnvalue)
  (if (== _returnvalue "mainmenu")
    (`Widget.RemoveFromParent` (`self.WBP_GameHUD`))
    (`Widget.RemoveFromParent` (`self.WBP_MainMenu`))
    (`UserWidget.AddToViewport` _wbp_mainmenu 0)
    (`/Game/UI/MainMenu/WBP_MainMenu.ToggleMainMenu` _wbp_mainmenu "SelfHitTestInvisible")
    (else
      (`Widget.RemoveFromParent` (`self.WBP_GameHUD`))
      (`Widget.RemoveFromParent` (`self.WBP_MainMenu`))
      (`UserWidget.AddToViewport` (`self.WBP_GameHUD`) 0)
      (`/Game/UI/MainMenu/WBP_MainMenu.ToggleMainMenu` _wbp_mainmenu "Collapsed"))))

(fn `UserConstructionScript`)