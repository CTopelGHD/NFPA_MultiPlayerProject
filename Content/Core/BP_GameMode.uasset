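; Game mode that sets up per-player voice chat and player name display.
; On login it spawns a PlayerVoiceChatActor owned by the new player, with a random voice chat ID.
; In ResidentialHouses, after a short delay, it matches each FPSPawn to the game instance's PlayerInfoMap by the last digit of its display name, then shows that name to all.
; A separate event pushes the map back to the game instance.
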(event `self.ReceiveBeginPlay`
  (bind _returnvalue (`GameplayStatics.GetCurrentLevelName` true))
  (if (== _returnvalue "ResidentialHouses")
    (bind _asbp_game_instance (cast `/Game/Core/BP_GameInstance` (`GameplayStatics.GetGameInstance`)))
    (set `self.PlayerInfoMap` (`/Game/Core/BP_GameInstance.PlayerInfoMap` _asbp_game_instance))
    (`KismetSystemLibrary.Delay` 2.0)
    (bind _outactors (`GameplayStatics.GetAllActorsOfClass` "/Game/Core/Systems/Pawns/FirstPerson/FPSPawn.FPSPawn_C"))
    (for _array_element _outactors
      (bind _returnvalue_2 (`KismetSystemLibrary.GetDisplayName` _array_element))
      (bind (_value _returnvalue_3) (`BlueprintMapLibrary.Map_Find` (`self.PlayerInfoMap`) (`KismetStringLibrary.Conv_StringToInt` (`KismetStringLibrary.GetSubstring` _returnvalue_2 (- (`KismetArrayLibrary.Array_Length` (`KismetStringLibrary.GetCharacterArrayFromString` _returnvalue_2)) 1)))))
      (if _returnvalue_3
        (bind _asbp_game_instance_2 (cast `/Game/Core/BP_GameInstance` (`GameplayStatics.GetGameInstance`)))
        (set `/Game/Core/BP_GameInstance.PlayerInfoMap` (`self.PlayerInfoMap`) _asbp_game_instance_2)
        (`/Game/Core/Systems/Pawns/FirstPerson/FPSPawn.ShowPlayerNamesToAll` _array_element (`.Name_2_0C6571EF462395317E57F791C91F2B73` (break `/Game/Core/Data/PlayerInfo_Struct` _value)))))))

(event `self.K2_PostLogin`
  (params (NewPlayer :type "PlayerController Object Reference"))
  (`|SpawnActorFromClass` "/Script/UniversalVoiceChatPro.PlayerVoiceChatActor" (`KismetMathLibrary.MakeTransform` (0.0 0.0 0.0)) "AlwaysSpawn" "OverrideRootScale" NewPlayer (`KismetMathLibrary.RandomInteger` 100) "" false true true 1000.0 null))

(event `UpdateServerGameInstance`
  (bind _asbp_game_instance (cast `/Game/Core/BP_GameInstance` (`GameplayStatics.GetGameInstance`)))
  (`/Game/Core/BP_GameInstance.UpdatePlayerInfo` _asbp_game_instance (`self.PlayerInfoMap`)))

(fn `UserConstructionScript`)