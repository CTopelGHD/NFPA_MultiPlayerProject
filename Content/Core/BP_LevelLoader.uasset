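; BP_LevelLoader streams in either the Familiarization level or the EV garage fire scenario at startup, based on the game instance's module selection or a debug flag.
; Familiarization removes tagged actors and all decals and hides dispatch UI, while the fire scenario adds spray, shows dispatch text and disables the checklist.
; HousesUpdate streams house levels when realism or debug is on, otherwise removing high-graphics-only decals.
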(event `self.ReceiveBeginPlay`
  (bind _returnvalue (`GameplayStatics.GetPlayerController` 0))
  (`KismetSystemLibrary.Delay` 0.2)
  (bind _wbp_gamehud (message `/Game/Core/Interfaces/BPI_GameController.GetWBP_GameHUD` _returnvalue))
  (`WidgetBlueprintLibrary.SetInputMode_UIOnlyEx` _returnvalue (`/Game/UI/GameHUD/WBP_GameHUD.DispatchUI` _wbp_gamehud))
  (set `PlayerController.bShowMouseCursor` true _returnvalue)
  (if (`self.DebugFamLevel`)
    (`GameplayStatics.LoadStreamLevelBySoftObjectPtr` "/Game/Art/Levels/FamiliarizationLevel.FamiliarizationLevel" true :!label _label)
    (`self.Houses Update`)
    (`KismetSystemLibrary.Delay` 0.2)
    (bind _outactors (`GameplayStatics.GetAllActorsWithTag` "RemoveActorOnFamLevel"))
    (for _array_element _outactors
      (`self.K2_DestroyActor` _array_element))
    (`KismetSystemLibrary.Delay` 0.5)
    (bind _wbp_gamehud_2 (message `/Game/Core/Interfaces/BPI_GameController.GetWBP_GameHUD` (`GameplayStatics.GetPlayerController` 0)))
    (`/Game/UI/GameHUD/WBP_GameHUD.ToggleDispatchUI` _wbp_gamehud_2 false)
    (bind _outactors_2 (`GameplayStatics.GetAllActorsOfClass` "/Script/Engine.DecalActor"))
    (for _array_element_2 _outactors_2
      (`self.K2_DestroyActor` _array_element_2))
    (else
      (bind _moduleselected (message `/Game/Core/Interfaces/BPI_GameInstance.GetModuleSelection` (`GameplayStatics.GetGameInstance`)))
      (if (`KismetStringLibrary.Contains` (`KismetStringLibrary.Conv_NameToString` _moduleselected) "Familiarization")
        (goto _label)
        (else
          (`GameplayStatics.LoadStreamLevelBySoftObjectPtr` "/Game/Art/Levels/Scenario_EVFireInGarage.Scenario_EVFireInGarage" true)
          (`self.Houses Update`)
          (bind _wbp_gamehud_3 (message `/Game/Core/Interfaces/BPI_GameController.GetWBP_GameHUD` (`GameplayStatics.GetPlayerController` 0)))
          (`/Game/UI/GameHUD/WBP_GameHUD.ToggleDispatchUI` _wbp_gamehud_3 true)
          (`/Game/UI/Dispatch/DispatchUI.Show Dispatch Text` (`/Game/UI/GameHUD/WBP_GameHUD.DispatchUI` _wbp_gamehud_3))
          (`GameplayStatics.LoadStreamLevelBySoftObjectPtr` "/Game/Art/Levels/EVFireSpray.EVFireSpray" true)
          (message `/Game/Core/Interfaces/BPI_GameController.Set CanUseChecklist` (`GameplayStatics.GetPlayerController` 0) false))))))

(event `Houses Update`
  (bind _realism_ (message `/Game/Core/Interfaces/BPI_GameInstance.Get Realism` (`GameplayStatics.GetGameInstance`)))
  (if (or _realism_ (`self.DebugHousesOn?`))
    (`GameplayStatics.LoadStreamLevelBySoftObjectPtr` "/Game/ResidentialHouses/Maps/SubLevels/Houses.Houses" true)
    (`GameplayStatics.LoadStreamLevelBySoftObjectPtr` "/Game/ResidentialHouses/Maps/SubLevels/BackgroundHouses.BackgroundHouses" true)
    (else
      (bind _outactors (`GameplayStatics.GetAllActorsOfClass` "/Script/Engine.DecalActor"))
      (for _array_element _outactors
        (if (`ActorComponent.ComponentHasTag` (`DecalActor.Decal` _array_element) "HighGraphicsOnly")
          (`self.K2_DestroyActor` _array_element))))))

(fn `UserConstructionScript`)