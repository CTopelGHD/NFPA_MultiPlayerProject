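; HUD Blueprint that owns the main menu and in-game HUD widgets and switches the player between them.
; On BeginPlay it shows the menu with UI-only input and cursor, then after a short delay adds the game HUD hidden.
; ShiftTheHud takes a "MM" or "Game" string and toggles widget visibility, input mode and cursor to match.
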(event `self.ReceiveBeginPlay`
  (bind _returnvalue (`GameplayStatics.GetPlayerController` 0))
  (`|ExecutionSequence`
    (:`then_0`
      (bind _returnvalue_2 (`|CreateWidget` "/Game/UI/MainMenu/WBP_MainMenu.WBP_MainMenu_C" (`GameplayStatics.GetPlayerController` 0)))
      (bind _output_get (set `self.WBP_MainMenu` _returnvalue_2))
      (`WidgetBlueprintLibrary.SetInputMode_UIOnlyEx` _returnvalue null)
      (`UserWidget.AddToViewport` _output_get 0)
      (set `PlayerController.bShowMouseCursor` true _returnvalue))
    (:`then_1`
      (`KismetSystemLibrary.Delay` 0.2)
      (bind _returnvalue_3 (`|CreateWidget` "/Game/UI/GameHUD/WBP_GameHUD.WBP_GameHUD_C" (`GameplayStatics.GetPlayerController` 0)))
      (bind _output_get_2 (set `self.WBP_GameHUD` _returnvalue_3))
      (`Widget.SetVisibility` _output_get_2 "Hidden")
      (`UserWidget.AddToViewport` _output_get_2 0))))

(fn `Shift the Hud`
  (params (`MM/Game` :type String))
  (bind _returnvalue (`GameplayStatics.GetPlayerController` 0))
  (if (== `MM/Game` "MM")
    (`Widget.SetVisibility` (`self.WBP_GameHUD`) "Hidden")
    (`Widget.SetVisibility` (`self.WBP_MainMenu`) "Visible")
    (`WidgetBlueprintLibrary.SetInputMode_UIOnlyEx` _returnvalue (`self.WBP_MainMenu`))
    (set `PlayerController.bShowMouseCursor` true _returnvalue)
    (elif (== `MM/Game` "Game")
      (`Widget.SetVisibility` (`self.WBP_GameHUD`) "Visible")
      (`Widget.SetVisibility` (`self.WBP_MainMenu`) "Hidden")
      (`WidgetBlueprintLibrary.SetInputMode_GameOnly` _returnvalue)
      (set `PlayerController.bShowMouseCursor` false _returnvalue))))

(fn `UserConstructionScript`)