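; BP_ActivateFire is a level trigger actor that reveals a fire effect when the player enters its box.
; On BeginPlay it caches the BP_EVFire instance returned by GetActorOfClass, so it targets only one fire actor.
; Player pawn overlap makes that actor's NSJetStream component visible, and leaving the box never hides it.
; The construction script sizes the box from InBoxExtent plus a fixed padding.
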(event `self.ReceiveBeginPlay`
  (bind _returnvalue (`GameplayStatics.GetActorOfClass` "/Game/Art/VFX/JetFlame/BP_EVFire.BP_EVFire_C"))
  (set `self.BP_EVFire` _returnvalue))

(event `self.BoxCollision.OnComponentBeginOverlap`
  (params (OverlappedComponent :type "PrimitiveComponent Object Reference") (OtherActor :type "Actor Object Reference") (OtherComp :type "PrimitiveComponent Object Reference") (OtherBodyIndex :type Integer) (bFromSweep :type Boolean) (SweepResult :type "HitResult Structure (by ref)"))
  ;[1 1 1] Once hte fire is visibile, don't turn it off
  (if (== OtherActor (`GameplayStatics.GetPlayerPawn` 0))
    (`SceneComponent.SetVisibility` (`/Game/Art/VFX/JetFlame/BP_EVFire.NS_JetStream` (`self.BP_EVFire`)) true false)))

(event `self.BoxCollision.OnComponentEndOverlap`
  (params (OverlappedComponent :type "PrimitiveComponent Object Reference") (OtherActor :type "Actor Object Reference") (OtherComp :type "PrimitiveComponent Object Reference") (OtherBodyIndex :type Integer)))

(fn `UserConstructionScript`
  (`BoxComponent.SetBoxExtent` (`self.BoxCollision`) (+ (`self.In Box Extent`) (100.0 100.0 100.0)) true))