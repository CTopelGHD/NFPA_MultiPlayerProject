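; BP_DoorActionsTrigger is a trigger volume in the BackDoorSpray system that shows an interaction prompt for door actions.
; Box overlap sets InCollision, plays a notification sound, toggles an indicator arrow on and phases in the interactive UI.
; End overlap or a CloseOut event clears the flag and arrow, phases the UI out, then hides it after a short delay.
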(event `self.ReceiveBeginPlay`
  (`parent.ReceiveBeginPlay`))

(event `self.BoxCollision.OnComponentBeginOverlap`
  (params (OverlappedComponent :type "PrimitiveComponent Object Reference") (OtherActor :type "Actor Object Reference") (OtherComp :type "PrimitiveComponent Object Reference") (OtherBodyIndex :type Integer) (bFromSweep :type Boolean) (SweepResult :type "HitResult Structure (by ref)"))
  (set `self.InCollision?` true)
  (`GameplayStatics.PlaySound2D` "/Game/Art/Audio/UI/DescriptorNotification.DescriptorNotification" 1.0 1.0 0.0 null null)
  (`SceneComponent.SetVisibility` (`self.InteractiveUI`) true false)
  (`/Game/UI/InteractiveUI/WBP_InteractiveUI.Phase IN` (`self.WBP_InteractiveUI`))
  (`self.ToggleIndicatorArrowOnInteract` true))

(event `self.BoxCollision.OnComponentEndOverlap`
  (params (OverlappedComponent :type "PrimitiveComponent Object Reference") (OtherActor :type "Actor Object Reference") (OtherComp :type "PrimitiveComponent Object Reference") (OtherBodyIndex :type Integer))
  (`self.ToggleIndicatorArrowOnInteract` false :!label _label)
  (set `self.InCollision?` false)
  (`/Game/UI/InteractiveUI/WBP_InteractiveUI.Phase OUT` (`self.WBP_InteractiveUI`))
  (`KismetSystemLibrary.Delay` 0.5)
  (`SceneComponent.SetVisibility` (`self.InteractiveUI`) false false))

(event `Close Out`
  (goto _label))

(fn `UserConstructionScript`
  (`parent.UserConstructionScript`))