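; Trigger actor for the garage back door spray task, where the player repeatedly sprays a steaming, cracked door until it opens.
; Each FireKiller overlap adds one hit to the HUD counter, with a DoOnce reset on end overlap.
; An overlap after ten hits stops the steam, updates player state through controller messages and swings the tagged door open via timeline.
; When the door finishes, it enables the EV fire's trigger boxes.
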(event `self.Spray Trigger.OnComponentBeginOverlap`
  (params (OverlappedComponent :type "PrimitiveComponent Object Reference") (OtherActor :type "Actor Object Reference") (OtherComp :type "PrimitiveComponent Object Reference") (OtherBodyIndex :type Integer) (bFromSweep :type Boolean) (SweepResult :type "HitResult Structure (by ref)"))
  (bind _returnvalue (`GameplayStatics.GetPlayerController` 0))
  (if (`ActorComponent.ComponentHasTag` OtherComp "FireKiller")
    (if (>= (`self.DoorTimesHit`) 10)
      (message `/Game/Core/Interfaces/BPI_GameController.Set Cracked Door Sprayed?` (`GameplayStatics.GetPlayerController` 0) true)
      (`self.Steam On/Off` false)
      (`PrimitiveComponent.SetCollisionEnabled` (`self.Spray Trigger`) "NoCollision")
      (`GameplayStatics.PlaySound2D` "/Game/Art/Audio/SFX/Extinguish/PutOut_Cue.PutOut_Cue" 1.0 1.0 0.0 null null)
      (bind _wbp_gamehud (message `/Game/Core/Interfaces/BPI_GameController.GetWBP_GameHUD` (`GameplayStatics.GetPlayerController` 0)))
      (bind _wbp_spraycountui (`/Game/UI/GameHUD/WBP_GameHUD.WBP_SprayCountUI` _wbp_gamehud))
      (`/Game/UI/SprayCountUI/WBP_SprayCountUI.Door Close Out` _wbp_spraycountui)
      (`self.Move Door to Full Open`)
      (`KismetSystemLibrary.Delay` 2.1)
      (`Widget.SetVisibility` _wbp_spraycountui "Collapsed")
      (message `/Game/Core/Interfaces/BPI_GameController.Turn Off SprayGun` _returnvalue)
      (message `/Game/Core/Interfaces/BPI_GameController.Set CanUseSpray` _returnvalue false)
      (message `/Game/Core/Interfaces/BPI_GameController.Freeze| UnFreeze FPS Pawn` _returnvalue false)
      (else
        (`/Engine/EditorBlueprintResources/StandardMacros.DoOnce` false :!label _label
          (:`Completed`
            (`self.Add Door Spray Count`)
            (`GameplayStatics.PlaySound2D` "/Game/Art/Audio/SFX/Extinguish/PutOut_Cue.PutOut_Cue" 1.0 1.0 0.0 null null)))))))

(event `self.Spray Trigger.OnComponentEndOverlap`
  (params (OverlappedComponent :type "PrimitiveComponent Object Reference") (OtherActor :type "Actor Object Reference") (OtherComp :type "PrimitiveComponent Object Reference") (OtherBodyIndex :type Integer))
  (if (`ActorComponent.ComponentHasTag` OtherComp "FireKiller")
    (goto _label :!via `Reset`)))

(event `Add Door Spray Count`
  (bind _wbp_gamehud (message `/Game/Core/Interfaces/BPI_GameController.GetWBP_GameHUD` (`GameplayStatics.GetPlayerController` 0)))
  (bind _result (`/Engine/EditorBlueprintResources/StandardMacros.IncrementInt` (`self.DoorTimesHit`))
    (:`  `
      (`/Game/UI/SprayCountUI/WBP_SprayCountUI.Set Door Spray Score` (`/Game/UI/GameHUD/WBP_GameHUD.WBP_SprayCountUI` _wbp_gamehud) _result))))

(event `Move Door to Full Open`
  (bind _outactors (`GameplayStatics.GetAllActorsOfClassWithTag` "/Script/Engine.Actor" "Garage BackDoor"))
  (bind (_direction _lerp) (`Timeline|Rotate`)
    (:`Update`
      (bind _output (`|GetArrayItem` _outactors))
      (`self.K2_SetActorRelativeRotation` _output (`KismetMathLibrary.RLerp` (`self.K2_GetActorRotation` _output) (struct :`Yaw` -15.0) _lerp) false false))
    (:`Finished`
      (message `/Game/Core/Interfaces/BPI_GameController.Set Back GarageDoor Opened?` (`GameplayStatics.GetPlayerController` 0) true)
      (`self.Turn On EVFire Triggers`))))

(event `Turn On EVFire Triggers`
  (bind _outactors (`GameplayStatics.GetAllActorsOfClass` "/Game/Art/VFX/JetFlame/BP_EVFire.BP_EVFire_C"))
  (bind _output (`|GetArrayItem` _outactors))
  (`/Game/Art/VFX/JetFlame/BP_EVFire.Collision Control` _output (`/Game/Art/VFX/JetFlame/BP_EVFire.EVTriggerBox` _output) "QueryOnly")
  (`/Game/Art/VFX/JetFlame/BP_EVFire.Collision Control` _output (`/Game/Art/VFX/JetFlame/BP_EVFire.ESS_TriggerBox` _output) "QueryOnly"))

(fn `Steam On/Off`
  (params (`On?` :type Boolean))
  (bind _steam (`self.Steam`))
  (if `On?`
    (`ActorComponent.Activate` _steam false)
    (else
      (`ActorComponent.Deactivate` _steam))))

(fn `UserConstructionScript`)