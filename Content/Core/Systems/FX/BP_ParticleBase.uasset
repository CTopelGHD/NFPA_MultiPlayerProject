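; BP_ParticleBase is a base particle effect actor with recolorable fire, smoke, ember and spark colors.
; Its construction script pushes the color variables into matching named color parameters on the ParticleSystem component, including two separate fire colors.
; The event graph holds only disabled placeholder events, so the actor runs no gameplay logic of its own.
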(fn `UserConstructionScript`
  (bind _particlesystem (`self.ParticleSystem`))
  (`FXSystemComponent.SetColorParameter` _particlesystem "FireColor" (`self.FireColor`))
  (`FXSystemComponent.SetColorParameter` _particlesystem "FireColor2" (`self.FireColor2`))
  (`FXSystemComponent.SetColorParameter` _particlesystem "SmokeColor" (`self.SmokeColor`))
  (`FXSystemComponent.SetColorParameter` _particlesystem "EmberColor" (`self.EmberColor`))
  (`FXSystemComponent.SetColorParameter` _particlesystem "SparksColor" (`self.SparksColor`)))