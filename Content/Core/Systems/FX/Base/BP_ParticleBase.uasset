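; BP_ParticleBase is a configurable effect actor that displays one of five particle presets: fire, smoke, sparks, dandelion or shot shockwave.
; Its Construction Script branches on the PEnumerator selection to set the ParticleSystem component's template.
; Each branch then pushes color variables into that template's named color parameters, except dandelion, which sets a fixed black FireColor.
; The event graph holds no active logic.
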(fn `UserConstructionScript`
  (bind _particlesystem (`self.ParticleSystem`))
  (bind _particlesystem_2 (`self.ParticleSystem`))
  (bind _particlesystem_3 (`self.ParticleSystem`))
  (bind _particlesystem_4 (`self.ParticleSystem`))
  (bind _penumerator (`self.PEnumerator`))
  (if (`|EnumEquality` _penumerator "NewEnumerator0")
    (`ParticleSystemComponent.SetTemplate` _particlesystem "/Game/Core/Systems/FX/Fire/P_Fire.P_Fire")
    (`FXSystemComponent.SetColorParameter` _particlesystem "FireColor" (`self.FireColor`))
    (`FXSystemComponent.SetColorParameter` _particlesystem "FireColor2" (`self.FireColor2`))
    (`FXSystemComponent.SetColorParameter` _particlesystem "SmokeColor" (`self.SmokeColor`))
    (`FXSystemComponent.SetColorParameter` _particlesystem "EmberColor" (`self.EmberColor`))
    (`FXSystemComponent.SetColorParameter` _particlesystem "SparksColor" (`self.SparksColor`))
    (elif (`|EnumEquality` _penumerator "NewEnumerator1")
      (`ParticleSystemComponent.SetTemplate` _particlesystem "/Game/Core/Systems/FX/Smoke/P_Smoke.P_Smoke")
      (`FXSystemComponent.SetColorParameter` _particlesystem "SmokeColor" (`self.SmokeColor`))
      (elif (`|EnumEquality` _penumerator "NewEnumerator2")
        (`ParticleSystemComponent.SetTemplate` _particlesystem_4 "/Game/Core/Systems/FX/Electricity/P_Sparks.P_Sparks")
        (`FXSystemComponent.SetColorParameter` _particlesystem_4 "SparkColor" (`self.SparkColor`))
        (`FXSystemComponent.SetColorParameter` _particlesystem_4 "SparkSmokeColor" (`self.SparkSmokeColor`))
        (elif (`|EnumEquality` _penumerator "NewEnumerator3")
          (`ParticleSystemComponent.SetTemplate` _particlesystem_3 "/Game/Core/Systems/FX/Wind/Particles_Wind_Control_System/Blueprints/Components/Particles/P_Dandelion.P_Dandelion")
          (`FXSystemComponent.SetColorParameter` :`self` _particlesystem_3 :`ParameterName` "FireColor")
          (elif (`|EnumEquality` _penumerator "NewEnumerator4")
            (`ParticleSystemComponent.SetTemplate` _particlesystem_2 "/Game/Core/Systems/FX/Hit/P_ky_shotShockwave.P_ky_shotShockwave")
            (`FXSystemComponent.SetColorParameter` _particlesystem_2 "LightColor" (`self.LightColor`))))))))