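; BP_InteractiveHose is a training-level interaction point that shows a "Press F to Interact" widget when the local player enters its box.
; Overlap begin plays a sound, fades the prompt in and removes the indicator arrow unless set to always show; overlap end or CloseOut reverses this.
; Events switch indicator visibility modes, and construction applies box extent, height offset and tag.
; Sending the training-step tag message is unwired, and no input is handled here.
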(event `self.ReceiveBeginPlay`
  (`|ExecutionSequence`
    (:`then_0`
      (bind _returnvalue (`|CreateWidget` "/Game/UI/InteractiveUI/WBP_InteractiveUI.WBP_InteractiveUI_C" (`GameplayStatics.GetPlayerController` 0)))
      (bind _output_get (set `self.InteractiveUI Ref` _returnvalue))
      (`WidgetComponent.SetWidget` (`self.InteractiveUI`) _output_get))
    (:`then_1`
      (`/Game/UI/InteractiveUI/WBP_InteractiveUI.SetText` (`self.InteractiveUI Ref`) (`self.Title Text`) "Press \"F\" to Interact"))))

(event `self.Collision.OnComponentBeginOverlap`
  (params (OverlappedComponent :type "PrimitiveComponent Object Reference") (OtherActor :type "Actor Object Reference") (OtherComp :type "PrimitiveComponent Object Reference") (OtherBodyIndex :type Integer) (bFromSweep :type Boolean) (SweepResult :type "HitResult Structure (by ref)"))
  (if (== (`self.GetOwner` OtherActor) (`GameplayStatics.GetPlayerController` 0))
    (set `self.InCollision?` true)
    (`GameplayStatics.PlaySound2D` "/Game/Art/Audio/UI/DescriptorNotification.DescriptorNotification" 1.0 1.0 0.0 null null)
    (`SceneComponent.SetVisibility` (`self.InteractiveUI`) true false)
    (`/Game/UI/InteractiveUI/WBP_InteractiveUI.Phase IN` (`self.InteractiveUI Ref`))
    (`self.Show/Hide Arrow` true)))

(event `self.Collision.OnComponentEndOverlap`
  (params (OverlappedComponent :type "PrimitiveComponent Object Reference") (OtherActor :type "Actor Object Reference") (OtherComp :type "PrimitiveComponent Object Reference") (OtherBodyIndex :type Integer))
  (if (== (`self.GetOwner` OtherActor) (`GameplayStatics.GetPlayerController` 0))
    (if (`self.InCollision?`)
      (`self.Show/Hide Arrow` false)
      (set `self.InCollision?` false :!label _label)
      (`/Game/UI/InteractiveUI/WBP_InteractiveUI.Phase OUT` (`self.InteractiveUI Ref`))
      (`KismetSystemLibrary.Delay` 0.5)
      (`SceneComponent.SetVisibility` (`self.InteractiveUI`) false false))))

(event `Close Out`
  (goto _label))

(event `ToggleIndicatorToAlwaysShow`
  (set `/Game/IndicatorComponent/BP/BP_IndicatorComponent.DistanceVisibilityMethod` "NewEnumerator0" (`self.BP_IndicatorComponent`)))

(event `ToggleIndicatorToShowOnlyAtDistance`
  (set `/Game/IndicatorComponent/BP/BP_IndicatorComponent.DistanceVisibilityMethod` "NewEnumerator1" (`self.BP_IndicatorComponent`)))

(event `ToggleIndicatorVisibility`
  (params (bVisibility :type Boolean))
  (bind _bp_indicatorcomponent (`self.BP_IndicatorComponent`))
  (if bVisibility
    (set `/Game/IndicatorComponent/BP/BP_IndicatorComponent.ShowIndicatorMethod` "NewEnumerator0" _bp_indicatorcomponent)
    (set `/Game/IndicatorComponent/BP/BP_IndicatorComponent.ShowDistanceMethod` "NewEnumerator2" _bp_indicatorcomponent)
    (else
      (set `/Game/IndicatorComponent/BP/BP_IndicatorComponent.ShowIndicatorMethod` "NewEnumerator3" _bp_indicatorcomponent)
      (set `/Game/IndicatorComponent/BP/BP_IndicatorComponent.ShowDistanceMethod` "NewEnumerator3" _bp_indicatorcomponent))))

(fn `Show/Hide Arrow`
  (params (`Hide?` :type Boolean))
  (bind _bp_indicatorcomponent (`self.BP_IndicatorComponent`))
  (if `Hide?`
    (if (not (`self.AlwaysShowIndicatorArrow`))
      (`/Game/IndicatorComponent/BP/BP_IndicatorComponent.RemoveFromViewport` _bp_indicatorcomponent))
    (else
      (`/Game/IndicatorComponent/BP/BP_IndicatorComponent.AddToViewport` _bp_indicatorcomponent))))

(fn `UserConstructionScript`
  (bind _collision (`self.Collision`))
  (bind _tags (`self.Tags`))
  (`BoxComponent.SetBoxExtent` _collision (+ (`BoxComponent.BoxExtent` _collision) (`self.In Box Extent`)) true)
  (`SceneComponent.K2_SetRelativeLocation` (`self.Billboard`) (`KismetMathLibrary.MakeVector` 0.0 0.0 (`self.Interactive Z Offset`)) false false)
  (`KismetArrayLibrary.Array_Clear` _tags)
  (`/Engine/EditorBlueprintResources/StandardMacros.DoOnce` false
    (:`Completed`
      (`KismetArrayLibrary.Array_Add` _tags (`self.Tag`)))))