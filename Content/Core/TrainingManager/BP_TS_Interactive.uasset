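; Training-step interactive actor with a trigger box, prompt widget and indicator arrow.
; Local player overlap shows the prompt and sends the step tag to the controller, while AI pawn overlap starts the interaction directly.
; Interacting locks input, hides the pawn and plays a Level Sequence, optionally reversible or with X-ray vision or sound.
; Delayed completion restores control, swaps tagged actors' visibility and collision, and notifies BP_TrainingTracker.
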(event `self.ReceiveBeginPlay`
  (`|ExecutionSequence`
    (:`then_0`
      (bind _returnvalue (`|CreateWidget` "/Game/UI/InteractiveUI/WBP_InteractiveUI.WBP_InteractiveUI_C" (`GameplayStatics.GetPlayerController` 0)))
      (bind _output_get (set `self.WBP_InteractiveUI` _returnvalue))
      (`WidgetComponent.SetWidget` (`self.InteractiveUI`) _output_get))
    (:`then_1`
      (bind _returnvalue_2 (`GameplayStatics.GetActorOfClass` "/Game/Core/BP_GameHUD.BP_GameHUD_C"))
      (set `self.BP_GameHUD` _returnvalue_2)
      (bind _outactors (`GameplayStatics.GetAllActorsOfClass` "/Game/Core/Systems/XRayVision/XRayVisionPostProcessVolume_Blueprint.XRayVisionPostProcessVolume_Blueprint_C"))
      (set `self.XRay Vision PP Ref` (`|GetArrayItem` _outactors)))
    (:`then_2`
      (`KismetSystemLibrary.Delay` 3.0)
      (`/Game/UI/InteractiveUI/WBP_InteractiveUI.SetText` (`self.WBP_InteractiveUI`) (`self.Title Text`) (`self.PressResultText`))
      (bind (_outactor _returnvalue_3) (`LevelSequencePlayer.CreateLevelSequencePlayer` (`self.Level Sequence`)))
      (set `self.CurrentLevelSequence` _returnvalue_3))
    (:`then_3`
      (bind _returnvalue_4 (`GameplayStatics.GetActorOfClass` "/Game/Core/TrainingManager/BP_TrainingTracker.BP_TrainingTracker_C"))
      (set `self.BP_TrainingTracker` _returnvalue_4))
    (:`then_4`
      (bind _outactors_2 (`GameplayStatics.GetAllActorsOfClassWithTag` "/Game/Core/Systems/Pawns/FirstPerson/M_Pawn.M_Pawn_C" "AI_Pawn"))
      (set `self.AI_Pawns` _outactors_2))
    (:`then_5`
      (set `PrimitiveComponent.bGenerateOverlapEvents` (`self.OverrideGenerate Overlap Events`) (`self.BoxCollision`))
      (`self.ToggleIndicatorAddToViewport` (`self.RunParentOverlap`)))))

(event `StartInteractiveUI`
  (if (`self.InteractionCompleted?`)
    _
    (elif (not (`self.AlreadyActivated?`))
      (set `self.InCollision?` true)
      (`GameplayStatics.PlaySound2D` "/Game/Art/Audio/UI/DescriptorNotification.DescriptorNotification" 1.0 1.0 0.0 null null)
      (message `/Game/Core/Interfaces/BPI_GameController.SendTrainingStepInteractiveTagID` (`GameplayStatics.GetPlayerController` 0) (`|GetArrayItem` (`self.Tags`)))
      (`self.ToggleInteraction_OwningClient`))))

(event `CheckCollisionWithInteractive`
  (params (AI_Pawn :type "Object Object Reference"))
  (set `self.IsAiInCollision?` false :!label _label)
  (for _array_element (`self.AI_Pawns`)
    (if (or (== (stale `self.BoxCollision.OnComponentBeginOverlap` OtherActor) _array_element) (== _array_element AI_Pawn))
      (set `self.IsAiInCollision?` true)
      (break)))
  (if (`self.IsAiInCollision?`)
    (`self.StartInteractiveUI`)))

(event `OpenCollision`
  (`PrimitiveComponent.SetCollisionEnabled` (`self.BoxCollision`) "QueryOnly"))

(event `self.BoxCollision.OnComponentBeginOverlap`
  (params (OverlappedComponent :type "PrimitiveComponent Object Reference") (OtherActor :type "Actor Object Reference") (OtherComp :type "PrimitiveComponent Object Reference") (OtherBodyIndex :type Integer) (bFromSweep :type Boolean) (SweepResult :type "HitResult Structure (by ref)"))
  (if (`self.RunParentOverlap`)
    (if (== (`self.GetOwner` OtherActor) (`GameplayStatics.GetPlayerController` 0))
      (`/Engine/EditorBlueprintResources/StandardMacros.DoOnce` false :!label _label_2
        (:`Completed`
          (if (`self.InteractionCompleted?`)
            _
            (elif (not (`self.AlreadyActivated?`))
              (set `self.InCollision?` true)
              (`GameplayStatics.PlaySound2D` "/Game/Art/Audio/UI/DescriptorNotification.DescriptorNotification" 1.0 1.0 0.0 null null)
              (`SceneComponent.SetVisibility` (`self.InteractiveUI`) true false)
              (`/Game/UI/InteractiveUI/WBP_InteractiveUI.Phase IN` (`self.WBP_InteractiveUI`))
              (message `/Game/Core/Interfaces/BPI_GameController.SendTrainingStepInteractiveTagID` (`GameplayStatics.GetPlayerController` 0) (`|GetArrayItem` (`self.Tags`)))
              (goto _label_3 :!via `Reset`)))))
      (else
        (goto _label)))))

(event `self.BoxCollision.OnComponentEndOverlap`
  (params (OverlappedComponent :type "PrimitiveComponent Object Reference") (OtherActor :type "Actor Object Reference") (OtherComp :type "PrimitiveComponent Object Reference") (OtherBodyIndex :type Integer))
  (if (`self.RunParentOverlap`)
    (if (== (`self.GetOwner` OtherActor) (`GameplayStatics.GetPlayerController` 0))
      (`/Engine/EditorBlueprintResources/StandardMacros.DoOnce` true :!label _label_3
        (:`Completed`
          (set `self.InCollision?` false)
          (`/Game/UI/InteractiveUI/WBP_InteractiveUI.Phase OUT` (`self.WBP_InteractiveUI`))
          (`KismetSystemLibrary.Delay` 0.5)
          (`SceneComponent.SetVisibility` (`self.InteractiveUI`) false false)
          (message `/Game/Core/Interfaces/BPI_GameController.SendTrainingStepInteractiveTagID` (`GameplayStatics.GetPlayerController` 0) "None")
          (if (not (`self.InteractionCompleted?`))
            (goto _label_2 :!via `Reset`)))))))

(event `CloseCollision`
  (`PrimitiveComponent.SetCollisionEnabled` (`self.BoxCollision`) "NoCollision")
  (`/Game/UI/InteractiveUI/WBP_InteractiveUI.Phase OUT` (`self.WBP_InteractiveUI`))
  (`KismetSystemLibrary.Delay` 0.5)
  (`SceneComponent.SetVisibility` (`self.InteractiveUI`) false false))

(event `ToggleInteraction_OwningClient`
  (bind _returnvalue (`GameplayStatics.GetPlayerController` 0))
  (bind _currentlevelsequence (`self.CurrentLevelSequence`))
  (message `/Game/Core/Interfaces/BPI_Pawn.TogglePawnVisibility` (`GameplayStatics.GetPlayerPawn` 0) false)
  (`self.DisableInput` _returnvalue _returnvalue)
  (`self.DisableInput` (`GameplayStatics.GetPlayerPawn` 0) _returnvalue)
  (`self.ToggleIndicatorArrowOnInteract` true)
  (`self.CloseCollision`)
  (`self.CurrentLevelSequence`
    (:`then`
      (if (`self.IsThere a LS Animation`)
        (if (`self.PlayReverse?`)
          ;[1 1 1] Backward
          (`MovieSceneSequencePlayer.PlayReverse` _currentlevelsequence)
          (set `self.PlayReverse?` false)
          (`KismetSystemLibrary.Delay` (`self.Interaction Delay`) :!label _label_4)
          (`self.OpenCollision` :!label _label_5)
          (`self.OnCompletion`)
          (else
            (`KismetSystemLibrary.PrintString` (`KismetSystemLibrary.GetDisplayName` _currentlevelsequence) true true (struct :`G` 0.66 :`B` 1.0 :`A` 1.0) 50.0)
            ;[1 1 1] Forward
            (`MovieSceneSequencePlayer.Play` _currentlevelsequence)
            (if (`self.X-Ray?`)
              (`/Game/Core/Systems/XRayVision/XRayVisionPostProcessVolume_Blueprint.Xray Execution` (`self.XRay Vision PP Ref`))
              (`KismetSystemLibrary.Delay` (`self.Interaction Delay`))
              (`/Game/Core/Systems/XRayVision/XRayVisionPostProcessVolume_Blueprint.Xray Execution` (`self.XRay Vision PP Ref`)))
            (if (`self.ActivateOnce?`)
              (if (not (`self.X-Ray?`))
                (`KismetSystemLibrary.Delay` (`self.Interaction Delay`)))
              (`self.OnCompletion`)
              (else
                (set `self.PlayReverse?` true)
                (if (`self.X-Ray?`)
                  (goto _label_5)
                  (else
                    (goto _label_4)))))))
        (else
          (if (`self.InteractionCompleted?`)
            (`KismetSystemLibrary.PrintString` (`KismetStringLibrary.Concat_StrStr` "Warning:" (`KismetSystemLibrary.GetDisplayName` self) " interaction has already completed!"))
            (else
              (`MovieSceneSequencePlayer.Play` (`self.CurrentLevelSequence`))
              (bind _sound (`self.Sound`)
                (:`then`
                  (`GameplayStatics.PlaySound2D` _sound 1.0 1.0 0.0 null null)
                  (`KismetSystemLibrary.Delay` (`self.Interaction Delay`)))
                (:`else`
                  (`KismetSystemLibrary.PrintString` (`KismetStringLibrary.Concat_StrStr` "Warning:" (`KismetSystemLibrary.GetDisplayName` _sound) " did not play in " (`KismetSystemLibrary.GetDisplayName` self) "."))))))
          (`self.OnCompletion`))))
    (:`else`)))

(event `ToggleInteraction_RemoteClient`
  (`KismetSystemLibrary.Delay` (`self.Interaction Delay`))
  (`self.OnCompletion`))

(event `OnCompletionAI`
  (`self.TryActorsOnCompletion` :!label _label_6)
  (bind _bp_trainingtracker (`self.BP_TrainingTracker`)
    (:`then`
      _)
    (:`else`
      (bind _returnvalue (`GameplayStatics.GetActorOfClass` "/Game/Core/TrainingManager/BP_TrainingTracker.BP_TrainingTracker_C"))
      (set `self.BP_TrainingTracker` _returnvalue)))
  (`/Game/Core/TrainingManager/BP_TrainingTracker.OnInteractComplete` _bp_trainingtracker (`|GetArrayItem` (`self.Tags`)))
  (if (`self.ActivateOnce?`)
    (set `self.AlreadyActivated?` true)
    (bind _output_get (set `self.OverrideGenerate Overlap Events` false))
    (`self.ToggleIndicatorAddToViewport` _output_get)))

(event `OnCompletion`
  (message `/Game/Core/Interfaces/BPI_Pawn.TogglePawnVisibility` (`GameplayStatics.GetPlayerPawn` 0) true)
  (bind _asgame_controller (cast `/Game/Core/Systems/Pawns/GameController` (`GameplayStatics.GetPlayerController` 0)))
  (`/Game/Core/Systems/Pawns/GameController.Toggle All Indicators Visibility` _asgame_controller true)
  (`self.EnableInput` (`GameplayStatics.GetPlayerPawn` 0) (`GameplayStatics.GetPlayerController` 0))
  (`self.EnableInput` (`GameplayStatics.GetPlayerController` 0) (`GameplayStatics.GetPlayerController` 0))
  (set `self.InteractionCompleted?` true)
  (goto _label_6))

(event `TryActorsOnCompletion`
  (`KismetSystemLibrary.PrintString` "TryActors")
  (for _array_element (`self.ActorTagsBeforeCompletion`)
    (bind _outactors (`GameplayStatics.GetAllActorsWithTag` _array_element))
    (for _array_element_2 _outactors
      (`self.SetActorHiddenInGame` _array_element_2 true)
      (`self.SetActorEnableCollision` _array_element_2 false)))
  (for _array_element_3 (`self.ActorTagsAfterCompletion`)
    (bind _outactors_2 (`GameplayStatics.GetAllActorsWithTag` _array_element_3))
    (for _array_element_4 _outactors_2
      (`self.SetActorHiddenInGame` _array_element_4 false)
      (`self.SetActorEnableCollision` _array_element_4 true))))

(event `ToggleIndicatorToAlwaysShow`
  (set `/Game/IndicatorComponent/BP/BP_IndicatorComponent.DistanceVisibilityMethod` "NewEnumerator0" (`self.BP_IndicatorComponent`)))

(event `ToggleIndicatorToShowOnlyAtDistance`
  (set `/Game/IndicatorComponent/BP/BP_IndicatorComponent.DistanceVisibilityMethod` "NewEnumerator1" (`self.BP_IndicatorComponent`)))

(fn `OnRep_InteractionCompleted?`
  (`KismetSystemLibrary.PrintString` "RepCompleted Notify"))

(fn `ToggleIndicatorAddToViewport`
  (params (Condition :type Boolean))
  (bind _bp_indicatorcomponent (`self.BP_IndicatorComponent`))
  (if Condition
    (`/Game/IndicatorComponent/BP/BP_IndicatorComponent.AddToViewport` _bp_indicatorcomponent)
    (else
      (`/Game/IndicatorComponent/BP/BP_IndicatorComponent.RemoveFromViewport` _bp_indicatorcomponent))))

(fn `ToggleIndicatorArrowOnInteract`
  (params (`Hide?` :type Boolean))
  (bind _bp_indicatorcomponent (`self.BP_IndicatorComponent`))
  (if `Hide?`
    (if (not (`self.AlwaysShowIndicatorArrow`))
      (`/Game/IndicatorComponent/BP/BP_IndicatorComponent.RemoveFromViewport` _bp_indicatorcomponent))
    (else
      (`/Game/IndicatorComponent/BP/BP_IndicatorComponent.AddToViewport` _bp_indicatorcomponent))))

(fn `ToggleIndicatorVisibility`
  (params (bVisibility :type Boolean))
  (bind _bp_indicatorcomponent (`self.BP_IndicatorComponent`))
  (if bVisibility
    (set `/Game/IndicatorComponent/BP/BP_IndicatorComponent.ShowIndicatorMethod` "NewEnumerator0" _bp_indicatorcomponent)
    (set `/Game/IndicatorComponent/BP/BP_IndicatorComponent.ShowDistanceMethod` "NewEnumerator2" _bp_indicatorcomponent)
    (else
      (set `/Game/IndicatorComponent/BP/BP_IndicatorComponent.ShowIndicatorMethod` "NewEnumerator3" _bp_indicatorcomponent)
      (set `/Game/IndicatorComponent/BP/BP_IndicatorComponent.ShowDistanceMethod` "NewEnumerator3" _bp_indicatorcomponent))))

(fn `UserConstructionScript`
  (bind _boxcollision (`self.BoxCollision`))
  (bind _tags (`self.Tags`))
  (`BoxComponent.SetBoxExtent` _boxcollision (+ (`BoxComponent.BoxExtent` _boxcollision) (`self.In Box Extent`)) true)
  (`SceneComponent.K2_SetRelativeLocation` (`self.Billboard`) (`KismetMathLibrary.MakeVector` 0.0 0.0 (`self.Interactive Z Offset`)) false false)
  (`KismetArrayLibrary.Array_Clear` _tags)
  (`/Engine/EditorBlueprintResources/StandardMacros.DoOnce` false
    (:`Completed`
      (`KismetArrayLibrary.Array_Add` _tags (`self.ID Tag`)))))