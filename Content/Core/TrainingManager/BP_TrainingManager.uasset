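; BP_TrainingManager is a training manager that gathers the level actors relevant to a training session.
; On BeginPlay it looks up actors for each tag in the interactable and descriptive tag lists.
; Both sets are appended into the single InteractableActors array, interactable ones first.
; An unconnected fragment for setting CurrentSequenceActor from that array never runs, so no sequence stepping happens here.
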(event `self.ReceiveBeginPlay`
  (for _array_element (`self.IntearctableActorsWithTags`)
    (bind _outactors (`GameplayStatics.GetAllActorsWithTag` _array_element))
    (`KismetArrayLibrary.Array_Append` (`self.InteractableActors`) _outactors))
  (for _array_element_2 (`self.DescriptiveActorsWithTags`)
    (bind _outactors_2 (`GameplayStatics.GetAllActorsWithTag` _array_element_2))
    (`KismetArrayLibrary.Array_Append` (`self.InteractableActors`) _outactors_2)))

(fn `UserConstructionScript`)