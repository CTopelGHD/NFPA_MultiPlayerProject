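; Training checkpoint actor that shows a descriptive widget with title, text and media while the player is in its collision box.
; BeginPlay creates and fills the widget; overlap plays a sound, opens the media and phases the widget in, reversing on exit.
; Overlap also checks off the title-matched HUD checklist row, briefly sliding the checklist open on first visit.
; The construction script applies box extent and billboard height offsets and adds a tag.
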(event `self.ReceiveBeginPlay`
  (bind _wbp_descriptive_ui_ref (`self.WBP Descriptive UI Ref`))
  (`|ExecutionSequence`
    (:`then_0`
      (bind _returnvalue (`|CreateWidget` "/Game/UI/DescriptiveUI/WBP_DescriptinveUI.WBP_DescriptinveUI_C"))
      (bind _output_get (set `self.WBP Descriptive UI Ref` _returnvalue))
      (`WidgetComponent.SetWidget` (`self.DescriptiveUI`) _output_get))
    (:`then_1`
      (bind _returnvalue_2 (`GameplayStatics.GetActorOfClass` "/Game/Core/BP_GameHUD.BP_GameHUD_C"))
      (set `self.BP_GameHUD` _returnvalue_2))
    (:`then_2`
      (`KismetSystemLibrary.Delay` 0.5)
      (`/Game/UI/DescriptiveUI/WBP_DescriptinveUI.SetText` _wbp_descriptive_ui_ref (`self.TitleText`) (`self.DescriptiveText`))
      (`/Game/UI/DescriptiveUI/WBP_DescriptinveUI.SetMediaContent` _wbp_descriptive_ui_ref (`self.MediaSource`)))))

(event `self.Collision.OnComponentBeginOverlap`
  (params (OverlappedComponent :type "PrimitiveComponent Object Reference") (OtherActor :type "Actor Object Reference") (OtherComp :type "PrimitiveComponent Object Reference") (OtherBodyIndex :type Integer) (bFromSweep :type Boolean) (SweepResult :type "HitResult Structure (by ref)"))
  (`GameplayStatics.PlaySound2D` "/Game/Art/Audio/UI/DescriptorNotification.DescriptorNotification" 1.0 1.0 0.0 null null)
  (`self.PlaySpecificMediaSource`)
  (`SceneComponent.SetVisibility` (`self.DescriptiveUI`) true false)
  (`/Game/UI/DescriptiveUI/WBP_DescriptinveUI.Phase IN` (`self.WBP Descriptive UI Ref`))
  (for _array_element (`PanelWidget.GetAllChildren` (`/Game/UI/ChecklistUI/WBP_Checklist.ChecklistScrollBox` (`/Game/UI/GameHUD/WBP_GameHUD.WBP_Checklist` (`/Game/Core/BP_GameHUD.WBP_GameHUD` (`self.BP_GameHUD`)))))
    (bind _aswbp_checklist_row_item (cast `/Game/UI/ChecklistUI/WBP_ChecklistRowItem` _array_element))
    (if (== (`/Game/UI/ChecklistUI/WBP_ChecklistRowItem.TitleText` _aswbp_checklist_row_item) (`self.TitleText`))
      ;[1 1 1] Automatically show checklist if the player enters a checkpoint for the first time.
      (if (not (`|EnumEquality` (`CheckBox.CheckedState` (`/Game/UI/ChecklistUI/WBP_ChecklistRowItem.ChecklistCheckbox` _aswbp_checklist_row_item)) "Checked"))
        (`self.ShowChecklist`)
        (`/Game/UI/ChecklistUI/WBP_ChecklistRowItem.CheckOffRowItem` _aswbp_checklist_row_item))))
  (`KismetSystemLibrary.Delay` 3.0)
  (`self.CloseChecklist`))

(event `self.Collision.OnComponentEndOverlap`
  (params (OverlappedComponent :type "PrimitiveComponent Object Reference") (OtherActor :type "Actor Object Reference") (OtherComp :type "PrimitiveComponent Object Reference") (OtherBodyIndex :type Integer))
  (`MediaPlayer.Close` (`self.MediaPlayer`))
  (`/Game/UI/DescriptiveUI/WBP_DescriptinveUI.Phase OUT` (`self.WBP Descriptive UI Ref`))
  (`KismetSystemLibrary.Delay` 0.25)
  (`self.CloseChecklist`)
  (`SceneComponent.SetVisibility` (`self.DescriptiveUI`) false false))

(event `Phase IN`
  (bind (_direction _lerp) (`Timeline|Phase` :!via `PlayFromStart` :!label _label)
    (:`Update`
      (`SceneComponent.SetRelativeScale3D` (`self.DescriptiveUI`) (`KismetMathLibrary.VLerp` (0.0 0.0 0.0) (1.0 1.0 1.0) _lerp)))))

(event `Phase OUT`
  (goto _label :!via `Reverse`))

(fn `CloseChecklist`
  (bind _wbp_gamehud (`/Game/Core/BP_GameHUD.WBP_GameHUD` (`self.BP_GameHUD`)))
  ;[1 1 1] Check to see if the checklist opened. If so, close it.
  (if (>= (`KismetMathLibrary.BreakVector2D` (`.Translation` (break `WidgetTransform` (`Widget.RenderTransform` (`/Game/UI/GameHUD/WBP_GameHUD.WBP_Checklist` _wbp_gamehud))))) 0.0)
    (`UserWidget.PlayAnimation` _wbp_gamehud (`/Game/UI/GameHUD/WBP_GameHUD.MoveChecklistUI` _wbp_gamehud) 0.0 1 "Reverse" 1.0 false)))

(fn `PlaySpecificMediaSource`
  (locals (localMediaPlayer :type "MediaPlayer Object Reference" :default "/Script/MediaAssets.MediaPlayer'/Game/Art/Video_Clips/MediaPlayers/MediaPlayer.MediaPlayer'"))
  (`/Engine/EditorBlueprintResources/StandardMacros.IsValid` (`self.MediaSource`)
    (:`Is Valid`
      (`MediaPlayer.OpenSourceWithOptions` (`self.MediaPlayer`) (`self.MediaSource`) (make `MediaPlayerOptions` (struct :`Caption` -1 :`Metadata` -1 :`Script` -1 :`Subtitle` -1 :`Text` -1) "+00000000.00:00:00.000000000" "UseMediaPlayerSetting" (`self.LoopOptions`))))))

(fn `ShowChecklist`
  (bind _wbp_gamehud (`/Game/Core/BP_GameHUD.WBP_GameHUD` (`self.BP_GameHUD`)))
  ;[1 1 1] Check to see if the animation has already played manually by the player (The player can already see the checklist so no need to show it)
  (if (< (`KismetMathLibrary.BreakVector2D` (`.Translation` (break `WidgetTransform` (`Widget.RenderTransform` (`/Game/UI/GameHUD/WBP_GameHUD.WBP_Checklist` _wbp_gamehud))))) 0.0)
    (`UserWidget.PlayAnimation` _wbp_gamehud (`/Game/UI/GameHUD/WBP_GameHUD.MoveChecklistUI` _wbp_gamehud) 0.0 1 "Forward" 1.0 false)))

(fn `UserConstructionScript`
  (bind _collision (`self.Collision`))
  (`BoxComponent.SetBoxExtent` _collision (+ (`BoxComponent.BoxExtent` _collision) (`self.In Box Extent Offset`)) true)
  (`SceneComponent.K2_SetRelativeLocation` (`self.Billboard`) (`KismetMathLibrary.MakeVector` 0.0 0.0 (`self.In Descriptive Z Offset`)) false false)
  (`KismetArrayLibrary.Array_Add` (`self.Tags`) (`self.DescriptiveUITag`)))