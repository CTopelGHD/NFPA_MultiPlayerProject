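; Training checkpoint trigger that shows a descriptive tutorial panel when the local player walks into its box.
; Overlap fills the HUD widget with text, image and media, switches to UI-only input, freezes movement, then destroys the actor.
; A separate Server_CheckBoxes event ticks the checklist row matching the title, then closes the checklist.
; Construction sizes the box and sets the tag, while a looping delay re-rotates the text render toward the player.
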(event `self.ReceiveBeginPlay`
  (`self.Face the player`))

(event `Server_CheckBoxes`
  (`self.CheckBoxes`))

(event `self.Collision.OnComponentBeginOverlap`
  (params (OverlappedComponent :type "PrimitiveComponent Object Reference") (OtherActor :type "Actor Object Reference") (OtherComp :type "PrimitiveComponent Object Reference") (OtherBodyIndex :type Integer) (bFromSweep :type Boolean) (SweepResult :type "HitResult Structure (by ref)"))
  (if (== (`self.GetOwner` OtherActor) (`GameplayStatics.GetPlayerController` 0))
    (message `/Game/Core/Interfaces/BPI_GameController.SetDescriptiveUI_Available` (`GameplayStatics.GetPlayerController` 0) true)
    (bind _wbp_gamehud (message `/Game/Core/Interfaces/BPI_GameController.GetWBP_GameHUD` (`GameplayStatics.GetPlayerController` 0)))
    (bind _descriptiveupdatedui (`/Game/UI/GameHUD/WBP_GameHUD.DescriptiveUpdatedUI` _wbp_gamehud))
    (`/Game/UI/DescriptiveUI/DescriptiveUpdatedUI.Set Variables` _descriptiveupdatedui (`self.TitleText`) (`self.DescriptiveText`) (`self.Image`) (`self.DescriptiveUITag`) (`self.Media Player`) (`self.Media Source`) (`self.Media Material`) (`self.LoopOptions`))
    (`self.Set Input Mode Settings` _descriptiveupdatedui)
    (`GameplayStatics.PlaySound2D` "/Game/Art/Audio/UI/DescriptorNotification.DescriptorNotification" 1.0 1.0 0.0 null null)
    (`Widget.SetVisibility` _descriptiveupdatedui "Visible")
    (`/Game/UI/DescriptiveUI/DescriptiveUpdatedUI.Phase IN` _descriptiveupdatedui)
    (`KismetSystemLibrary.Delay` 1.0)
    (`self.K2_DestroyActor`)))

(event `CheckBoxes`
  (bind _wbp_gamehud (message `/Game/Core/Interfaces/BPI_GameController.GetWBP_GameHUD` (`GameplayStatics.GetPlayerController` 0)))
  (for _array_element (`PanelWidget.GetAllChildren` (`/Game/UI/ChecklistUI/WBP_Checklist.ChecklistScrollBox` (`/Game/UI/GameHUD/WBP_GameHUD.WBP_Checklist` _wbp_gamehud)))
    (bind _aswbp_checklist_row_item (cast `/Game/UI/ChecklistUI/WBP_ChecklistRowItem` _array_element))
    (if (== (`/Game/UI/ChecklistUI/WBP_ChecklistRowItem.TitleText` _aswbp_checklist_row_item) (`self.TitleText`))
      ;[1 1 1] Automatically show checklist if the player enters a checkpoint for the first time.
      (if (not (`|EnumEquality` (`CheckBox.CheckedState` (`/Game/UI/ChecklistUI/WBP_ChecklistRowItem.ChecklistCheckbox` _aswbp_checklist_row_item)) "Checked"))
        (`/Game/UI/ChecklistUI/WBP_ChecklistRowItem.CheckOffRowItem` _aswbp_checklist_row_item))))
  (`KismetSystemLibrary.Delay` 3.0)
  (`self.CloseChecklist`))

(event `self.Collision.OnComponentEndOverlap`
  (params (OverlappedComponent :type "PrimitiveComponent Object Reference") (OtherActor :type "Actor Object Reference") (OtherComp :type "PrimitiveComponent Object Reference") (OtherBodyIndex :type Integer)))

(event `Face the player`
  (bind _textrender (`self.TextRender`))
  (bind (_returnvalue_roll _returnvalue_pitch _returnvalue_yaw) (`KismetMathLibrary.BreakRotator` (`KismetMathLibrary.FindLookAtRotation` (`SceneComponent.RelativeLocation` _textrender) (`self.GetActorForwardVector` (`GameplayStatics.GetPlayerCharacter` 0)))))
  ;[0.05098 0.05098 0.05098] Face the Player
  (`SceneComponent.K2_SetRelativeRotation` _textrender (`KismetMathLibrary.MakeRotator` 0.0 0.0 _returnvalue_yaw) false false)
  (`KismetSystemLibrary.Delay` 0.2)
  (`self.Face the player`))

(fn `CloseChecklist`
  (bind _wbp_gamehud (message `/Game/Core/Interfaces/BPI_GameController.GetWBP_GameHUD` (`GameplayStatics.GetPlayerController` 0)))
  ;[1 1 1] Check to see if the checklist opened. If so, close it.
  (if (>= (`KismetMathLibrary.BreakVector2D` (`.Translation` (break `WidgetTransform` (`Widget.RenderTransform` (`/Game/UI/GameHUD/WBP_GameHUD.WBP_Checklist` _wbp_gamehud))))) 0.0)
    (`UserWidget.PlayAnimation` _wbp_gamehud (`/Game/UI/GameHUD/WBP_GameHUD.MoveChecklistUI` _wbp_gamehud) 0.0 1 "Reverse" 1.0 false)))

(fn `PlaySpecificMediaSource`
  (locals (localMediaPlayer :type "MediaPlayer Object Reference" :default null)))

(fn `Set Input Mode Settings`
  (params (InWidgetToFocus :type "Widget Object Reference"))
  (bind _returnvalue (`GameplayStatics.GetPlayerController` 0))
  (bind _charactermovement (`Character.CharacterMovement` (`GameplayStatics.GetPlayerCharacter` 0)))
  (bind _isdescriptiveui_available_ (message `/Game/Core/Interfaces/BPI_GameController.GetDescriptiveUI_Available` (`GameplayStatics.GetPlayerController` 0)))
  (if _isdescriptiveui_available_
    (`/Engine/EditorBlueprintResources/StandardMacros.IsValid` InWidgetToFocus
      (:`Is Valid`
        (`WidgetBlueprintLibrary.SetInputMode_UIOnlyEx` _returnvalue InWidgetToFocus)
        (set `PlayerController.bShowMouseCursor` true _returnvalue)
        (`CharacterMovementComponent.SetMovementMode` _charactermovement "MOVE_None" 0)))
    (else
      (`WidgetBlueprintLibrary.SetInputMode_GameOnly` _returnvalue)
      (set `PlayerController.bShowMouseCursor` false _returnvalue)
      (`CharacterMovementComponent.SetMovementMode` _charactermovement "MOVE_Walking" 0))))

(fn `ShowChecklist`
  (bind _wbp_gamehud (message `/Game/Core/Interfaces/BPI_GameController.GetWBP_GameHUD` (`GameplayStatics.GetPlayerController` 0)))
  ;[1 1 1] Check to see if the animation has already played manually by the player (The player can already see the checklist so no need to show it)
  (if (< (`KismetMathLibrary.BreakVector2D` (`.Translation` (break `WidgetTransform` (`Widget.RenderTransform` (`/Game/UI/GameHUD/WBP_GameHUD.WBP_Checklist` _wbp_gamehud))))) 0.0)
    (`UserWidget.PlayAnimation` _wbp_gamehud (`/Game/UI/GameHUD/WBP_GameHUD.MoveChecklistUI` _wbp_gamehud) 0.0 1 "Forward" 1.0 false)))

(fn `UserConstructionScript`
  (bind _collision (`self.Collision`))
  (bind _tags (`self.Tags`))
  (`BoxComponent.SetBoxExtent` _collision (+ (`BoxComponent.BoxExtent` _collision) (`self.In Box Extent Offset`)) true)
  (`SceneComponent.K2_SetRelativeLocation` (`self.Billboard`) (`KismetMathLibrary.MakeVector` 0.0 0.0 (`self.In Descriptive Z Offset`)) false false)
  (`KismetArrayLibrary.Array_Clear` _tags)
  (`/Engine/EditorBlueprintResources/StandardMacros.DoOnce` false
    (:`Completed`
      (`KismetArrayLibrary.Array_Add` _tags (`self.DescriptiveUITag`)))))