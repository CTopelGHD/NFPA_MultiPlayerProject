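; Interactive training step actor that shows a prompt and runs an interaction when triggered.
; Local-player overlap with its box shows the UI widget and sends the step's tag ID to the player controller.
; ToggleInteraction disables input, hides the pawn and plays a level sequence, with optional reverse replay, X-ray effect or sound.
; Completion restores the player, swaps visibility and collision on tagged actors, and notifies BP_TrainingTracker.
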(event `self.ReceiveBeginPlay`
  (`|ExecutionSequence`
    (:`then_0`
      (bind _returnvalue (`|CreateWidget` "/Game/UI/InteractiveUI/WBP_InteractiveUI.WBP_InteractiveUI_C"))
      (bind _output_get (set `self.InteractiveUI Ref` _returnvalue))
      (`WidgetComponent.SetWidget` (`self.InteractiveUI`) _output_get))
    (:`then_1`
      (bind _returnvalue_2 (`GameplayStatics.GetActorOfClass` "/Game/Core/BP_GameHUD.BP_GameHUD_C"))
      (set `self.BP_GameHUD` _returnvalue_2)
      (bind _outactors (`GameplayStatics.GetAllActorsOfClass` "/Game/Core/Systems/XRayVision/XRayVisionPostProcessVolume_Blueprint.XRayVisionPostProcessVolume_Blueprint_C"))
      (set `self.XRay Vision PP Ref` (`|GetArrayItem` _outactors)))
    (:`then_2`
      (`KismetSystemLibrary.Delay` 0.5)
      (`/Game/UI/InteractiveUI/WBP_InteractiveUI.SetText` (`self.InteractiveUI Ref`) (`self.Title Text`) (`self.PressResultText`)))
    (:`then_3`
      (bind _returnvalue_3 (`GameplayStatics.GetActorOfClass` "/Game/Core/TrainingManager/BP_TrainingTracker.BP_TrainingTracker_C"))
      (set `self.BP_TrainingTracker` _returnvalue_3))))

(event `OpenCollision`
  (`PrimitiveComponent.SetCollisionEnabled` (`self.Collision`) "QueryOnly"))

(event `self.Collision.OnComponentBeginOverlap`
  (params (OverlappedComponent :type "PrimitiveComponent Object Reference") (OtherActor :type "Actor Object Reference") (OtherComp :type "PrimitiveComponent Object Reference") (OtherBodyIndex :type Integer) (bFromSweep :type Boolean) (SweepResult :type "HitResult Structure (by ref)"))
  (if (== (`self.GetOwner` OtherActor) (`GameplayStatics.GetPlayerController` 0))
    (set `self.InCollision?` true)
    (`GameplayStatics.PlaySound2D` "/Game/Art/Audio/UI/DescriptorNotification.DescriptorNotification" 1.0 1.0 0.0 null null)
    (`SceneComponent.SetVisibility` (`self.InteractiveUI`) true false)
    (`/Game/UI/InteractiveUI/WBP_InteractiveUI.Phase IN` (`self.InteractiveUI Ref`))
    (message `/Game/Core/Interfaces/BPI_GameController.SendTrainingStepInteractiveTagID` (`GameplayStatics.GetPlayerController` 0) (`|GetArrayItem` (`self.Tags`)))
    (else
      (`KismetSystemLibrary.PrintString` "Another Player Overlapped"))))

(event `self.Collision.OnComponentEndOverlap`
  (params (OverlappedComponent :type "PrimitiveComponent Object Reference") (OtherActor :type "Actor Object Reference") (OtherComp :type "PrimitiveComponent Object Reference") (OtherBodyIndex :type Integer))
  (if (== (`self.GetOwner` OtherActor) (`GameplayStatics.GetPlayerController` 0))
    (set `self.InCollision?` false)
    (`KismetSystemLibrary.PrintString` "Closing Out" true true (struct :`R` 255.0 :`G` 209.000061 :`A` 1.0))
    (`/Game/UI/InteractiveUI/WBP_InteractiveUI.Phase OUT` (`self.InteractiveUI Ref`))
    (`KismetSystemLibrary.Delay` 0.5)
    (`SceneComponent.SetVisibility` (`self.InteractiveUI`) false false)
    (message `/Game/Core/Interfaces/BPI_GameController.SendTrainingStepInteractiveTagID` (`GameplayStatics.GetPlayerController` 0) "None")))

(event `CloseCollision`
  (`PrimitiveComponent.SetCollisionEnabled` (`self.Collision`) "NoCollision")
  (`SceneComponent.SetVisibility` (`self.InteractiveUI`) false false))

(event `ToggleInteraction`
  (bind _returnvalue (`GameplayStatics.GetPlayerController` 0))
  (`self.DisableInput` _returnvalue _returnvalue)
  (`self.DisableInput` (`GameplayStatics.GetPlayerPawn` 0) _returnvalue)
  (message `/Game/Core/Interfaces/BPI_Pawn.TogglePawnVisibility` (`GameplayStatics.GetPlayerPawn` 0) false)
  (`self.CloseCollision`)
  (if (`self.IsThereA LevelSequence`)
    (if (`self.PlayReverse?`)
      ;[1 1 1] Backward
      (`MovieSceneSequencePlayer.PlayReverse` (stale _returnvalue_2))
      (set `self.PlayReverse?` false)
      (`KismetSystemLibrary.Delay` (`self.Interaction Delay`) :!label _label)
      (`self.OpenCollision` :!label _label_2)
      (`self.OnCompletion`)
      (else
        (bind (_outactor _returnvalue_2) (`LevelSequencePlayer.CreateLevelSequencePlayer` (`self.Level Sequence`)))
        ;[1 1 1] Forward
        (`MovieSceneSequencePlayer.Play` _returnvalue_2)
        (if (`self.X-Ray?`)
          (`/Game/Core/Systems/XRayVision/XRayVisionPostProcessVolume_Blueprint.Xray Execution` (`self.XRay Vision PP Ref`))
          (`KismetSystemLibrary.Delay` (`self.Interaction Delay`))
          (`/Game/Core/Systems/XRayVision/XRayVisionPostProcessVolume_Blueprint.Xray Execution` (`self.XRay Vision PP Ref`)))
        (if (`self.ActivateOnce?`)
          (if (not (`self.X-Ray?`))
            (`KismetSystemLibrary.Delay` (`self.Interaction Delay`)))
          (`self.OnCompletion`)
          (else
            (set `self.PlayReverse?` true)
            (if (`self.X-Ray?`)
              (goto _label_2)
              (else
                (goto _label)))))))
    (else
      (if (`self.InteractionCompleted?`)
        (`KismetSystemLibrary.PrintString` (`KismetStringLibrary.Concat_StrStr` "Warning:" (`KismetSystemLibrary.GetDisplayName` self) " interaction has already completed!"))
        (else
          (bind (_outactor_2 _returnvalue_3) (`LevelSequencePlayer.CreateLevelSequencePlayer` (`self.Level Sequence`)))
          (`MovieSceneSequencePlayer.Play` _returnvalue_3)
          (`KismetSystemLibrary.Delay` (`self.Interaction Delay`))
          (bind _sound (`self.Sound`)
            (:`then`
              (`GameplayStatics.PlaySound2D` _sound 1.0 1.0 0.0 null null))
            (:`else`
              (`KismetSystemLibrary.PrintString` (`KismetStringLibrary.Concat_StrStr` "Warning:" (`KismetSystemLibrary.GetDisplayName` _sound) " did not play in " (`KismetSystemLibrary.GetDisplayName` self) "."))))))
      (`self.OnCompletion`))))

(event `OnCompletion`
  (message `/Game/Core/Interfaces/BPI_Pawn.TogglePawnVisibility` (`GameplayStatics.GetPlayerPawn` 0) true)
  (`self.EnableInput` (`GameplayStatics.GetPlayerPawn` 0) (`GameplayStatics.GetPlayerController` 0))
  (`self.EnableInput` (`GameplayStatics.GetPlayerController` 0) (`GameplayStatics.GetPlayerController` 0))
  (set `self.InteractionCompleted?` true)
  (`self.TryActorsOnCompletion`)
  (bind _bp_trainingtracker (`self.BP_TrainingTracker`)
    (:`then`
      (`/Game/Core/TrainingManager/BP_TrainingTracker.OnInteractComplete` _bp_trainingtracker (`|GetArrayItem` (`self.Tags`))))
    (:`else`
      (`KismetSystemLibrary.PrintString` (`KismetStringLibrary.Concat_StrStr` "Error:" (`KismetSystemLibrary.GetDisplayName` _bp_trainingtracker) " in " (`KismetSystemLibrary.GetDisplayName` self) " is not valid.")))))

(event `TryActorsOnCompletion`
  (for _array_element (`self.ActorTagsBeforeCompletion`)
    (bind _outactors (`GameplayStatics.GetAllActorsWithTag` _array_element))
    (for _array_element_2 _outactors
      (`self.SetActorHiddenInGame` _array_element_2 true)
      (`self.SetActorEnableCollision` _array_element_2 false)))
  (for _array_element_3 (`self.ActorTagsAfterCompletion`)
    (bind _outactors_2 (`GameplayStatics.GetAllActorsWithTag` _array_element_3))
    (for _array_element_4 _outactors_2
      (`self.SetActorHiddenInGame` _array_element_4 false)
      (`self.SetActorEnableCollision` _array_element_4 true))))

(fn `UserConstructionScript`
  (bind _collision (`self.Collision`))
  (`BoxComponent.SetBoxExtent` _collision (+ (`BoxComponent.BoxExtent` _collision) (`self.In Box Extent`)) true)
  (`SceneComponent.K2_SetRelativeLocation` (`self.Billboard`) (`KismetMathLibrary.MakeVector` 0.0 0.0 (`self.Interactive Z Offset`)) false false)
  (`/Engine/EditorBlueprintResources/StandardMacros.DoOnce` false
    (:`Completed`
      (`KismetArrayLibrary.Array_Add` (`self.Tags`) (`self.ID Tag`)))))