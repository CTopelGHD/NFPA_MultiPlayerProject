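; Tracks progression through a firefighting training scenario involving EV, ESS, solar and hose tasks.
; On BeginPlay it fills tagged descriptive and interactive step actors from two data tables.
; OnInteractComplete branches on step ID to set player controller message flags, enable or disable tagged interactives, play a hose sequence and trigger HUD spray and end-screen results.
; Activation helpers toggle each step's collision, overlap events and indicator.
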(event `self.ReceiveBeginPlay`
  (`KismetSystemLibrary.Delay` 1.0)
  (`self.SetDescriptiveTrainingStepVariables`)
  (`self.SetInteractiveTrainingStepVariables`)
  (bind _returnvalue (`GameplayStatics.GetActorOfClass` "/Game/Core/BP_GameHUD.BP_GameHUD_C"))
  (set `self.BP_GameHUD` _returnvalue))

(event `OnInteractComplete`
  (params (TrainingInteractiveStepTagID :type Name))
  (bind _returnvalue (`GameplayStatics.GetPlayerController` 0))
  (bind _returnvalue_2 (`GameplayStatics.GetPlayerController` 0))
  (bind _returnvalue_3 (`GameplayStatics.GetPlayerController` 0))
  (if (== TrainingInteractiveStepTagID "FHose")
    (`KismetSystemLibrary.PrintString` "Fire Put Out")
    (elif (== TrainingInteractiveStepTagID "Engine Handline")
      (`KismetSystemLibrary.Delay` 0.2)
      (`self.Activate Next Interactive` "Engine Handline")
      (elif (== TrainingInteractiveStepTagID "Civilian")
        (message `/Game/Core/Interfaces/BPI_GameController.Set TalkedToOwner` (`GameplayStatics.GetPlayerController` 0) true)
        (elif (== TrainingInteractiveStepTagID "EBox")
          (message `/Game/Core/Interfaces/BPI_GameController.Set Turned Off PV Panels?` (`GameplayStatics.GetPlayerController` 0) true)
          (elif (== TrainingInteractiveStepTagID "Wench")
            (message `/Game/Core/Interfaces/BPI_GameController.Set Wench Used?` (`GameplayStatics.GetPlayerController` 0) true)
            (elif (== TrainingInteractiveStepTagID "L Fence Door")
              (message `/Game/Core/Interfaces/BPI_GameController.Set LeftGate Opened?` _returnvalue true)
              (bind _outactors (`GameplayStatics.GetAllActorsWithTag` "LFenceGate"))
              (`self.SetActorEnableCollision` (`|GetArrayItem` _outactors) false)
              (elif (== TrainingInteractiveStepTagID "BackGarageDoorHose")
                (message `/Game/Core/Interfaces/BPI_GameController.Set Back GarageDoor Opened?` _returnvalue true)
                (elif (== TrainingInteractiveStepTagID "SolarPanels")
                  (message `/Game/Core/Interfaces/BPI_GameController.Set Observed Solar Panels?` (`GameplayStatics.GetPlayerController` 0) true)
                  (elif (== TrainingInteractiveStepTagID "Tools")
                    (set `self.bToolsActivated` true)
                    (`self.DeactivateInteractive` "Tools")
                    (`self.Activate Next Interactive` "Hydrant" true)
                    (`self.Activate Next Interactive` "Engine Handline")
                    (elif (== TrainingInteractiveStepTagID "Electrical Box")
                      (bind _returnvalue_4 (`GameplayStatics.GetActorOfClass` "/Game/Core/Systems/Pawns/GameController.GameController_C"))
                      (set `/Game/Core/Systems/Pawns/GameController.bBasementCircuitBreakerChecked` true _returnvalue_4)
                      (elif (== TrainingInteractiveStepTagID "FirstEVandESS_FireOut")
                        (`self.Activate Next Interactive` "CommanderVehicle")
                        (elif (== TrainingInteractiveStepTagID "SecondEV_FireOut")
                          (`self.Activate Next Interactive` "EV Thermal Gun" true)
                          (`self.DeactivateInteractive` "FrontGarageDoorHose")
                          (bind (_outactor _returnvalue_5) (`LevelSequencePlayer.CreateLevelSequencePlayer` "/Game/Art/Video_Clips/LevelSequences/FireHose/LS_AdjustHosePositionGarage.LS_AdjustHosePositionGarage"))
                          (`MovieSceneSequencePlayer.Play` _returnvalue_5)
                          (`self.Activate Next Interactive` "GarageHose")
                          (message `/Game/Core/Interfaces/BPI_GameController.Set FinalHose Available?` _returnvalue_2 true)
                          (message `/Game/Core/Interfaces/BPI_GameController.Set EV Fire Put Out Again?` _returnvalue_2 true)
                          (message `/Game/Core/Interfaces/BPI_GameController.Set Ready to Spray ESS Again?` _returnvalue_2 true)
                          (bind _returnvalue_6 (`GameplayStatics.GetActorOfClass` "/Game/Art/VFX/JetFlame/BP_EVFire.BP_EVFire_C"))
                          (`PrimitiveComponent.SetCollisionEnabled` (`/Game/Art/VFX/JetFlame/BP_EVFire.ESS_TriggerBox` _returnvalue_6) "QueryOnly")
                          (elif (== TrainingInteractiveStepTagID "CommanderVehicle")
                            (`self.Activate Next Interactive` "FrontGarageDoorHose")
                            (`self.DeactivateInteractive` "CommanderVehicle")
                            (elif (== TrainingInteractiveStepTagID "EV Thermal Gun")
                              _
                              (elif (== TrainingInteractiveStepTagID "ESS Thermal Gun")
                                _
                                (elif (== TrainingInteractiveStepTagID "GarageHose")
                                  _
                                  (elif (== TrainingInteractiveStepTagID "GarageBackDoor")
                                    (`self.DeactivateInteractive` "GarageBackDoor")
                                    (elif (== TrainingInteractiveStepTagID "HoseSelected")
                                      (`self.DeactivateInteractive` "GarageBackDoor")
                                      (`self.DeactivateInteractive` "BackGarageDoorHose")
                                      (elif (== TrainingInteractiveStepTagID "SecondESS_FireOut")
                                        (`self.Activate Next Interactive` "ESS Thermal Gun" true)
                                        (`self.DeactivateInteractive` "GarageHose")
                                        (`self.Activate Next Interactive` "EndScenario" true)
                                        (message `/Game/Core/Interfaces/BPI_GameController.Set ESS Fire Put Out?` _returnvalue_3 true)
                                        (message `/Game/Core/Interfaces/BPI_GameController.Set EV Fire Put Out Again?` _returnvalue_3 true)
                                        (elif (== TrainingInteractiveStepTagID "EndScenario")
                                          (bind _returnvalue_7 (`GameplayStatics.GetActorOfClass` "/Game/Core/BP_GameHUD.BP_GameHUD_C"))
                                          (`/Game/UI/EndScreen/EndScreenUI.GetEndTimeResults` (`/Game/UI/GameHUD/WBP_GameHUD.EndScreenUI` (`/Game/Core/BP_GameHUD.WBP_GameHUD` _returnvalue_7)))
                                          (elif (== TrainingInteractiveStepTagID "Hydrant")
                                            (message `/Game/Core/Interfaces/BPI_GameController.Set Attached Hydrant?` (`GameplayStatics.GetPlayerController` 0) true)
                                            (elif (== TrainingInteractiveStepTagID "Main Breaker")
                                              (message `/Game/Core/Interfaces/BPI_GameController.Set Turned Off Electric Box?` (`GameplayStatics.GetPlayerController` 0) true)
                                              (elif (== TrainingInteractiveStepTagID "BackDoorCrackedSprayCompleted")
                                                (`self.Activate Next Interactive` "BackGarageDoorHose")
                                                (`/Game/UI/InteractiveUI/WBP_FireHoseOptions.StartSprayNozzleEvent` (`/Game/UI/GameHUD/WBP_GameHUD.WBP_FireHoseOptions` (`/Game/Core/BP_GameHUD.WBP_GameHUD` (`self.BP_GameHUD`))))
                                                (elif (== TrainingInteractiveStepTagID "EV Thermal Gun")
                                                  (message `/Game/Core/Interfaces/BPI_GameController.Set Used the Thermal Gun After Second Fire?` (`GameplayStatics.GetPlayerController` 0) true)
                                                  (elif (== TrainingInteractiveStepTagID "ESS Thermal Gun")
                                                    (message `/Game/Core/Interfaces/BPI_GameController.Set Used Thermal Gun on ESS?` (`GameplayStatics.GetPlayerController` 0) true)
                                                    (elif (== TrainingInteractiveStepTagID "DoorCrackedSuccessfully")
                                                      (message `/Game/Core/Interfaces/BPI_GameController.Set Cracked Door Sprayed?` (`GameplayStatics.GetPlayerController` 0) true)
                                                      (`/Game/UI/InteractiveUI/WBP_FireHoseOptions.StartSprayNozzleEvent` (`/Game/UI/GameHUD/WBP_GameHUD.WBP_FireHoseOptions` (`/Game/Core/BP_GameHUD.WBP_GameHUD` (`self.BP_GameHUD`))))
                                                      (elif (== TrainingInteractiveStepTagID "DisableFireTruckHoseOptions")
                                                        (set `self.bEngineHardlineDeactivated` true)
                                                        (`self.DeactivateInteractive` "Engine Handline")
                                                        (elif (== TrainingInteractiveStepTagID "BackDoorOpenedFully")
                                                          (`/Game/UI/InteractiveUI/WBP_FireHoseOptions.StartSprayNozzleEvent` (`/Game/UI/GameHUD/WBP_GameHUD.WBP_FireHoseOptions` (`/Game/Core/BP_GameHUD.WBP_GameHUD` (`self.BP_GameHUD`)))))))))))))))))))))))))))))))))

(event `Activate Next Interactive`
  (params (Tag :type Name) (RunParentOverlap :type Boolean))
  ;[1 1 1] Activate Next
  (bind _outactors (`GameplayStatics.GetAllActorsOfClassWithTag` "/Game/Core/TrainingManager/BP_TS_Interactive.BP_TS_Interactive_C" Tag))
  (for _array_element _outactors
    (bind _boxcollision (`/Game/Core/TrainingManager/BP_TS_Interactive.BoxCollision` _array_element))
    (`PrimitiveComponent.SetCollisionEnabled` _boxcollision "QueryOnly")
    (bind _output_get (set `PrimitiveComponent.bGenerateOverlapEvents` true _boxcollision))
    (`/Game/Core/TrainingManager/BP_TS_Interactive.ToggleIndicatorAddToViewport` _array_element _output_get)
    (set `/Game/Core/TrainingManager/BP_TS_Interactive.RunParentOverlap` RunParentOverlap _array_element))
  (bind _asgame_controller (cast `/Game/Core/Systems/Pawns/GameController` (`GameplayStatics.GetPlayerController` 0)))
  (`/Game/Core/Systems/Pawns/GameController.ToggleAllIndicatorIcons` _asgame_controller false))

(event `DeactivateInteractive`
  (params (Tag :type Name))
  ;[1 1 1] Deactiavte interactive
  (bind _outactors (`GameplayStatics.GetAllActorsOfClassWithTag` "/Game/Core/TrainingManager/BP_TS_Interactive.BP_TS_Interactive_C" Tag))
  (for _array_element _outactors
    (bind _boxcollision (`/Game/Core/TrainingManager/BP_TS_Interactive.BoxCollision` _array_element))
    (`PrimitiveComponent.SetCollisionEnabled` _boxcollision "NoCollision")
    (bind _output_get (set `PrimitiveComponent.bGenerateOverlapEvents` false _boxcollision))
    (`/Game/Core/TrainingManager/BP_TS_Interactive.ToggleIndicatorAddToViewport` _array_element _output_get)))

(fn `SetDescriptiveTrainingStepVariables`
  (bind _outrownames (`DataTableFunctionLibrary.GetDataTableRowNames` "/Game/Core/Data/DescriptiveUI/DT_DescriptiveActors.DT_DescriptiveActors"))
  (for _array_element _outrownames
    (bind _returnvalue (`|GetDataTableRow` "/Game/Core/Data/DescriptiveUI/DT_DescriptiveActors.DT_DescriptiveActors" _array_element)
      (:`then`
        (bind _outactors (`GameplayStatics.GetAllActorsOfClassWithTag` "/Game/Core/TrainingManager/BP_TrainingStepD.BP_TrainingStepD_C" (`KismetStringLibrary.Conv_StringToName` (break `/Game/Core/Data/DescriptiveUI/DescriptiveUI_Struct` _returnvalue))))
        (for _array_element_2 _outactors
          (set `/Game/Core/TrainingManager/BP_TrainingStepD.TitleText` (`KismetTextLibrary.Conv_StringToText` (`.Title_2_7A8083074D03ACDC9B58D081AB3CD9C7` (break `/Game/Core/Data/DescriptiveUI/DescriptiveUI_Struct` _returnvalue))) _array_element_2)
          (set `/Game/Core/TrainingManager/BP_TrainingStepD.DescriptiveText` (`KismetTextLibrary.Conv_StringToText` (`.Description_4_729DB175460C5B13190D26ABBB1285E1` (break `/Game/Core/Data/DescriptiveUI/DescriptiveUI_Struct` _returnvalue))) _array_element_2)
          (set `/Game/Core/TrainingManager/BP_TrainingStepD.Image` (`.Image_47_CCC2575D4DB3C89886B0ACA5D495D012` (break `/Game/Core/Data/DescriptiveUI/DescriptiveUI_Struct` _returnvalue)) _array_element_2)
          (set `/Game/Core/TrainingManager/BP_TrainingStepD.Media Player` (`.MediaPlayer_51_D539D1F2493505537D737082DB6413BE` (break `/Game/Core/Data/DescriptiveUI/DescriptiveUI_Struct` _returnvalue)) _array_element_2)
          (set `/Game/Core/TrainingManager/BP_TrainingStepD.LoopOptions` (`.Looped?_32_F325ECE04C5E29AFD9AD04A81FF1F6EB` (break `/Game/Core/Data/DescriptiveUI/DescriptiveUI_Struct` _returnvalue)) _array_element_2)
          (set `/Game/Core/TrainingManager/BP_TrainingStepD.Media Source` (`.MediaSource_54_21FDC5574948694415BD10B648F39935` (break `/Game/Core/Data/DescriptiveUI/DescriptiveUI_Struct` _returnvalue)) _array_element_2)
          (set `/Game/Core/TrainingManager/BP_TrainingStepD.Media Material` (`.MediaMaterial_61_70414290448128A1BD58BC93AE19ADBA` (break `/Game/Core/Data/DescriptiveUI/DescriptiveUI_Struct` _returnvalue)) _array_element_2))))))

(fn `SetInteractiveTrainingStepVariables`
  (bind _outrownames (`DataTableFunctionLibrary.GetDataTableRowNames` "/Game/Core/Data/TrainingResourcesData/DT_TrainingInteractive.DT_TrainingInteractive"))
  (for _array_element _outrownames
    (bind _returnvalue (`|GetDataTableRow` "/Game/Core/Data/TrainingResourcesData/DT_TrainingInteractive.DT_TrainingInteractive" _array_element)
      (:`then`
        (`KismetArrayLibrary.Array_Add` (`self.ActorID_Tags`) (break `/Game/Core/Data/TrainingResourcesData/TrainingInteractive_Struct` _returnvalue))
        (bind _outactors (`GameplayStatics.GetAllActorsOfClassWithTag` "/Game/Core/TrainingManager/BP_TS_Interactive.BP_TS_Interactive_C" (break `/Game/Core/Data/TrainingResourcesData/TrainingInteractive_Struct` _returnvalue)))
        (for _array_element_2 _outactors
          (set `/Game/Core/TrainingManager/BP_TS_Interactive.Title Text` (`.TitleText_13_66182FE445F66BB5891AE9812D9614E5` (break `/Game/Core/Data/TrainingResourcesData/TrainingInteractive_Struct` _returnvalue)) _array_element_2)
          (set `/Game/Core/TrainingManager/BP_TS_Interactive.PressResultText` (`.InteractText_15_9F5ED5F547E8EA5675EF9C98F42AE311` (break `/Game/Core/Data/TrainingResourcesData/TrainingInteractive_Struct` _returnvalue)) _array_element_2)
          (set `/Game/Core/TrainingManager/BP_TS_Interactive.Level Sequence` (`.LevelSequence_18_BD096980402629A787C13C912A6D8BC2` (break `/Game/Core/Data/TrainingResourcesData/TrainingInteractive_Struct` _returnvalue)) _array_element_2)
          (set `/Game/Core/TrainingManager/BP_TS_Interactive.IsSubStep?` (`.IsSubStep?_26_5B6FD4AC4A095E1DE0E12A8E64BE0F10` (break `/Game/Core/Data/TrainingResourcesData/TrainingInteractive_Struct` _returnvalue)) _array_element_2)
          (set `/Game/Core/TrainingManager/BP_TS_Interactive.SubStep ID` (`.SubStepID_30_C955EE344E4B7F17D1B1A1A28A9717BE` (break `/Game/Core/Data/TrainingResourcesData/TrainingInteractive_Struct` _returnvalue)) _array_element_2)
          (set `/Game/Core/TrainingManager/BP_TS_Interactive.SubStep Index` (`.SubStepIndex_33_AB28781E48A646FE42D05383AB5B52B5` (break `/Game/Core/Data/TrainingResourcesData/TrainingInteractive_Struct` _returnvalue)) _array_element_2)
          (set `/Game/Core/TrainingManager/BP_TS_Interactive.IsThere a LS Animation` (`.Animation?_43_3E4B44A446453C19BFF3688F06E0D31A` (break `/Game/Core/Data/TrainingResourcesData/TrainingInteractive_Struct` _returnvalue)) _array_element_2)
          (set `/Game/Core/TrainingManager/BP_TS_Interactive.Sound` (`.Sound_46_C358F3AC4033553DB259B0B3C1BCFBE2` (break `/Game/Core/Data/TrainingResourcesData/TrainingInteractive_Struct` _returnvalue)) _array_element_2)
          (set `/Game/Core/TrainingManager/BP_TS_Interactive.X-Ray?` (`.X-Ray?_48_E2EAA2954185B6CDE303A098823D975F` (break `/Game/Core/Data/TrainingResourcesData/TrainingInteractive_Struct` _returnvalue)) _array_element_2)
          (set `/Game/Core/TrainingManager/BP_TS_Interactive.Interaction Delay` (`.InteractionDelay_56_5DD3D91847CAF509C31462927DDB771A` (break `/Game/Core/Data/TrainingResourcesData/TrainingInteractive_Struct` _returnvalue)) _array_element_2)
          (set `/Game/Core/TrainingManager/BP_TS_Interactive.ActivateOnce?` (`.ActivateOnce?_54_013190B249A679EA755BECBCD87F2916` (break `/Game/Core/Data/TrainingResourcesData/TrainingInteractive_Struct` _returnvalue)) _array_element_2))))))

(fn `Turn on Interactive Hose`
  (bind _outactors (`GameplayStatics.GetAllActorsOfClassWithTag` "/Game/Core/TrainingManager/BP_InteractiveHose.BP_InteractiveHose_C" "FireTruckHose"))
  (for _array_element _outactors
    (`PrimitiveComponent.SetCollisionEnabled` (`/Game/Core/TrainingManager/BP_TS_Interactive.BoxCollision` _array_element) "QueryOnly")))

(fn `Turn On Interactive Hydrant Attach`
  (bind _outactors (`GameplayStatics.GetAllActorsOfClassWithTag` "/Game/Core/TrainingManager/BP_TS_Interactive.BP_TS_Interactive_C" "Hydrant"))
  (`PrimitiveComponent.SetCollisionEnabled` (`/Game/Core/TrainingManager/BP_TS_Interactive.BoxCollision` (`|GetArrayItem` _outactors)) "QueryOnly")
  (`KismetSystemLibrary.PrintString` "Hydrant Attach collision enabled" true true (struct :`R` 0.017294 :`G` 1.0 :`B` 0.050139 :`A` 1.0)))

(fn `UserConstructionScript`)