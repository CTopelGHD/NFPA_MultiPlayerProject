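; BP_TrainingTracker is a manager actor that fills the level's training steps with their instructional text and video from a data table.
; On BeginPlay it loops every row of DT_DescriptiveActors and finds BP_TrainingStep actors whose tag matches the row's TagID.
; It copies title, description, media texture, player and source onto each match, so content binds by actor tag rather than direct references.
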(event `self.ReceiveBeginPlay`
  (bind _outrownames (`DataTableFunctionLibrary.GetDataTableRowNames` "/Game/Core/Data/DescriptiveUI/DT_DescriptiveActors.DT_DescriptiveActors"))
  (for _array_element _outrownames
    (bind _returnvalue (`|GetDataTableRow` "/Game/Core/Data/DescriptiveUI/DT_DescriptiveActors.DT_DescriptiveActors" _array_element)
      (:`then`
        (bind (_tagid _title _description _videoclip _mediaplayer _mediasource) (break `/Game/Core/Data/DescriptiveUI/DescriptiveUI_Struct` _returnvalue))
        (bind _outactors (`GameplayStatics.GetAllActorsOfClassWithTag` "/Game/Core/TrainingManager/JohnsVersion/BP_TrainingStep.BP_TrainingStep_C" (`KismetStringLibrary.Conv_StringToName` _tagid)))
        (for _array_element_2 _outactors
          (set `/Game/Core/TrainingManager/JohnsVersion/BP_TrainingStep.TitleText` (`KismetTextLibrary.Conv_StringToText` _title) _array_element_2)
          (set `/Game/Core/TrainingManager/JohnsVersion/BP_TrainingStep.DescriptiveText` (`KismetTextLibrary.Conv_StringToText` _description) _array_element_2)
          (set `/Game/Core/TrainingManager/JohnsVersion/BP_TrainingStep.MediaTexture` _videoclip _array_element_2)
          (set `/Game/Core/TrainingManager/JohnsVersion/BP_TrainingStep.MediaPlayer` _mediaplayer _array_element_2)
          (set `/Game/Core/TrainingManager/JohnsVersion/BP_TrainingStep.MediaSource` _mediasource _array_element_2))))))

(fn `UserConstructionScript`)