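; BP_IndicatorComponent is a component that creates and manages an on-screen indicator widget.
; On BeginPlay, except on dedicated servers, it creates the configured widget class, passes itself in as the owning indicator component, and adds it to the viewport.
; Events let other code remove or re-add the widget and toggle it between non-hit-testable visible and collapsed.
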(event `self.ReceiveBeginPlay`
  (if (not (`KismetSystemLibrary.IsDedicatedServer`))
    (bind _returnvalue (`|CreateWidget` (`self.IndicatorWidgetClass`) null self))
    (bind _output_get (set `self.W_Indicator` _returnvalue))
    (`UserWidget.AddToViewport` _output_get 0)))

(event `RemoveFromViewport`
  (`Widget.RemoveFromParent` (`self.W_Indicator`)))

(event `AddToViewport`
  (`UserWidget.AddToViewport` (`self.W_Indicator`) 0))

(event `ToggleVis`
  (params (Condition :type Boolean))
  (bind _w_indicator (`self.W_Indicator`))
  (if Condition
    (`Widget.SetVisibility` _w_indicator "SelfHitTestInvisible")
    (else
      (`Widget.SetVisibility` _w_indicator "Collapsed"))))