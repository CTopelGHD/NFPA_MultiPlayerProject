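; Preview actor for a modular male firefighter character, with toggles for outfit pieces, equipment, head and bat.
; The Construction Script makes head, gloves, pants, boots and helmet follow the Body's pose via Leader Pose, assigns the animation and applies visibility.
; SetOutfitsVisability also drives per-slot Body material scalars for jacket, gloves, pants and boots.
; The helmet toggle sets a head morph target, reapplied on BeginPlay.
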(event `self.ReceiveBeginPlay`
  (`SkeletalMeshComponent.SetMorphTarget` (`self.Head`) "mt_firefighter_helmet" (`KismetMathLibrary.Conv_BoolToDouble` (`self.IsHelmetOn`)) true))

(fn `SetOutfitsVisability`
  (bind _isjacketon (`self.IsJacketOn`))
  (bind _isgloveson (`self.IsGlovesOn`))
  (bind _ispantson (`self.IsPantsOn`))
  (bind _isbootson (`self.IsBootsOn`))
  (bind _ishelmeton (`self.IsHelmetOn`))
  (`|ExecutionSequence`
    (:`then_0`
      (`SceneComponent.SetVisibility` (`self.SKM_m_med_nrw_Firefighter_Jacket`) _isjacketon false)
      (`MeshComponent.SetScalarParameterValueOnMaterials` (`self.Body`) "Slot_1" (`KismetMathLibrary.Conv_BoolToDouble` _isjacketon)))
    (:`then_1`
      (`SceneComponent.SetVisibility` (`self.SKM_m_med_nrw_Firefighter_Gloves`) _isgloveson false)
      (`MeshComponent.SetScalarParameterValueOnMaterials` (`self.Body`) "Slot_2" (`KismetMathLibrary.Conv_BoolToDouble` _isgloveson)))
    (:`then_2`
      (`SceneComponent.SetVisibility` (`self.SKM_m_med_nrw_Firefighter_Pants`) _ispantson false)
      (`MeshComponent.SetScalarParameterValueOnMaterials` (`self.Body`) "Slot_3" (`KismetMathLibrary.Conv_BoolToDouble` _ispantson)))
    (:`then_3`
      (`SceneComponent.SetVisibility` (`self.SKM_m_med_nrw_Firefighter_Boots`) _isbootson false)
      (`MeshComponent.SetScalarParameterValueOnMaterials` (`self.Body`) "Slot_4" (`KismetMathLibrary.Conv_BoolToDouble` _isbootson)))
    (:`then_4`
      (`SceneComponent.SetVisibility` (`self.SKM_m_med_nrw_Firefighter_Helmet`) _ishelmeton false)
      (`SkeletalMeshComponent.SetMorphTarget` (`self.Head`) "mt_firefighter_helmet" (`KismetMathLibrary.Conv_BoolToDouble` _ishelmeton) true))
    (:`then_5`
      (`SceneComponent.SetVisibility` (`self.SKM_m_med_nrw_Firefighter_Equipment`) (`self.IsEquipmentOn`) false))))

(fn `UserConstructionScript`
  (`SkinnedMeshComponent.SetLeaderPoseComponent` (`self.Head`) (`self.Body`) false false)
  (`SkinnedMeshComponent.SetLeaderPoseComponent` (`self.SKM_m_med_nrw_Firefighter_Gloves`) (`self.Body`) false false)
  (`SkinnedMeshComponent.SetLeaderPoseComponent` (`self.SKM_m_med_nrw_Firefighter_Pants`) (`self.Body`) false false)
  (`SkinnedMeshComponent.SetLeaderPoseComponent` (`self.SKM_m_med_nrw_Firefighter_Boots`) (`self.Body`) false false)
  (`SkinnedMeshComponent.SetLeaderPoseComponent` (`self.SKM_m_med_nrw_Firefighter_Helmet`) (`self.Body`) false false)
  (set `SkeletalMeshComponent.AnimationData` (`self.Animation`) (`self.Body`))
  (`|ExecutionSequence`
    (:`then_0`
      (`SceneComponent.SetVisibility` (`self.Head`) (`self.IsHeadVisible`) false)
      (`SceneComponent.SetVisibility` (`self.SM_Bat`) (`self.IsBatArmed`) false))
    (:`then_1`
      (`self.SetOutfitsVisability`))))